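; BP_AbelInsight provides an insight-style highlight for AI guards and pickups in the level.
; At BeginPlay it caches every BP_AI_Guard and BP_Pickups actor into two arrays, so later spawns are not included.
; HighLightAll sets an outline overlay material on each guard and pickup mesh, and EndHighLight clears it.
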(event Custom|HighLightAll
  (for _array_element (Variables|Default|GetAIBP)
    (Rendering|Material|SetOverlayMaterial (Variables|/Script/Engine.Character|GetMesh _array_element) (Variables|Default|GetOutLineMaterial) :!class /Script/Engine.MeshComponent))
  (for _array_element_2 (Variables|Default|GetPickUps)
    (Rendering|Material|SetOverlayMaterial (Variables|/Game/Prototype/Environment/BP_PickUps/BP_Pickups.BP_Pickups_C|GetPickups _array_element_2) (Variables|Default|GetOutLineMaterial) :!class /Script/Engine.MeshComponent)))

(event Custom|EndHighLight
  (for _array_element (Variables|Default|GetAIBP)
    (Rendering|Material|SetOverlayMaterial (Variables|/Script/Engine.Character|GetMesh _array_element) 0 :!class /Script/Engine.MeshComponent))
  (for _array_element_2 (Variables|Default|GetPickUps)
    (Rendering|Material|SetOverlayMaterial (Variables|/Game/Prototype/Environment/BP_PickUps/BP_Pickups.BP_Pickups_C|GetPickups _array_element_2) 0 :!class /Script/Engine.MeshComponent)))

(event EventBeginPlay
  (bind _outactors (Actor|GetAllActorsOfClass "/Game/Prototype/AI/BP_AI_Guard.BP_AI_Guard_C"))
  (Variables|Default|SetAIBP _outactors)
  (bind _outactors_2 (Actor|GetAllActorsOfClass "/Game/Prototype/Environment/BP_PickUps/BP_Pickups.BP_Pickups_C"))
  (Variables|Default|SetPickUps _outactors_2))

(fn ConstructionScript)