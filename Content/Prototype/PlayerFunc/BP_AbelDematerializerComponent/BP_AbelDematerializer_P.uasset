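; Prototype dematerializer actor that builds a block of cube components and shows a special material while the player is in hack mode.
; The construction script spawns X×Y×Z dematerialize components with the normal material, then MoveCube lays them out as a grid using the cube dimensions.
; On BeginPlay it binds to the player character's enter and end hack mode events, which swap every cube's material between hack and normal.
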(event Custom|ChangeMaterialToNormal
  ;[0.15 0.15 0.15 0.5] 进入骇客模式显示特殊材质
  (for _array_element (Variables|Default|GetDematerializeComp)
    (Rendering|Material|SetMaterial _array_element 0 (Variables|Default|GetNormalMaterial))))

(event Custom|ChangeMaterialToHack
  ;[0.15 0.15 0.15 0.5] 进入骇客模式显示特殊材质
  (for _array_element (Variables|Default|GetDematerializeComp)
    (Rendering|Material|SetMaterial _array_element 0 (Variables|Default|GetHackModeMaterial))))

(event EventBeginPlay
  (bind _returnvalue (Game|GetPlayerCharacter 0))
  (bind _asbp_3dcharacter_p (Utilities|Casting|CastToBP_3DCharacter_P _returnvalue))
  (EventDispatchers|BindEventtoEnterHackMode _asbp_3dcharacter_p (delegate Custom|ChangeMaterialToHack))
  (EventDispatchers|BindEventtoEndHackMode _asbp_3dcharacter_p (delegate Custom|ChangeMaterialToNormal)))

(fn ConstructionScript
  ;[0.15 0.15 0.15 0.5] 创建新的虚化物（大于0执行）
  (bind _output_get (Variables|Default|SetTotalCubeNum (* (Variables|Config|GetXCubeNum) (Variables|Config|GetYCubeNum) (Variables|Config|GetZCubeNum))))
  (Math|Integer|CompareInt _output_get
    (:>
      (bind _dematerializecomp (CallFunction|CreateCube "0, 0, 0" _output_get))
      (CallFunction|MoveCube _dematerializecomp))))

(fn CreateCube
  (params (Location :type Vector) (CreateNum :type Integer))
  ;[0.15 0.15 0.15 0.5] 创建一个Cube并把他加入到数组中
  (for _index (range 0 (- CreateNum 1))
    (bind _returnvalue (AddComponent|AddBPCDematerializeComp false (Math|Transform|MakeTransform Location "0, 0, 0" "1.000000,1.000000,1.000000")))
    (Rendering|Material|SetMaterial _returnvalue 0 (Variables|Default|GetNormalMaterial))
    (Utilities|Array|Add (Variables|Default|GetDematerializeComp) _returnvalue)
    (Transformation|SetMobility _returnvalue "Stationary"))
  (return (Variables|Default|GetDematerializeComp)))

(fn MoveCube
  (params (CubeArray :type Array%20of%20BPC%20Dematerialize%20Comp%20Object%20References))
  (for _index (range 1 (Variables|Config|GetZCubeNum))
    (for _index_2 (range 1 (Variables|Config|GetYCubeNum))
      (for _index_3 (range 1 (Variables|Config|GetXCubeNum))
        (LocalVariables|SetXPos (+ (* (- _index_3 1) (Variables|Default|GetCubeXLength)) (/ (Variables|Default|GetCubeXLength) 2.0)))
        (LocalVariables|SetYPos (+ (* (- _index_2 1) (Variables|Default|GetCubeYLength)) (/ (Variables|Default|GetCubeYLength) -2.0)))
        (LocalVariables|SetZPos (+ (* (- _index 1) (Variables|Default|GetCubeZLength)) (/ (Variables|Default|GetCubeZLength) 2.0)))
        (Transformation|SetRelativeLocation (Utilities|Array|Get(acopy) CubeArray (LocalVariables|GetNowIndex)) (Math|Vector|MakeVector (LocalVariables|GetXPos) (LocalVariables|GetYPos) (LocalVariables|GetZPos)) false true)
        (Math|Integer|IncrementInt (LocalVariables|GetNowIndex))))))