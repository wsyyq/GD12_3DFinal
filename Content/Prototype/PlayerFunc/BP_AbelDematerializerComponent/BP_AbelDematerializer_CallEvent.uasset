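; Dematerializer Blueprint variant that broadcasts HasBeenDematerialized whenever one of its child cubes is dematerialized.
; CreateCube adds BPC_DematerializeComp_CallEvent components at a given location, sets their normal material and Stationary mobility, and collects them in DematerializeComp.
; BeginPlay runs the parent logic, then binds each component's brick-destroy event to a handler that relays it through that dispatcher.
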(event Custom|OneHasBeenDematerialized
  ;[0.15 0.15 0.15 0.5] 在子物体被去物质化后，发送事件
  (Default|CallEventHasBeenDematerialized))

(event EventBeginPlay
  (|CallParentFunction)
  ;[0.15 0.15 0.15 0.5] 在子物体被去物质化后，发送事件
  (for _array_element (Variables|Default|GetDematerializeComp)
    (EventDispatchers|BindEventtoEventBrickCompDestroy (.AsBPC%20Dematerialize%20Comp%20Call%20Event (Utilities|Casting|CastToBPC_DematerializeComp_CallEvent _array_element)) (delegate Custom|OneHasBeenDematerialized))))

(fn ConstructionScript
  (|CallParentFunction))

(fn CreateCube
  (params (Location :type Vector :default "0, 0, 0") (CreateNum :type Integer))
  (for _index (range 0 (- CreateNum 1))
    (bind _returnvalue (AddComponent|AddBPCDematerializeCompCallEvent false (Math|Transform|MakeTransform Location "0, 0, 0" "1.000000,1.000000,1.000000")))
    (Rendering|Material|SetMaterial _returnvalue 0 (Variables|Default|GetNormalMaterial))
    (Utilities|Array|Add (Variables|Default|GetDematerializeComp) _returnvalue)
    (Transformation|SetMobility _returnvalue "Stationary"))
  (return (Variables|Default|GetDematerializeComp)))