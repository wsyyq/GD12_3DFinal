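; Hologram decoy actor for the Abel hologram ability that can distract listeners with noise.
; While ShouldDistract is set, it emits a loud, range-limited noise at its location every tick.
; PlaceBoom, when UseSecret is set, waits briefly and then spawns BP_SecretWeapon at the BoomPlace transform.
; On EndPlay it clears HasPreviewHologram on the player's BP_3DCharacter_P.
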(event Custom|PlaceBoom
  (if (Variables|Default|GetUseSecret)
    (Utilities|FlowControl|Delay 2.5)
    (Game|SpawnActorfromClass "/Game/Prototype/PlayerFunc/BP_AbelHologram/BP_SecretWeapon.BP_SecretWeapon_C" (Transformation|GetWorldTransform (Variables|Default|GetBoomPlace)) "Undefined" "MultiplyWithRoot" 0 0)))

(event EventEndPlay
  (params (EndPlayReason :type EEndPlayReason%20Enum :default "Destroyed"))
  (bind _returnvalue (Game|GetPlayerCharacter 0))
  (bind _asbp_3dcharacter_p (Utilities|Casting|CastToBP_3DCharacter_P _returnvalue))
  (Utilities|IsValid _asbp_3dcharacter_p
    (:Is%20Valid
      (Variables|/Game/Prototype/GameMode/BP_3DCharacter_P.BP_3DCharacter_P_C|SetHasPreviewHologram _asbp_3dcharacter_p false))))

(event EventTick
  (params (DeltaSeconds :type Float%20%28single-precision%29))
  (if (Variables|Default|GetShouldDistract)
    (Class|Actor|MakeNoise 5.5e+02 (Game|GetInstigator) (Transformation|GetActorLocation) 1e+03 "None")))

(fn ConstructionScript)