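; BP_SecretWeapon is a one-shot bomb trap for AI guards whose small Niagara effect shows during the player's hack mode.
; DamageBox tracks guards in range and reveals that effect when they enter or leave.
; The first guard entering KillBox takes heavy damage, then living tracked guards receive FallHurt after a brief delay.
; A timeline scales up the explosion effect, then the actor disables collision and destroys itself.
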(event OnComponentBeginOverlap(KillBox)
  (params (OverlappedComponent :type Primitive%20Component%20Object%20Reference) (OtherActor :type Actor%20Object%20Reference) (OtherComp :type Primitive%20Component%20Object%20Reference) (OtherBodyIndex :type Integer) (bFromSweep :type Boolean) (SweepResult :type Hit%20Result%20Structure%20%28by%20ref%29))
  (bind _asbp_ai_guard (Utilities|Casting|CastToBP_AI_Guard OtherActor))
  ;[0.15 0.15 0.15 0.5] 造成致命伤害与爆炸伤害
  (Utilities|FlowControl|DoOnce false
    (:Completed
      (Game|Damage|ApplyDamage _asbp_ai_guard 1e+02 0 self)
      (Utilities|FlowControl|Delay 0.1)
      (for _array_element (Variables|Default|GetDamageActors)
        (Utilities|IsValid _array_element
          (:Is%20Valid
            (if (not (Variables|/Game/Prototype/AI/BP_AI_Guard.BP_AI_Guard_C|GetIsAIDie _array_element))
              (Default|FallHurt _array_element)))))
      (CallFunction|StartBoom))))

(event OnComponentBeginOverlap(DamageBox)
  (params (OverlappedComponent :type Primitive%20Component%20Object%20Reference) (OtherActor :type Actor%20Object%20Reference) (OtherComp :type Primitive%20Component%20Object%20Reference) (OtherBodyIndex :type Integer) (bFromSweep :type Boolean) (SweepResult :type Hit%20Result%20Structure%20%28by%20ref%29))
  ;[0.15 0.15 0.15 0.5] 记录要伤害的对象
  (bind _asbp_ai_guard (Utilities|Casting|CastToBP_AI_Guard OtherActor))
  (Utilities|Array|Add (Variables|Default|GetDamageActors) _asbp_ai_guard)
  (Development|SetHiddeninGame (Variables|Default|GetNS_BombSmall) false false)
  (Variables|Default|SetIsActivate true))

(event OnComponentEndOverlap(DamageBox)
  (params (OverlappedComponent :type Primitive%20Component%20Object%20Reference) (OtherActor :type Actor%20Object%20Reference) (OtherComp :type Primitive%20Component%20Object%20Reference) (OtherBodyIndex :type Integer))
  ;[0.15 0.15 0.15 0.5] 记录要伤害的对象
  (bind _asbp_ai_guard (Utilities|Casting|CastToBP_AI_Guard OtherActor))
  (Utilities|Array|RemoveItem (Variables|Default|GetDamageActors) _asbp_ai_guard)
  (Development|SetHiddeninGame (Variables|Default|GetNS_BombSmall) false false)
  (Variables|Default|SetIsActivate false))

(event Custom|SelfDestruction
  ;[0.15 0.15 0.15 0.5] 结束后自毁
  (Collision|SetCollisionEnabled (Variables|Default|GetKillBox) "NoCollision")
  (Collision|SetCollisionEnabled (Variables|Default|GetDamageBox) "NoCollision")
  (Components|Activation|SetAutoActivate (Variables|Default|GetNS_BombBig) false)
  (Components|Activation|SetAutoActivate (Variables|Default|GetNS_BombSmall) false)
  (Utilities|FlowControl|Delay 0.5)
  (Actor|DestroyActor))

(event Custom|StartBoom
  (bind _ns_bombbig (Variables|Default|GetNS_BombBig))
  ;[0.15 0.15 0.15 0.5] 爆炸VFX
  (Components|Activation|Activate _ns_bombbig true)
  (Components|Activation|SetAutoActivate _ns_bombbig false)
  (bind _time (Timeline|NSBigger PlayFromStart)
    (:Update
      (Transformation|SetRelativeScale3D (Variables|Default|GetScene) (Math|Vector|Lerp(Vector) "0.050000,0.050000,0.050000" "4.000000,4.000000,4.000000" _time)))
    (:Finished
      (CallFunction|SelfDestruction))))

(event Custom|ShowNS
  (Development|SetHiddeninGame (Variables|Default|GetNS_BombSmall) false false))

(event Custom|HideNS
  (Development|SetHiddeninGame (Variables|Default|GetNS_BombSmall) true false))

(event EventBeginPlay
  (bind _returnvalue (Game|Player|GetPlayerPawn 0))
  (bind _asbp_3dcharacter_p (Utilities|Casting|CastToBP_3DCharacter_P _returnvalue))
  (Development|SetHiddeninGame (Variables|Default|GetNS_BombSmall) true false)
  (if (not (Variables|Default|GetIsActivate))
    (EventDispatchers|BindEventtoEnterHackMode _asbp_3dcharacter_p (delegate Custom|ShowNS))
    (EventDispatchers|BindEventtoEndHackMode _asbp_3dcharacter_p (delegate Custom|HideNS))))

(fn ConstructionScript)