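; BP_AbelReborn is a respawn point that the player can pick up and later place in the level.
; PlaceAndActiveSelf moves it to the given position, marks it active, switches to the enabled decal and restores visibility and collision.
; E2Interactive hides it, disables collision, deactivates it and returns itself as pickable.
; Box overlap toggles the interaction prompt, while the player's hack-mode events toggle its Niagara effect.
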(event OnComponentBeginOverlap(Box)
  (params (OverlappedComponent :type Primitive%20Component%20Object%20Reference) (OtherActor :type Actor%20Object%20Reference) (OtherComp :type Primitive%20Component%20Object%20Reference) (OtherBodyIndex :type Integer) (bFromSweep :type Boolean) (SweepResult :type Hit%20Result%20Structure%20%28by%20ref%29))
  (Utilities|Casting|CastToBP_3DCharacter_P OtherActor)
  (Development|SetHiddeninGame (Variables|Default|GetInteractWidget) false false)
  (Default|ShowObjectType (.AsWBP%20Interact%20Panel (Utilities|Casting|CastToWBP_InteractPanel (UserInterface|GetWidget (Variables|Default|GetInteractWidget)))) (Variables|Default|GetObjectName) "NewEnumerator13"))

(event OnComponentEndOverlap(Box)
  (params (OverlappedComponent :type Primitive%20Component%20Object%20Reference) (OtherActor :type Actor%20Object%20Reference) (OtherComp :type Primitive%20Component%20Object%20Reference) (OtherBodyIndex :type Integer))
  (Utilities|Casting|CastToBP_3DCharacter_P OtherActor)
  (Development|SetHiddeninGame (Variables|Default|GetInteractWidget) true false))

(event Custom|PlaceAndActiveSelf
  (params (PlacePosition :type Vector))
  ;[0.15 0.15 0.15 0.5] 将当前重生点激活
  (Variables|Default|SetIsActivate true)
  (Transformation|SetActorLocation PlacePosition false true)
  (Rendering|Components|Decal|SetDecalMaterial (Variables|Default|GetDecal) "/Game/GD12_3D/UI/Resources/Materials/M_Reborn_Enable_Decal.M_Reborn_Enable_Decal")
  ;[0.15 0.15 0.15 0.5] 将当前物体显形
  (Rendering|SetActorHiddenInGame false)
  (Collision|SetCollisionEnabled (Variables|Default|GetStaticMesh) "QueryAndPhysics")
  (Collision|SetCollisionEnabled (Variables|Default|GetBox) "QueryAndPhysics"))

(event Custom|HackerActivate
  (Development|SetHiddeninGame (Variables|Default|GetNiagara) false false))

(event Custom|HackerDeactivate
  (Development|SetHiddeninGame (Variables|Default|GetNiagara) true false))

(event EventBeginPlay
  (Utilities|FlowControl|Sequence
    (:then_0
      ;[0.15 0.15 0.15 0.5] 刚进入游戏场上所有重生点拾取物均不激活
      (Variables|Default|SetIsActivate false)
      (Development|SetHiddeninGame (Variables|Default|GetInteractWidget) true false))
    (:then_1
      (bind _asbp_3dcharacter_p (Utilities|Casting|CastToBP_3DCharacter_P (Game|Player|GetPlayerPawn 0)))
      (EventDispatchers|BindEventtoEnterHackMode _asbp_3dcharacter_p (delegate Custom|HackerActivate))
      (EventDispatchers|BindEventtoEndHackMode _asbp_3dcharacter_p (delegate Custom|HackerDeactivate)))))

(fn ConstructionScript)

(fn E2Interactive
  ;[0.15 0.15 0.15 0.5] 将当前物体隐形
  (Rendering|SetActorHiddenInGame true)
  (Collision|SetCollisionEnabled (Variables|Default|GetStaticMesh) "NoCollision")
  (Collision|SetCollisionEnabled (Variables|Default|GetBox) "NoCollision")
  (Default|CallEventFinishInteract)
  (Default|HideObjectType (.AsWBP%20Interact%20Panel (Utilities|Casting|CastToWBP_InteractPanel (UserInterface|GetWidget (Variables|Default|GetInteractWidget)))))
  ;[0.15 0.15 0.15 0.5] 设置为不可用状态
  (Variables|Default|SetIsActivate false)
  (return true "NewEnumerator13" self 0 "" ""))