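; BP_AbelChip is a pickup that unlocks hacker mode for the 3D player character.
; Its trigger box shows or hides an interact widget labeled with the object's type and name as the player enters or leaves.
; E2Interactive runs once: it hides the chip, disables its collision, sets HasHackerChip on the player, fires the finish-interact event, posts a pickup hint and returns the pickup result.
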(event OnComponentBeginOverlap(PickTriggerBox)
  (params (OverlappedComponent :type Primitive%20Component%20Object%20Reference) (OtherActor :type Actor%20Object%20Reference) (OtherComp :type Primitive%20Component%20Object%20Reference) (OtherBodyIndex :type Integer) (bFromSweep :type Boolean) (SweepResult :type Hit%20Result%20Structure%20%28by%20ref%29))
  ;[0.15 0.15 0.15 0.5] WBP
  (Utilities|Casting|CastToBP_3DCharacter_P OtherActor)
  (Development|SetHiddeninGame (Variables|Default|GetInteractWidget) false false)
  (Default|ShowObjectType (.AsWBP%20Interact%20Panel (Utilities|Casting|CastToWBP_InteractPanel (UserInterface|GetWidget (Variables|Default|GetInteractWidget)))) "NewEnumerator8" "" (Variables|Default|GetObjectName)))

(event OnComponentEndOverlap(PickTriggerBox)
  (params (OverlappedComponent :type Primitive%20Component%20Object%20Reference) (OtherActor :type Actor%20Object%20Reference) (OtherComp :type Primitive%20Component%20Object%20Reference) (OtherBodyIndex :type Integer))
  ;[0.15 0.15 0.15 0.5] WBP
  (Utilities|Casting|CastToBP_3DCharacter_P OtherActor)
  (Development|SetHiddeninGame (Variables|Default|GetInteractWidget) true false))

(event EventBeginPlay
  (Development|SetHiddeninGame (Variables|Default|GetInteractWidget) true false))

(fn ConstructionScript)

(fn E2Interactive
  (bind _returnvalue (Game|Player|GetPlayerPawn 0))
  (bind _asbp_3dcharacter_p (Utilities|Casting|CastToBP_3DCharacter_P _returnvalue))
  (Utilities|FlowControl|DoOnce false
    (:Completed
      (Development|PrintString "Hacker Mode Available. 可使用骇客技能。")
      (Rendering|SetActorHiddenInGame true)
      (Collision|SetCollisionEnabled (Variables|Default|GetChip) "NoCollision")
      (Collision|SetCollisionEnabled (Variables|Default|GetPickTriggerBox) "NoCollision")
      (bind _asbp_3dcharacter_p_2 (Utilities|Casting|CastToBP_3DCharacter_P (Game|GetPlayerCharacter 0)))
      (Variables|/Game/Prototype/GameMode/BP_3DCharacter_P.BP_3DCharacter_P_C|SetHasHackerChip _asbp_3dcharacter_p_2 true)
      (Default|HideObjectType (.AsWBP%20Interact%20Panel (Utilities|Casting|CastToWBP_InteractPanel (UserInterface|GetWidget (Variables|Default|GetInteractWidget)))))
      (Default|CallEventFinishInteract)
      (Default|AddHint _asbp_3dcharacter_p "Hacker Chip" (Utilities|String|ToString(Text) (Variables|Default|GetObjectName)) false false)
      (Default|SetHint _asbp_3dcharacter_p)
      (return true "NewEnumerator8" 0 0 "" ""))))