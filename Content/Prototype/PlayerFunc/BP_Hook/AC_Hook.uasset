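; Prototype grappling-hook component for a character that targets and pulls toward hook anchors.
; Anchors register through add/remove events; each Tick selects the one best aligned with camera forward by dot product and highlights it.
; Middle mouse yaws the character toward that anchor, starts MoveComponentTo to just above it and plays a montage.
; Travel time divides the character's distance from world origin, not the anchor, by Speed.
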(event Custom|REMOVEHOOK
  (params (Item :type BP%20Anchor%20Object%20Reference%20%28by%20ref%29))
  ;[0.15 0.15 0.15 0.5] 2
  (Utilities|Array|RemoveItem (Variables|Default|GetHooksSelected) Item))

(event Custom|ADDTOHOOK
  (params (NewItem :type BP%20Anchor%20Object%20Reference%20%28by%20ref%29))
  ;[0.15 0.15 0.15 0.5] 2
  (Utilities|Array|Add (Variables|Default|GetHooksSelected) NewItem))

(event Custom|角色转向
  ;[0.15 0.15 0.15 0.5] 角色看向锚点
  (Transformation|SetActorRotation (Variables|Default|GetCharacter) (Math|Rotator|MakeRotator 0.0 0.0 (.yaw (Math|Rotator|FindLookatRotation (Transformation|GetActorLocation (Variables|Default|GetCharacter)) (Transformation|GetActorLocation (Variables|Default|GetCurrentHook)))))))

(event Custom|角色移动
  (bind _speed (Variables|Default|GetSpeed))
  (bind _character (Variables|Default|GetCharacter))
  (bind _currenthook (Variables|Default|GetCurrentHook))
  (bind _returnvalue (Transformation|GetActorLocation _character))
  (bind _returnvalue_2 (Transformation|GetActorLocation _currenthook))
  (bind _returnvalue_3 (Math|Vector|Distance(Vector) _returnvalue "0, 0, 0"))
  (bind _returnvalue_4 (/ _returnvalue_3 _speed))
  ;[0.15 0.15 0.15 0.5] 钩锁速度保持
  (Utilities|FlowControl|Sequence
    (:then_0
      (Components|MoveComponentTo (Variables|/Script/Engine.Actor|GetRootComponent (Variables|Default|GetCharacter)) (Math|Vector|MakeVector (.x _returnvalue_2) (.y _returnvalue_2) (+ (.z _returnvalue_2) 1e+02)) (Transformation|GetActorRotation _character) false false _returnvalue_4 false))
    (:then_1
      (Utilities|FlowControl|Delay _returnvalue_4))))

(event EventBeginPlay
  ;[0.15 0.15 0.15 0.5] 1
  (bind _ascharacter (Utilities|Casting|CastToCharacter (Components|GetOwner)))
  (Variables|Default|SetCharacter _ascharacter)
  (bind _asplayer_controller (Utilities|Casting|CastToPlayerController (Pawn|GetController _ascharacter)))
  (Variables|Default|SetController _asplayer_controller))

(event EventTick
  (params (DeltaSeconds :type Float%20%28single-precision%29))
  ;[0.15 0.15 0.15 0.5] 3
  (bind _新锚点 (CallFunction|与准心角度最小的锚点检测))
  (if (not (== _新锚点 (Variables|Default|GetCurrentHook)))
    (Utilities|IsValid (Variables|Default|GetCurrentHook)
      (:Is%20Valid
        (Default|ResetTargetColor (Variables|Default|GetCurrentHook)))
      (:Is%20Not%20Valid
        _))
    (bind _output_get (Variables|Default|SetCurrentHook _新锚点))
    (Utilities|IsValid _output_get
      (:Is%20Valid
        (Default|SetTargetColor _output_get)))))

(event Input|MouseEvents|MiddleMouseButton
  (params (Key :type Key%20Structure :default "None"))
  ;[0.15 0.15 0.15 0.5] 元神启动
  (:Pressed
    (Utilities|IsValid (Variables|Default|GetCurrentHook)
      (:Is%20Valid
        (CallFunction|角色转向)
        (CallFunction|角色移动)
        (Animation|PlayAnimMontage (Variables|Default|GetCharacter) 0 1.0 "None")))))

(fn 角度判断
  (params (钩索actor :type BP%20Anchor%20Object%20Reference))
  (bind _returnvalue (Transformation|GetActorLocation 钩索actor))
  ;[0.15 0.15 0.15 0.5] 计算夹角
  (return (Math|Vector|DotProduct (Math|Vector|GetForwardVector (Variables|/Script/Engine.Actor|GetRootComponent (Game|GetPlayerCameraManager 0))) (Math|Vector|GetUnitDirection(Vector) (Transformation|GetActorLocation (Game|GetPlayerCharacter 0)) (Math|Vector|MakeVector (.x _returnvalue) (.y _returnvalue) (+ (.z _returnvalue) -7e+01))))))

(fn 与准心角度最小的锚点检测
  (Utilities|FlowControl|DoOnce false :!label _label
    (:Completed
      (LocalVariables|Set目标锚点 0)
      (for _array_element (Variables|Default|GetHooksSelected)
        ;[0.15 0.15 0.15 0.5] 视野范围内
        (bind _output_get (Variables|/Game/Prototype/PlayerFunc/BP_Hook/BP_Anchor.BP_Anchor_C|Set目标Dot _array_element (CallFunction|角度判断 _array_element)))
        (Math|Float|CompareFloat _output_get 0.0
          (:>
            (if (> (CallFunction|角度判断 _array_element) 0.0) :!label _label_2
              (bind _目标锚点 (LocalVariables|Get目标锚点)
                (:then
                  ;[0.15 0.15 0.15 0.5] 如果已经存在目标锚点，比大小
                  (if (> (CallFunction|角度判断 _array_element) (Variables|/Game/Prototype/PlayerFunc/BP_Hook/BP_Anchor.BP_Anchor_C|Get目标Dot _目标锚点))
                    ;[0.15 0.15 0.15 0.5] 如果准心更接近该物体，则将该物体设置为目标
                    (LocalVariables|Set目标锚点 _array_element)))
                (:else
                  ;[0.15 0.15 0.15 0.5] 不存在，则将他设为目标锚点
                  (LocalVariables|Set目标锚点 _array_element)))))
          (:==
            (goto _label_2))
          (:<
            (Development|PrintString "球在身后"))))
      (Utilities|FlowControl|Sequence
        (:then_0
          (return (LocalVariables|Get目标锚点)))
        (:then_1
          (goto _label Reset))))))