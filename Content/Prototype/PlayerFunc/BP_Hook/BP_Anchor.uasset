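; BP_Anchor is a hook anchor point that registers itself with actors able to hook onto it.
; When an actor with an AC_Hook component overlaps its collision sphere, it adds itself to that component, and it removes itself when the overlap ends.
; SetTargetColor and ResetTargetColor events swap the sphere's material between a look and an ignore material to show whether it is targeted.
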(event OnComponentBeginOverlap(Sphere_collision)
  (params (OverlappedComponent :type Primitive%20Component%20Object%20Reference) (OtherActor :type Actor%20Object%20Reference) (OtherComp :type Primitive%20Component%20Object%20Reference) (OtherBodyIndex :type Integer) (bFromSweep :type Boolean) (SweepResult :type Hit%20Result%20Structure%20%28by%20ref%29))
  (bind _returnvalue (Actor|GetComponentbyClass OtherActor "/Game/Prototype/PlayerFunc/BP_Hook/AC_Hook.AC_Hook_C"))
  (Utilities|IsValid _returnvalue
    (:Is%20Valid
      (Default|ADDTOHOOK _returnvalue self))))

(event OnComponentEndOverlap(Sphere_collision)
  (params (OverlappedComponent :type Primitive%20Component%20Object%20Reference) (OtherActor :type Actor%20Object%20Reference) (OtherComp :type Primitive%20Component%20Object%20Reference) (OtherBodyIndex :type Integer))
  (bind _returnvalue (Actor|GetComponentbyClass OtherActor "/Game/Prototype/PlayerFunc/BP_Hook/AC_Hook.AC_Hook_C"))
  (Utilities|IsValid _returnvalue
    (:Is%20Valid
      (Default|REMOVEHOOK _returnvalue self))))

(event Custom|ResetTargetColor
  (Rendering|Material|SetMaterial (Variables|Default|GetSphere) 0 "/Game/Prototype/PlayerFunc/BP_Hook/BP_Ignore.BP_Ignore"))

(event Custom|SetTargetColor
  (Rendering|Material|SetMaterial (Variables|Default|GetSphere) 0 "/Game/Prototype/PlayerFunc/BP_Hook/BP_Look.BP_Look"))

(event EventBeginPlay)

(event Collision|EventActorBeginOverlap
  (params (OtherActor :type Actor%20Object%20Reference)))

(event EventTick
  (params (DeltaSeconds :type Float%20%28single-precision%29)))

(fn ConstructionScript)