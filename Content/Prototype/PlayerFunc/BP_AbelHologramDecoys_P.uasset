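; BP_AbelHologramDecoys_P is a player hologram decoy that draws attention through noise and can spawn a secret weapon.
; While ShouldDistract is set, it reports a loud, range-limited noise event at its location every tick, attributed to its instigator.
; When UseSecret is set, the PlaceBoom event waits briefly, then spawns BP_SecretWeapon at the BoomPlace component's transform.
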(event Custom|PlaceBoom
  (if (Variables|Default|GetUseSecret)
    (Utilities|FlowControl|Delay 2.5)
    (Game|SpawnActorfromClass "/Game/Prototype/PlayerFunc/BP_SecretWeapon.BP_SecretWeapon_C" (Transformation|GetWorldTransform (Variables|Default|GetBoomPlace)) "Undefined" "MultiplyWithRoot" 0 0)))

(event EventTick
  (params (DeltaSeconds :type Float%20%28single-precision%29))
  (if (Variables|Default|GetShouldDistract)
    (Class|Actor|MakeNoise 5.5e+02 (Game|GetInstigator) (Transformation|GetActorLocation) 1e+03 "None")))

(fn ConstructionScript)