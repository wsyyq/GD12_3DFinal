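; BP_AbelDematerializer_P is a prototype cube actor that responds to the player's hack mode and can be dematerialized.
; On BeginPlay it binds to the enter and end hack mode events on the player's BP_3DCharacter_P, swapping the cube between hack and normal materials.
; Its Dematerialize event, which nothing in this Blueprint calls, hides the actor and disables the cube's collision, with no restore path here.
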(event Custom|ChangeMaterialToNormal
  (Rendering|Material|SetMaterial (Variables|Components|GetCube) 0 (Variables|Default|GetNormalMaterial)))

(event Custom|ChangeMaterialToHack
  (Rendering|Material|SetMaterial (Variables|Components|GetCube) 0 (Variables|Default|GetHackModeMaterial)))

(event Custom|Dematerialize
  (Rendering|SetActorHiddenInGame true)
  (Collision|SetCollisionEnabled (Variables|Components|GetCube) "NoCollision"))

(event EventBeginPlay
  (bind _returnvalue (Game|GetPlayerCharacter 0))
  (bind _asbp_3dcharacter_p (Utilities|Casting|CastToBP_3DCharacter_P _returnvalue))
  (EventDispatchers|BindEventtoEnterHackMode _asbp_3dcharacter_p (delegate Custom|ChangeMaterialToHack))
  (EventDispatchers|BindEventtoEndHackMode _asbp_3dcharacter_p (delegate Custom|ChangeMaterialToNormal)))

(fn ConstructionScript)