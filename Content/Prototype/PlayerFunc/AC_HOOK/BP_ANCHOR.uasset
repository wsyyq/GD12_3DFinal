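; BP_ANCHOR is a hook anchor actor that registers itself with the AC_HOOK component of actors that come within range.
; Overlap begin and end on Sphere_collision call ADDTOHOOK and REMOVEHOOK on that component, passing the anchor.
; Two events for setting and exiting target-anchor state swap the Sphere's material between LOOK_at_BP and Ignore_at_BP as visual feedback.
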(event OnComponentBeginOverlap(Sphere_collision)
  (params (OverlappedComponent :type Primitive%20Component%20Object%20Reference) (OtherActor :type Actor%20Object%20Reference) (OtherComp :type Primitive%20Component%20Object%20Reference) (OtherBodyIndex :type Integer) (bFromSweep :type Boolean) (SweepResult :type Hit%20Result%20Structure%20%28by%20ref%29))
  (bind _returnvalue (Actor|GetComponentbyClass OtherActor "/Game/Prototype/PlayerFunc/AC_HOOK/AC_HOOK.AC_HOOK_C"))
  (Utilities|IsValid _returnvalue
    (:Is%20Valid
      (Default|ADDTOHOOK _returnvalue self))))

(event OnComponentEndOverlap(Sphere_collision)
  (params (OverlappedComponent :type Primitive%20Component%20Object%20Reference) (OtherActor :type Actor%20Object%20Reference) (OtherComp :type Primitive%20Component%20Object%20Reference) (OtherBodyIndex :type Integer))
  (bind _returnvalue (Actor|GetComponentbyClass OtherActor "/Game/Prototype/PlayerFunc/AC_HOOK/AC_HOOK.AC_HOOK_C"))
  (Utilities|IsValid _returnvalue
    (:Is%20Valid
      (Default|REMOVEHOOK _returnvalue self))))

(event Custom|退出目标锚点
  (Rendering|Material|SetMaterial (Variables|Default|GetSphere) 0 "/Game/Prototype/PlayerFunc/AC_HOOK/Ignore_at_BP.Ignore_at_BP"))

(event Custom|设为目标锚点
  (Rendering|Material|SetMaterial (Variables|Default|GetSphere) 0 "/Game/Prototype/PlayerFunc/AC_HOOK/LOOK_at_BP.LOOK_at_BP"))

(event EventBeginPlay)

(event Collision|EventActorBeginOverlap
  (params (OtherActor :type Actor%20Object%20Reference)))

(event EventTick
  (params (DeltaSeconds :type Float%20%28single-precision%29)))

(fn ConstructionScript)