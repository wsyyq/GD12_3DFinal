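; Player actor component that picks which grappling-hook anchor the player is targeting.
; ADDTOHOOK and REMOVEHOOK maintain the candidate list, which is scanned every Tick for the anchor best aligned with the view.
; Alignment is the dot product of camera forward and the direction from the character to a height-offset anchor point, ignoring anchors behind.
; When the best anchor changes, the old and new anchors are notified to exit or enter target state.
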(event Custom|REMOVEHOOK
  (params (Item :type BP%20ANCHOR%20Object%20Reference%20%28by%20ref%29))
  ;[0.15 0.15 0.15 0.5] 2
  (Utilities|Array|RemoveItem (Variables|Default|GetHOOK_SELECTED) Item))

(event Custom|ADDTOHOOK
  (params (NewItem :type BP%20ANCHOR%20Object%20Reference%20%28by%20ref%29))
  ;[0.15 0.15 0.15 0.5] 2
  (Utilities|Array|Add (Variables|Default|GetHOOK_SELECTED) NewItem))

(event EventBeginPlay
  ;[0.15 0.15 0.15 0.5] 1
  (bind _ascharacter (Utilities|Casting|CastToCharacter (Components|GetOwner)))
  (Variables|Default|SetAs%20Character _ascharacter)
  (bind _asplayer_controller (Utilities|Casting|CastToPlayerController (Pawn|GetController _ascharacter)))
  (Variables|Default|SetAs%20Player%20Controller _asplayer_controller))

(event EventTick
  (params (DeltaSeconds :type Float%20%28single-precision%29))
  ;[0.15 0.15 0.15 0.5] 3
  (bind _新锚点 (CallFunction|与准心角度最小的锚点检测))
  (if (not (== _新锚点 (Variables|Default|Get当前的锚点)))
    (Utilities|IsValid (Variables|Default|Get当前的锚点)
      (:Is%20Valid
        (Default|退出目标锚点 (Variables|Default|Get当前的锚点)))
      (:Is%20Not%20Valid
        _))
    (bind _output_get (Variables|Default|Set当前的锚点 _新锚点))
    (Utilities|IsValid _output_get
      (:Is%20Valid
        (Default|设为目标锚点 _output_get)))))

(fn 角度判断
  (params (钩索actor :type BP%20ANCHOR%20Object%20Reference))
  (bind _returnvalue (Transformation|GetActorLocation 钩索actor))
  ;[0.15 0.15 0.15 0.5] 计算夹角
  (return (Math|Vector|DotProduct (Math|Vector|GetForwardVector (Variables|/Script/Engine.Actor|GetRootComponent (Game|GetPlayerCameraManager 0))) (Math|Vector|GetUnitDirection(Vector) (Transformation|GetActorLocation (Game|GetPlayerCharacter 0)) (Math|Vector|MakeVector (.x _returnvalue) (.y _returnvalue) (+ (.z _returnvalue) -7e+01))))))

(fn 与准心角度最小的锚点检测
  (Utilities|FlowControl|DoOnce false :!label _label
    (:Completed
      (LocalVariables|Set目标锚点 0)
      (for _array_element (Variables|Default|GetHOOK_SELECTED)
        ;[0.15 0.15 0.15 0.5] 视野范围内
        (bind _output_get (Variables|/Game/Prototype/PlayerFunc/AC_HOOK/BP_ANCHOR.BP_ANCHOR_C|Set目标Dot _array_element (CallFunction|角度判断 _array_element)))
        (Math|Float|CompareFloat _output_get 0.0
          (:>
            _)
          (:==
            _))
        (if (> (CallFunction|角度判断 _array_element) 0.0)
          (bind _目标锚点 (LocalVariables|Get目标锚点)
            (:then
              ;[0.15 0.15 0.15 0.5] 如果已经存在目标锚点，比大小
              (if (> (CallFunction|角度判断 _array_element) (Variables|/Game/Prototype/PlayerFunc/AC_HOOK/BP_ANCHOR.BP_ANCHOR_C|Get目标Dot _目标锚点))
                ;[0.15 0.15 0.15 0.5] 如果准心更接近该物体，则将该物体设置为目标
                (LocalVariables|Set目标锚点 _array_element)))
            (:else
              ;[0.15 0.15 0.15 0.5] 不存在，则将他设为目标锚点
              (LocalVariables|Set目标锚点 _array_element)))))
      (Utilities|FlowControl|Sequence
        (:then_0
          (return (LocalVariables|Get目标锚点)))
        (:then_1
          (goto _label Reset))))))