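; Vending machine prop that shows an interact panel with its name and object type while the player character is inside its trigger.
; On BeginPlay it hides the widget and binds to the player's enter and end hack mode events.
; Those events swap the displayed name between a hack-mode name and the normal one, which reaches the panel on the next trigger overlap.
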(event OnComponentBeginOverlap(InteractTrigger)
  (params (OverlappedComponent :type Primitive%20Component%20Object%20Reference) (OtherActor :type Actor%20Object%20Reference) (OtherComp :type Primitive%20Component%20Object%20Reference) (OtherBodyIndex :type Integer) (bFromSweep :type Boolean) (SweepResult :type Hit%20Result%20Structure%20%28by%20ref%29))
  ;[0.15 0.15 0.15 0.5] WBP
  (Utilities|Casting|CastToBP_3DCharacter_P OtherActor)
  (Development|SetHiddeninGame (Variables|Default|GetInteractWidget) false false)
  (Default|ShowObjectType (.AsWBP%20Interact%20Panel (Utilities|Casting|CastToWBP_InteractPanel (UserInterface|GetWidget (Variables|Default|GetInteractWidget)))) (Variables|Default|GetNameOrBelong) "NewEnumerator10"))

(event OnComponentEndOverlap(InteractTrigger)
  (params (OverlappedComponent :type Primitive%20Component%20Object%20Reference) (OtherActor :type Actor%20Object%20Reference) (OtherComp :type Primitive%20Component%20Object%20Reference) (OtherBodyIndex :type Integer))
  ;[0.15 0.15 0.15 0.5] WBP
  (Utilities|Casting|CastToBP_3DCharacter_P OtherActor)
  (Development|SetHiddeninGame (Variables|Default|GetInteractWidget) true false))

(event Custom|ChangeName
  (Variables|Default|SetNameOrBelong "Abel Eden"))

(event Custom|ChangeNameAgain
  (Variables|Default|SetNameOrBelong "Verpp"))

(event EventBeginPlay
  (bind _returnvalue (Game|Player|GetPlayerPawn 0))
  (bind _asbp_3dcharacter_p (Utilities|Casting|CastToBP_3DCharacter_P _returnvalue))
  (Utilities|FlowControl|Sequence
    (:then_0
      (Development|SetHiddeninGame (Variables|Default|GetInteractWidget) true false))
    (:then_1
      (EventDispatchers|BindEventtoEnterHackMode _asbp_3dcharacter_p (delegate Custom|ChangeName))
      (EventDispatchers|BindEventtoEndHackMode _asbp_3dcharacter_p (delegate Custom|ChangeNameAgain)))))

(fn ConstructionScript)