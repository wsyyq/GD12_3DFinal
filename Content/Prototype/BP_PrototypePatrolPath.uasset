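; BP_PrototypePatrolPath is a prototype spline actor that defines a patrol route, with a wait-time entry per point.
; The construction script resizes PointWaitTime to the spline's point count and spawns a colored, sized index label above each point for editor preview.
; On BeginPlay, DebugDrawInGame either unhides the spline in game or, when off, hides the labels.
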(event EventBeginPlay
  (if (Variables|Default|GetDebugDrawInGame)
    (Development|SetHiddeninGame (Variables|Default|GetSpline) false false)
    (else
      (for _array_element (Variables|Default|GetTextRenders)
        (bind _astext_render_component (Utilities|Casting|CastToTextRenderComponent _array_element))
        (Rendering|SetVisibility _astext_render_component false false)))))

(fn ConstructionScript
  (bind _spline (Variables|Default|GetSpline))
  ;[0.15 0.15 0.15 0.5] 当前线段有几个点，就有几个PointWaitTime
  (Utilities|Array|Resize (Variables|Default|GetPointWaitTime) (Spline|GetNumberOfSplinePoints (Variables|Default|GetSpline)))
  ;[0.15 0.15 0.15 0.5] 预览界面显示当前为第几个巡逻点
  (Utilities|Array|Clear (Variables|Default|GetTextRenders))
  (for _index (range 0 (- (Spline|GetNumberOfSplinePoints (Variables|Default|GetSpline)) 1))
    (bind _returnvalue (AddComponent|AddTextRenderComponent false (Math|Transform|MakeTransform (+ (Spline|GetLocationatSplinePoint _spline _index "Local") "0.000000,0.000000,25.000000") (Transformation|GetWorldRotation _spline) "1.000000,1.000000,1.000000")))
    (Utilities|Array|Add (Variables|Default|GetTextRenders) _returnvalue)
    (Rendering|Components|TextRender|SetText _returnvalue (Utilities|Text|ToText(Integer) _index))
    (Rendering|Components|TextRender|SetTextRenderColor _returnvalue (Math|Conversions|ToColor(LinearColor) (Variables|Default|GetTextColor)))
    (Rendering|Components|TextRender|SetWorldSize _returnvalue (Variables|Default|GetTextSize))))