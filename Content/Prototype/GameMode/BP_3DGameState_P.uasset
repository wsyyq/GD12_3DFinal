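; Prototype game state that runs background music and character dialogue for the 3D player character.
; BeginPlay caches the player and spawns one silent audio component, which PlayMusic reuses, fading out, swapping track, volume and pitch per music state, then fading in.
; PlayDialogue plays a voice line at the speaker behind a DoOnce gate, names the speaker by class cast, and steps through the sound's subtitles with delays, feeding log and HUD.
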(event Custom|PlayDialogue
  (params (Speaker :type Actor%20Object%20Reference) (Dialogue :type Sound%20Wave%20Object%20Reference))
  (bind _player (Variables|Default|GetPlayer))
  (bind _ingamehud (Variables|/Game/Prototype/GameMode/BP_3DCharacter_P.BP_3DCharacter_P_C|GetInGameHUD _player))
  ;[0.15 0.15 0.15 0.5] Dialogue System
  (Utilities|IsValid (Variables|Default|GetDialogue)
    (:Is%20Not%20Valid
      (Utilities|FlowControl|DoOnce false :!label _label
        (:Completed
          (bind _output_get (Variables|Default|SetDialogue Dialogue))
          (Audio|PlaySoundatLocation _output_get (Transformation|GetActorLocation Speaker) "0, 0, 0" 1.0 1.0 0.0 "/Game/GD12_3D/Audio/Attenuation/ATT_Character.ATT_Character" 0 Speaker 0)
          (Utilities|FlowControl|Sequence
            (:then_0
              (Utilities|Casting|CastToBP_3DCharacter_P Speaker)
              (bind _output_get_2 (Variables|/Game/Prototype/GameMode/BP_3DCharacter_P.BP_3DCharacter_P_C|SetDialogueSpeaker _player "Abel Eden"))
              (for _array_element (Variables|/Script/Engine.SoundWave|GetSubtitles Dialogue)
                (bind _output_get_3 (Variables|/Game/Prototype/GameMode/BP_3DCharacter_P.BP_3DCharacter_P_C|SetDialogueContent _player (Utilities|String|ToString(Text) (.text _array_element))))
                (Default|SetLog _player true _output_get_2 _output_get_3)
                (Default|ShowDialogue _ingamehud (Utilities|String|Append _output_get_2 ": " _output_get_3) (.time _array_element))
                (Utilities|FlowControl|Delay (.time _array_element))
                (goto _label Reset)))
            (:then_1
              (Utilities|Casting|CastToBP_AI_SecurityManager Speaker)
              (bind _output_get_4 (Variables|/Game/Prototype/GameMode/BP_3DCharacter_P.BP_3DCharacter_P_C|SetDialogueSpeaker _player "Mr. Judas"))
              (for _array_element_2 (Variables|/Script/Engine.SoundWave|GetSubtitles Dialogue)
                (bind _output_get_5 (Variables|/Game/Prototype/GameMode/BP_3DCharacter_P.BP_3DCharacter_P_C|SetDialogueContent _player (Utilities|String|ToString(Text) (.text _array_element_2))))
                (Default|SetLog _player true _output_get_4 _output_get_5)
                (Default|ShowDialogue _ingamehud (Utilities|String|Append _output_get_4 ": " _output_get_5) (.time _array_element_2))
                (Utilities|FlowControl|Delay (.time _array_element_2))
                (goto _label Reset)))
            (:then_2
              (Utilities|Casting|CastToBP_AI_FirstBoss Speaker)
              (bind _output_get_6 (Variables|/Game/Prototype/GameMode/BP_3DCharacter_P.BP_3DCharacter_P_C|SetDialogueSpeaker _player "Ms. Lailah"))
              (for _array_element_3 (Variables|/Script/Engine.SoundWave|GetSubtitles Dialogue)
                (bind _output_get_7 (Variables|/Game/Prototype/GameMode/BP_3DCharacter_P.BP_3DCharacter_P_C|SetDialogueContent _player (Utilities|String|ToString(Text) (.text _array_element_3))))
                (Default|SetLog _player true _output_get_6 _output_get_7)
                (Default|ShowDialogue _ingamehud (Utilities|String|Append _output_get_6 ": " _output_get_7) (.time _array_element_3))
                (Utilities|FlowControl|Delay (.time _array_element_3))
                (goto _label Reset)))))))))

(event Custom|PlayMusic
  (params (GameState :type E_GameStateType%20Enum :default "NewEnumerator0") (Volume :type Float%20%28single-precision%29) (Pitch :type Float%20%28single-precision%29))
  (bind _transduration (Variables|Default|GetTransDuration))
  (bind _returnvalue (- _transduration 0.5))
  ;[0.15 0.15 0.15 0.5] Background Music Sysytem
  (Utilities|IsValid (Variables|Default|GetBackgroundMusic)
    (:Is%20Valid
      (switch Utilities|FlowControl|Switch|SwitchonE_GameStateType GameState
        (:NewEnumerator0
          (Audio|Components|Audio|FadeOut (Variables|Default|GetBackgroundMusic) _transduration 0.0 "Linear" :!class /Script/Engine.AudioComponent)
          (Utilities|FlowControl|Delay _returnvalue)
          (Audio|Components|Audio|SetVolumeMultiplier (Variables|Default|GetBackgroundMusic) Volume :!class /Script/Engine.AudioComponent)
          (Audio|Components|Audio|SetPitchMultiplier (Variables|Default|GetBackgroundMusic) Pitch)
          (Audio|Components|Audio|SetSound (Variables|Default|GetBackgroundMusic) "/Game/GD12_3D/Audio/Music/A_SpaceDrift.A_SpaceDrift")
          (Audio|Components|Audio|FadeIn (Variables|Default|GetBackgroundMusic) _transduration 1.0 0.0 "Linear" :!class /Script/Engine.AudioComponent))
        (:NewEnumerator1
          (Audio|Components|Audio|FadeOut (Variables|Default|GetBackgroundMusic) _transduration 0.0 "Linear" :!class /Script/Engine.AudioComponent)
          (Utilities|FlowControl|Delay _returnvalue)
          (Audio|Components|Audio|SetVolumeMultiplier (Variables|Default|GetBackgroundMusic) Volume :!class /Script/Engine.AudioComponent)
          (Audio|Components|Audio|SetPitchMultiplier (Variables|Default|GetBackgroundMusic) Pitch)
          (Audio|Components|Audio|SetSound (Variables|Default|GetBackgroundMusic) "/Game/GD12_3D/Audio/Music/A_SpaceDrift_CreepyPoly.A_SpaceDrift_CreepyPoly")
          (Audio|Components|Audio|FadeIn (Variables|Default|GetBackgroundMusic) _transduration 1.0 0.0 "Linear" :!class /Script/Engine.AudioComponent))
        (:NewEnumerator7
          (Audio|Components|Audio|FadeOut (Variables|Default|GetBackgroundMusic) _transduration 0.0 "Linear" :!class /Script/Engine.AudioComponent)
          (Utilities|FlowControl|Delay _returnvalue)
          (Audio|Components|Audio|SetVolumeMultiplier (Variables|Default|GetBackgroundMusic) Volume :!class /Script/Engine.AudioComponent)
          (Audio|Components|Audio|SetPitchMultiplier (Variables|Default|GetBackgroundMusic) Pitch)
          (Audio|Components|Audio|SetSound (Variables|Default|GetBackgroundMusic) "/Game/GD12_3D/Audio/Music/A_SpaceDrift_CalmPoly.A_SpaceDrift_CalmPoly")
          (Audio|Components|Audio|FadeIn (Variables|Default|GetBackgroundMusic) _transduration 1.0 0.0 "Linear" :!class /Script/Engine.AudioComponent))
        (:NewEnumerator5
          (Audio|Components|Audio|FadeOut (Variables|Default|GetBackgroundMusic) _transduration 0.0 "Linear" :!class /Script/Engine.AudioComponent)
          (Utilities|FlowControl|Delay _returnvalue)
          (Audio|Components|Audio|SetVolumeMultiplier (Variables|Default|GetBackgroundMusic) Volume :!class /Script/Engine.AudioComponent)
          (Audio|Components|Audio|SetPitchMultiplier (Variables|Default|GetBackgroundMusic) Pitch)
          (Audio|Components|Audio|SetSound (Variables|Default|GetBackgroundMusic) "/Game/GD12_3D/Audio/Music/A_SpaceDrift_CorruptedPoly.A_SpaceDrift_CorruptedPoly")
          (Audio|Components|Audio|FadeIn (Variables|Default|GetBackgroundMusic) _transduration 1.0 0.0 "Linear" :!class /Script/Engine.AudioComponent))
        (:NewEnumerator6
          (Audio|Components|Audio|FadeOut (Variables|Default|GetBackgroundMusic) _transduration 0.0 "Linear" :!class /Script/Engine.AudioComponent)
          (Utilities|FlowControl|Delay _returnvalue)
          (Audio|Components|Audio|SetVolumeMultiplier (Variables|Default|GetBackgroundMusic) Volume :!class /Script/Engine.AudioComponent)
          (Audio|Components|Audio|SetPitchMultiplier (Variables|Default|GetBackgroundMusic) Pitch)
          (Audio|Components|Audio|SetSound (Variables|Default|GetBackgroundMusic) "/Game/GD12_3D/Audio/Music/A_SpaceDrift_Pads.A_SpaceDrift_Pads")
          (Audio|Components|Audio|FadeIn (Variables|Default|GetBackgroundMusic) _transduration 1.0 0.0 "Linear" :!class /Script/Engine.AudioComponent))
        (:NewEnumerator2
          (Audio|Components|Audio|FadeOut (Variables|Default|GetBackgroundMusic) _transduration 0.0 "Linear" :!class /Script/Engine.AudioComponent)
          (Utilities|FlowControl|Delay _returnvalue)
          (Audio|Components|Audio|SetVolumeMultiplier (Variables|Default|GetBackgroundMusic) Volume :!class /Script/Engine.AudioComponent)
          (Audio|Components|Audio|SetPitchMultiplier (Variables|Default|GetBackgroundMusic) Pitch)
          (Audio|Components|Audio|SetSound (Variables|Default|GetBackgroundMusic) "/Game/GD12_3D/Audio/Music/A_SpaceDrift_Drum.A_SpaceDrift_Drum")
          (Audio|Components|Audio|FadeIn (Variables|Default|GetBackgroundMusic) _transduration 1.0 0.0 "Linear" :!class /Script/Engine.AudioComponent))
        (:NewEnumerator3
          (Audio|Components|Audio|FadeOut (Variables|Default|GetBackgroundMusic) _transduration 0.0 "Linear" :!class /Script/Engine.AudioComponent)
          (Utilities|FlowControl|Delay _returnvalue)
          (Audio|Components|Audio|SetVolumeMultiplier (Variables|Default|GetBackgroundMusic) Volume :!class /Script/Engine.AudioComponent)
          (Audio|Components|Audio|SetPitchMultiplier (Variables|Default|GetBackgroundMusic) Pitch)
          (Audio|Components|Audio|SetSound (Variables|Default|GetBackgroundMusic) "/Game/GD12_3D/Audio/Music/A_SpaceDrift_PolyFocus.A_SpaceDrift_PolyFocus")
          (Audio|Components|Audio|FadeIn (Variables|Default|GetBackgroundMusic) _transduration 1.0 0.0 "Linear" :!class /Script/Engine.AudioComponent))
        (:NewEnumerator10
          (Audio|Components|Audio|FadeOut (Variables|Default|GetBackgroundMusic) _transduration 0.0 "Linear" :!class /Script/Engine.AudioComponent)
          (Utilities|FlowControl|Delay _returnvalue)
          (Audio|Components|Audio|SetVolumeMultiplier (Variables|Default|GetBackgroundMusic) Volume :!class /Script/Engine.AudioComponent)
          (Audio|Components|Audio|SetPitchMultiplier (Variables|Default|GetBackgroundMusic) Pitch)
          (Audio|Components|Audio|SetSound (Variables|Default|GetBackgroundMusic) "/Game/GD12_3D/Audio/Music/A_SearchAndRescue_Loop_01.A_SearchAndRescue_Loop_01")
          (Audio|Components|Audio|FadeIn (Variables|Default|GetBackgroundMusic) _transduration 1.0 0.0 "Linear" :!class /Script/Engine.AudioComponent))
        (:NewEnumerator4
          (Audio|Components|Audio|FadeOut (Variables|Default|GetBackgroundMusic) _transduration 0.0 "Linear" :!class /Script/Engine.AudioComponent)
          (Utilities|FlowControl|Delay _returnvalue)
          (Audio|Components|Audio|SetVolumeMultiplier (Variables|Default|GetBackgroundMusic) Volume :!class /Script/Engine.AudioComponent)
          (Audio|Components|Audio|SetPitchMultiplier (Variables|Default|GetBackgroundMusic) Pitch)
          (Audio|Components|Audio|SetSound (Variables|Default|GetBackgroundMusic) "/Game/GD12_3D/Audio/Music/A_SpaceDrift_NoDrums.A_SpaceDrift_NoDrums")
          (Audio|Components|Audio|FadeIn (Variables|Default|GetBackgroundMusic) _transduration 1.0 0.0 "Linear" :!class /Script/Engine.AudioComponent))
        (:NewEnumerator9
          (Audio|Components|Audio|FadeOut (Variables|Default|GetBackgroundMusic) _transduration 0.0 "Linear" :!class /Script/Engine.AudioComponent)
          (Utilities|FlowControl|Delay _returnvalue)
          (Audio|Components|Audio|SetVolumeMultiplier (Variables|Default|GetBackgroundMusic) 0.0 :!class /Script/Engine.AudioComponent)
          (Audio|Components|Audio|SetPitchMultiplier (Variables|Default|GetBackgroundMusic) 0.0)
          (Audio|Components|Audio|SetSound (Variables|Default|GetBackgroundMusic) "/Game/GD12_3D/Audio/SoundWaves/Prompt/A_Loop_Beep_SourceRecordings.A_Loop_Beep_SourceRecordings")
          (Audio|Components|Audio|FadeIn (Variables|Default|GetBackgroundMusic) _transduration 1.0 0.0 "Linear" :!class /Script/Engine.AudioComponent))))
    (:Is%20Not%20Valid
      (Utilities|FlowControl|DoOnce false) ; enters at Reset
    )))

(event EventBeginPlay
  (Utilities|FlowControl|Sequence
    (:then_0
      (bind _asbp_3dcharacter_p (Utilities|Casting|CastToBP_3DCharacter_P (Game|Player|GetPlayerPawn 0)))
      (Variables|Default|SetPlayer _asbp_3dcharacter_p))
    (:then_1
      ;[0.15 0.15 0.15 0.5] Background Music Sysytem
      (Utilities|FlowControl|DoOnce false
        (:Completed
          (bind _returnvalue (Audio|SpawnSound2D "/Game/GD12_3D/Audio/SoundWaves/Prompt/A_Loop_Beep_SourceRecordings.A_Loop_Beep_SourceRecordings" 0.0 1.0 0.0 0))
          (Variables|Default|SetBackgroundMusic _returnvalue))))))

(fn ConstructionScript)