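; BP_3DHUD_P is a prototype HUD Blueprint that puts the in-game HUD and main menu widgets on screen.
; TriggerGameHUD and TriggerMainMenu each create their widget, add it to the viewport with the menu at a higher Z-order, and store the reference.
; Both events show player 0's mouse cursor, and neither removes or checks for an existing widget.
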(event EventTriggerMainMenu
  (bind _returnvalue (Game|ConstructObjectfromClass "/Game/GD12_3D/UI/GameMenu/GameMain/WBP_MainMenu.WBP_MainMenu_C"))
  (UserInterface|Viewport|AddtoViewport _returnvalue 1)
  (Variables|Default|SetMainMenu _returnvalue)
  (Variables|/Script/Engine.PlayerController|SetbShowMouseCursor (Game|GetPlayerController 0) true))

(event EventTriggerGameHUD
  (bind _returnvalue (Game|ConstructObjectfromClass "/Game/GD12_3D/UI/GameMenu/GameMain/WBP_HUD_InGame.WBP_HUD_InGame_C"))
  (UserInterface|Viewport|AddtoViewport _returnvalue 0)
  (Variables|Default|SetIngameHUD _returnvalue)
  (Variables|/Script/Engine.PlayerController|SetbShowMouseCursor (Game|GetPlayerController 0) true))

(fn ConstructionScript)