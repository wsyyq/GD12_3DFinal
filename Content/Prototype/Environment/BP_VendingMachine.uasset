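; BP_VendingMachine is an interactable vending machine that reveals hidden content while the player is in hack mode.
; It binds to the player character's hack mode enter and end events, toggling the Secret, Reborn and Decal components and swapping its displayed name.
; An overlap trigger shows or hides the interact panel widget.
; Interacting fires a finish event, hides the panel's type label and returns a non-pickable result.
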(event OnComponentBeginOverlap(InteractTrigger)
  (params (OverlappedComponent :type Primitive%20Component%20Object%20Reference) (OtherActor :type Actor%20Object%20Reference) (OtherComp :type Primitive%20Component%20Object%20Reference) (OtherBodyIndex :type Integer) (bFromSweep :type Boolean) (SweepResult :type Hit%20Result%20Structure%20%28by%20ref%29))
  ;[0.15 0.15 0.15 0.5] WBP
  (Utilities|Casting|CastToBP_3DCharacter_P OtherActor)
  (Development|SetHiddeninGame (Variables|Default|GetInteractWidget) false false)
  (Default|ShowObjectType (.AsWBP%20Interact%20Panel (Utilities|Casting|CastToWBP_InteractPanel (UserInterface|GetWidget (Variables|Default|GetInteractWidget)))) "NewEnumerator10" "" (Variables|Default|GetNameOrBelong) false))

(event OnComponentEndOverlap(InteractTrigger)
  (params (OverlappedComponent :type Primitive%20Component%20Object%20Reference) (OtherActor :type Actor%20Object%20Reference) (OtherComp :type Primitive%20Component%20Object%20Reference) (OtherBodyIndex :type Integer))
  ;[0.15 0.15 0.15 0.5] WBP
  (Utilities|Casting|CastToBP_3DCharacter_P OtherActor)
  (Development|SetHiddeninGame (Variables|Default|GetInteractWidget) true false))

(event Custom|ChangeName
  (Variables|Default|SetNameOrBelong "Abel Eden")
  (Development|SetHiddeninGame (Variables|Default|GetSecret) false false)
  ;[0.15 0.15 0.15 0.5] WBP
  (Default|ShowObjectType (.AsWBP%20Interact%20Panel (Utilities|Casting|CastToWBP_InteractPanel (UserInterface|GetWidget (Variables|Default|GetInteractWidget)))) "NewEnumerator10" "" (Variables|Default|GetNameOrBelong) false))

(event Custom|ChangeNameAgain
  (Variables|Default|SetNameOrBelong "Verpp")
  (Development|SetHiddeninGame (Variables|Default|GetSecret) true false)
  ;[0.15 0.15 0.15 0.5] WBP
  (Default|ShowObjectType (.AsWBP%20Interact%20Panel (Utilities|Casting|CastToWBP_InteractPanel (UserInterface|GetWidget (Variables|Default|GetInteractWidget)))) "NewEnumerator10" "" (Variables|Default|GetNameOrBelong) false))

(event EventBeginPlay
  (Utilities|FlowControl|Sequence
    (:then_0
      (Development|SetHiddeninGame (Variables|Default|GetInteractWidget) true false)
      (Variables|Default|SetNameOrBelong "Verpp"))
    (:then_1
      (bind _asbp_3dcharacter_p (Utilities|Casting|CastToBP_3DCharacter_P (Game|Player|GetPlayerPawn 0)))
      (EventDispatchers|BindEventtoEnterHackMode _asbp_3dcharacter_p (delegate Custom|ChangeName))
      (EventDispatchers|BindEventtoEndHackMode _asbp_3dcharacter_p (delegate Custom|ChangeNameAgain)))))

(fn ConstructionScript)

(fn E2Interactive
  (Default|CallEventFinishInteract)
  (Default|HideObjectType (.AsWBP%20Interact%20Panel (Utilities|Casting|CastToWBP_InteractPanel (UserInterface|GetWidget (Variables|Default|GetInteractWidget)))))
  (return false "NewEnumerator10" 0 0 "" ""))