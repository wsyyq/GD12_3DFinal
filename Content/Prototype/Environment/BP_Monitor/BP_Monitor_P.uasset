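; BP_Monitor_P is a destructible surveillance monitor that raises an alarm when the player enters its sensing capsule.
; An alarm, throttled by a DoOnce, recolors the light, loops a siren for WarningDuration and sends its location to AI guards.
; A construction-sized AlertBox tracks which guards are in range to be notified.
; MonitorBeDestroyed disables detection, flickers the light out, triggers explosion effects and sound, and silences any active alarm.
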(event OnComponentBeginOverlap(AlertBox)
  (params (OverlappedComponent :type Primitive%20Component%20Object%20Reference) (OtherActor :type Actor%20Object%20Reference) (OtherComp :type Primitive%20Component%20Object%20Reference) (OtherBodyIndex :type Integer) (bFromSweep :type Boolean) (SweepResult :type Hit%20Result%20Structure%20%28by%20ref%29))
  ;[0.15 0.15 0.15 0.5] 通知范围内的敌人
  (bind _asbp_aiguard_p (Utilities|Casting|CastToBP_AIGuard_P OtherActor))
  (Utilities|Array|Add (Variables|Default|GetNoticeAIs) _asbp_aiguard_p))

(event OnComponentEndOverlap(AlertBox)
  (params (OverlappedComponent :type Primitive%20Component%20Object%20Reference) (OtherActor :type Actor%20Object%20Reference) (OtherComp :type Primitive%20Component%20Object%20Reference) (OtherBodyIndex :type Integer))
  ;[0.15 0.15 0.15 0.5] 通知范围内的敌人
  (bind _asbp_aiguard_p (Utilities|Casting|CastToBP_AIGuard_P OtherActor))
  (Utilities|Array|RemoveItem (Variables|Default|GetNoticeAIs) _asbp_aiguard_p))

(event OnComponentBeginOverlap(SensingPlayerCapsule)
  (params (OverlappedComponent :type Primitive%20Component%20Object%20Reference) (OtherActor :type Actor%20Object%20Reference) (OtherComp :type Primitive%20Component%20Object%20Reference) (OtherBodyIndex :type Integer) (bFromSweep :type Boolean) (SweepResult :type Hit%20Result%20Structure%20%28by%20ref%29))
  ;[0.15 0.15 0.15 0.5] 检测范围内的玩家
  (Utilities|Casting|CastToBP_3DCharacter_P OtherActor)
  (Utilities|FlowControl|DoOnce false :!label _label
    (:Completed
      (CallFunction|AlartandCallAI)
      (Utilities|FlowControl|Delay (+ (Variables|Default|GetWarningDuration) 1.0))
      (goto _label Reset))))

(event Custom|AlartAndCallAI
  ;[0.15 0.15 0.15 0.5] 灯光闪烁
  (Rendering|Components|Light|SetLightColor (Variables|Default|GetSensingAreaLight) (Variables|Default|GetSensingLightAlart) true)
  ;[0.15 0.15 0.15 0.5] 发出警报
  (bind _returnvalue (Audio|SpawnSoundatLocation "/Game/GD12_3D/Audio/SoundWaves/Prompt/A_Loop_Alarm_02.A_Loop_Alarm_02" (Transformation|GetActorLocation) "0, 0, 0" 1.0 1.0 0.0 "/Game/GD12_3D/Audio/Attenuation/ATT_Character.ATT_Character" 0))
  (Variables|Default|SetAlarmSound _returnvalue)
  ;[0.15 0.15 0.15 0.5] 通知AI
  (for _array_element (Variables|Default|GetNoticeAIs)
    (Class|BIAIAlartandMoveP|AIMovetoAlartPlace(Message) _array_element (Transformation|GetActorLocation)))
  ;[0.15 0.15 0.15 0.5] 结束警报
  (Utilities|FlowControl|Delay (Variables|Default|GetWarningDuration))
  (Class|AudioComponent|SetPaused _returnvalue true)
  (Components|DestroyComponent _returnvalue)
  (Rendering|Components|Light|SetLightColor (Variables|Default|GetSensingAreaLight) (Variables|Default|GetSensingLightNormal) true))

(event Custom|MonitorBeDestroyed
  (bind _ns_monitorboom (Variables|Default|GetNS_MonitorBoom))
  (bind _alarmsound (Variables|Default|GetAlarmSound))
  (Utilities|FlowControl|Sequence
    (:then_0
      ;[0.15 0.15 0.15 0.5] 不再通知AI
      (Utilities|Array|Clear (Variables|Default|GetNoticeAIs))
      (Collision|SetCollisionEnabled (Variables|Default|GetSensingPlayerCapsule) "NoCollision"))
    (:then_1
      ;[0.15 0.15 0.15 0.5] 不再发出警报
      (Collision|SetCollisionEnabled (Variables|Default|GetAlertBox) "NoCollision")
      (Variables|Default|SetIsBroken true))
    (:then_2
      ;[0.15 0.15 0.15 0.5] 灯光闪烁三次然后关闭
      (Rendering|Components|Light|SetIntensity (Variables|Default|GetSensingAreaLight) 0.0)
      (Utilities|FlowControl|Delay 0.4)
      (Rendering|Components|Light|SetIntensity (Variables|Default|GetSensingAreaLight) 5e+03)
      (Utilities|FlowControl|Delay 0.4)
      (Rendering|Components|Light|SetIntensity (Variables|Default|GetSensingAreaLight) 0.0)
      (Utilities|FlowControl|Delay 0.3)
      (Rendering|Components|Light|SetIntensity (Variables|Default|GetSensingAreaLight) 5e+03)
      (Utilities|FlowControl|Delay 0.3)
      (Rendering|Components|Light|SetIntensity (Variables|Default|GetSensingAreaLight) 0.0)
      (Utilities|FlowControl|Delay 0.2)
      (Rendering|Components|Light|SetIntensity (Variables|Default|GetSensingAreaLight) 5e+03)
      (Utilities|FlowControl|Delay 0.2)
      (Rendering|Components|Light|SetIntensity (Variables|Default|GetSensingAreaLight) 0.0)
      (Utilities|FlowControl|Delay 0.1)
      (Rendering|Components|Light|SetIntensity (Variables|Default|GetSensingAreaLight) 5e+03)
      (Utilities|FlowControl|Delay 0.1)
      (Rendering|Components|Light|SetIntensity (Variables|Default|GetSensingAreaLight) 0.0))
    (:then_3
      ;[0.15 0.15 0.15 0.5] 播放爆炸特效
      (Components|Activation|ToggleActive _ns_monitorboom)
      (Utilities|FlowControl|Delay 1.5)
      (Components|Activation|ToggleActive _ns_monitorboom))
    (:then_4
      ;[0.15 0.15 0.15 0.5] 播放爆炸音效
      (Audio|PlaySoundatLocation "/Game/Fab_Temporary/Sci-Fi_Shots_Pack2_Game_Of_Weapons/Cue/SC_MonitorBroken.SC_MonitorBroken" (Transformation|GetWorldLocation (Variables|Default|GetMonitor)) "0, 0, 0" 1.0 1.0 0.0 0 0 0 0))
    (:then_5
      ;[0.15 0.15 0.15 0.5] 如果有警报则关闭警报
      (Utilities|IsValid _alarmsound
        (:Is%20Valid
          (Class|AudioComponent|SetPaused _alarmsound true)
          (Components|DestroyComponent _alarmsound))))))

(event EventBeginPlay
  (Rendering|Components|Light|SetLightColor (Variables|Default|GetSensingAreaLight) (Variables|Default|GetSensingLightNormal) true)
  (Components|Activation|SetActive (Variables|Default|GetNS_MonitorBoom) false false))

(fn ConstructionScript
  (Components|Box|SetBoxExtent (Variables|Default|GetAlertBox) (Variables|Default|GetInBoxExtent) true))