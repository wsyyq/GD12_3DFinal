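; Spline-based placer that lays out a row of child actors, likely color-change cubes, along an editable spline.
; The Construction Script divides the spline length by CubeNum and adds a child actor component at each step, both endpoints included.
; Each component is positioned in actor-local space, then rotated to match the spline's world rotation.
; There is no runtime logic.
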(event EventBeginPlay)

(event EventTick
  (params (DeltaSeconds :type Float%20%28single-precision%29)))

(fn ConstructionScript
  (bind _cube_num (Variables|Default|Getcube%20num))
  (bind _spline (Variables|Default|GetSpline))
  (bind _returnvalue (- _cube_num 0))
  (for _index (range 0 _returnvalue)
    (bind _returnvalue_2 (AddComponent|AddChildActorComponent false (Math|Transform|MakeTransform (Math|Transform|InverseTransformLocation (Transformation|GetActorTransform) (Spline|GetLocationatDistanceAlongSpline _spline (Math|Conversions|ToFloat(Integer) (* _index (/ (Spline|GetSplineLength (Variables|Default|GetSpline)) (Math|Conversions|ToFloat(Integer) _returnvalue)))) "World")))))
    (Transformation|SetWorldRotation _returnvalue_2 (Spline|GetRotationatDistanceAlongSpline _spline (Math|Conversions|ToFloat(Integer) (* _index (/ (Spline|GetSplineLength (Variables|Default|GetSpline)) (Math|Conversions|ToFloat(Integer) _returnvalue)))) "World") false false)))