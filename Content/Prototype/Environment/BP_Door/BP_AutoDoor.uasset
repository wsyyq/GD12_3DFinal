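; BP_AutoDoor is a sliding double door that opens automatically for AI guards on common doors and by interaction for the player.
; Trigger overlaps drive guard access, player eligibility and the prompt widget, while Timelines lerp both panels to end markers.
; E2Interactive checks door type and keycards before toggling, with Keycard 2 doors offering password entry as fallback and staying unlocked after card use.
; The Construction Script sets keypad and frame visibility.
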(event OnComponentBeginOverlap(TriggerBox)
  (params (OverlappedComponent :type Primitive%20Component%20Object%20Reference) (OtherActor :type Actor%20Object%20Reference) (OtherComp :type Primitive%20Component%20Object%20Reference) (OtherBodyIndex :type Integer) (bFromSweep :type Boolean) (SweepResult :type Hit%20Result%20Structure%20%28by%20ref%29))
  ;[0.15 0.15 0.15 0.5] 敌人经过普通门时，门自动打开，离开自动关闭
  (Utilities|FlowControl|Sequence
    (:then_0
      (switch Utilities|FlowControl|Switch|SwitchonE_DoorType (Variables|Default|GetDoorType)
        (:NewEnumerator0
          (Utilities|Casting|CastToBP_AIGuard_P OtherActor
            (:then
              (if (and (not (Variables|Default|GetIsDoorOpen)) (not (Variables|Default|GetIsDoorOpening)))
                (CallFunction|DoorOpen)))
            (:CastFailed
              ;[0.15 0.15 0.15 0.5] 玩家接近时，允许开门
              (Utilities|Casting|CastToBP_3DCharacter_P OtherActor :!label _label)
              (Variables|Default|SetCanUseDoor true))))
        (:NewEnumerator1
          (goto _label))
        (:NewEnumerator2
          (goto _label))
        (:NewEnumerator3
          (goto _label))))
    (:then_1
      (Utilities|Casting|CastToBP_3DCharacter_P OtherActor)
      (if (not (Variables|Default|GetIsDoorOpening))
        (Development|SetHiddeninGame (Variables|Default|GetInteractWidget) false false)
        (Default|ShowObjectType (.AsWBP%20Interact%20Panel (Utilities|Casting|CastToWBP_InteractPanel (UserInterface|GetWidget (Variables|Default|GetInteractWidget)))) "" "NewEnumerator1")))))

(event OnComponentEndOverlap(TriggerBox)
  (params (OverlappedComponent :type Primitive%20Component%20Object%20Reference) (OtherActor :type Actor%20Object%20Reference) (OtherComp :type Primitive%20Component%20Object%20Reference) (OtherBodyIndex :type Integer))
  ;[0.15 0.15 0.15 0.5] 敌人经过普通门时，门自动打开，离开自动关闭
  (Utilities|FlowControl|Sequence
    (:then_0
      (switch Utilities|FlowControl|Switch|SwitchonE_DoorType (Variables|Default|GetDoorType)
        (:NewEnumerator0
          (Utilities|Casting|CastToBP_AIGuard_P OtherActor
            (:then
              (if (and (Variables|Default|GetIsDoorOpen) (not (Variables|Default|GetIsDoorOpening)))
                (CallFunction|DoorClose)))
            (:CastFailed
              ;[0.15 0.15 0.15 0.5] 玩家接近时，允许开门
              (Utilities|Casting|CastToBP_3DCharacter_P OtherActor :!label _label)
              (Variables|Default|SetCanUseDoor false))))
        (:NewEnumerator1
          (goto _label))
        (:NewEnumerator2
          (goto _label))
        (:NewEnumerator3
          (goto _label))))
    (:then_1
      (Utilities|Casting|CastToBP_3DCharacter_P OtherActor)
      (Development|SetHiddeninGame (Variables|Default|GetInteractWidget) true false))))

(event Custom|DoorClose
  ;[0.15 0.15 0.15 0.5] 开关门以及门状态切换
  (Variables|Default|SetIsDoorOpening true)
  (bind _newtrack_0 (Timeline|Timeline_CloseDoor PlayFromStart)
    (:Update
      (Transformation|SetRelativeLocation (Variables|Default|GetDoorRight) (Math|Vector|Lerp(Vector) (Variables|/Script/Engine.SceneComponent|GetRelativeLocation (Variables|Default|GetRightDoorEndPlace)) (Variables|Default|GetRightDoorRelativeLocation) _newtrack_0) false false)
      (Transformation|SetRelativeLocation (Variables|Default|GetDoorLeft) (Math|Vector|Lerp(Vector) (Variables|/Script/Engine.SceneComponent|GetRelativeLocation (Variables|Default|GetLeftDoorEndPlace)) (Variables|Default|GetLeftDoorRelativeLocation) _newtrack_0) false false))
    (:Finished
      (Variables|Default|SetIsDoorOpening false)
      (Variables|Default|SetIsDoorOpen false))))

(event Custom|DoorOpen
  ;[0.15 0.15 0.15 0.5] 开关门以及门状态切换
  (Variables|Default|SetIsDoorOpening true)
  (Variables|Default|SetRightDoorRelativeLocation (Variables|/Script/Engine.SceneComponent|GetRelativeLocation (Variables|Default|GetDoorRight)))
  (Variables|Default|SetLeftDoorRelativeLocation (Variables|/Script/Engine.SceneComponent|GetRelativeLocation (Variables|Default|GetDoorLeft)))
  (bind _newtrack_0 (Timeline|Timeline_OpenDoor PlayFromStart)
    (:Update
      (Transformation|SetRelativeLocation (Variables|Default|GetDoorRight) (Math|Vector|Lerp(Vector) (Variables|Default|GetRightDoorRelativeLocation) (Variables|/Script/Engine.SceneComponent|GetRelativeLocation (Variables|Default|GetRightDoorEndPlace)) _newtrack_0) false false)
      (Transformation|SetRelativeLocation (Variables|Default|GetDoorLeft) (Math|Vector|Lerp(Vector) (Variables|Default|GetLeftDoorRelativeLocation) (Variables|/Script/Engine.SceneComponent|GetRelativeLocation (Variables|Default|GetLeftDoorEndPlace)) _newtrack_0) false false))
    (:Finished
      (Variables|Default|SetIsDoorOpening false)
      (Variables|Default|SetIsDoorOpen true))))

(event Custom|ToggleDoor
  ;[0.15 0.15 0.15 0.5] 开关门以及门状态切换
  (if (Variables|Default|GetCanOpen)
    (if (not (Variables|Default|GetIsDoorOpening))
      (Utilities|FlowControl|Sequence
        (:then_0
          (Default|CallEventFinishInteract)
          (Default|HideObjectType (.AsWBP%20Interact%20Panel (Utilities|Casting|CastToWBP_InteractPanel (UserInterface|GetWidget (Variables|Default|GetInteractWidget)))))
          (if (Variables|Default|GetIsDoorOpen)
            (CallFunction|DoorClose)
            (else
              (CallFunction|DoorOpen)
              (Development|SetHiddeninGame (Variables|Default|GetInteractWidget) true false))))
        (:then_1
          (Audio|PlaySoundatLocation "/Game/GD12_3D/Audio/Cue/A_MetalDoor_Open_Cue.A_MetalDoor_Open_Cue" (Transformation|GetActorLocation) "0, 0, 0" 1.0 1.0 0.0 0 0 self 0))))))

(event EventBeginPlay
  ;[0.15 0.15 0.15 0.5] 开始游戏门默认关闭
  (Transformation|SetRelativeLocation (Variables|Default|GetDoorLeft) "0, 0, 0" false false)
  (Transformation|SetRelativeLocation (Variables|Default|GetDoorRight) "0, 0, 0" false false)
  (Development|SetHiddeninGame (Variables|Default|GetInteractWidget) true false))

(fn ConstructionScript
  (bind _doorframe (Variables|Default|GetDoorFrame))
  (bind _keypadl (Variables|Default|GetKeyPadL))
  (Utilities|FlowControl|Sequence
    (:then_0
      (switch Utilities|FlowControl|Switch|SwitchonE_DoorType (Variables|Default|GetDoorType)
        (:NewEnumerator0
          (Development|SetHiddeninGame _keypadl true false))
        (:NewEnumerator1
          (Development|SetHiddeninGame _keypadl false false :!label _label))
        (:NewEnumerator2
          (goto _label))
        (:NewEnumerator3
          (goto _label))))
    (:then_1
      (if (Variables|Default|GetHasFrame)
        (Development|SetHiddeninGame _doorframe false false)
        (else
          (Development|SetHiddeninGame _doorframe true false))))))

(fn E2Interactive
  (switch Utilities|FlowControl|Switch|SwitchonE_DoorType (Variables|Default|GetDoorType)
    (:NewEnumerator0
      (if (Variables|Default|GetCanUseDoor)
        _
        (else
          (return false "NewEnumerator1" self 0 "" ""))))
    (:NewEnumerator1
      (if (and (Variables|Default|GetCanUseDoor) (Variables|/Game/Prototype/GameMode/BP_3DCharacter_P.BP_3DCharacter_P_C|GetHasPassCard1 (.AsBP%203DCharacter%20P (Utilities|Casting|CastToBP_3DCharacter_P (Game|GetPlayerCharacter 0)))))
        _
        (else
          (return false "NewEnumerator1" self 0 "" ""))))
    (:NewEnumerator2
      ;[0.15 0.15 0.15 0.5] 是否已经打开过
      (if (Variables|Default|GetIsDoor2AlreadyOpen)
        _
        (else
          ;[0.15 0.15 0.15 0.5] 是否有门禁
          (if (and (Variables|Default|GetCanUseDoor) (Variables|/Game/Prototype/GameMode/BP_3DCharacter_P.BP_3DCharacter_P_C|GetHasPassCard2 (.AsBP%203DCharacter%20P (Utilities|Casting|CastToBP_3DCharacter_P (Game|GetPlayerCharacter 0)))))
            (Variables|Default|SetIsDoor2AlreadyOpen true)
            (else
              ;[0.15 0.15 0.15 0.5] 如果都没有，则默认按E打开输入密码界面
              (return false "NewEnumerator6" self (Variables|Default|GetDoorPassward) "" ""))))))
    (:NewEnumerator3
      (if (and (Variables|Default|GetCanUseDoor) (Variables|/Game/Prototype/GameMode/BP_3DCharacter_P.BP_3DCharacter_P_C|GetHasPassCard3 (.AsBP%203DCharacter%20P (Utilities|Casting|CastToBP_3DCharacter_P (Game|GetPlayerCharacter 0)))))
        _
        (else
          (return false "NewEnumerator1" self 0 "" "")))))
  (CallFunction|ToggleDoor)
  (return true "NewEnumerator1" self 0 "" ""))