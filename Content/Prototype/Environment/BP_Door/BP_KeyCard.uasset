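; BP_KeyCard is a keycard pickup that grants the player one of three pass cards (Boss, F2, F1), chosen by PassCardType.
; The construction script sets the card mesh and label text for that type.
; Overlapping PickTriggerBox by the player character shows an interact panel widget, hidden again on exit.
; E2Interactive hides the actor, disables its collision, gives the card to the player with a hint and reports it as picked.
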(event OnComponentBeginOverlap(PickTriggerBox)
  (params (OverlappedComponent :type Primitive%20Component%20Object%20Reference) (OtherActor :type Actor%20Object%20Reference) (OtherComp :type Primitive%20Component%20Object%20Reference) (OtherBodyIndex :type Integer) (bFromSweep :type Boolean) (SweepResult :type Hit%20Result%20Structure%20%28by%20ref%29))
  ;[0.15 0.15 0.15 0.5] WBP
  (Utilities|Casting|CastToBP_3DCharacter_P OtherActor)
  (Development|SetHiddeninGame (Variables|Default|GetInteractWidget) false false)
  (Default|ShowObjectType (.AsWBP%20Interact%20Panel (Utilities|Casting|CastToWBP_InteractPanel (UserInterface|GetWidget (Variables|Default|GetInteractWidget)))) "NewEnumerator9" "Keycard" (Variables|Default|GetNameOrBelong)))

(event OnComponentEndOverlap(PickTriggerBox)
  (params (OverlappedComponent :type Primitive%20Component%20Object%20Reference) (OtherActor :type Actor%20Object%20Reference) (OtherComp :type Primitive%20Component%20Object%20Reference) (OtherBodyIndex :type Integer))
  ;[0.15 0.15 0.15 0.5] WBP
  (Utilities|Casting|CastToBP_3DCharacter_P OtherActor)
  (Development|SetHiddeninGame (Variables|Default|GetInteractWidget) true false))

(event EventBeginPlay
  (|CallParentFunction))

(fn ConstructionScript
  (switch Utilities|FlowControl|Switch|SwitchonE_PassCardType (Variables|Default|GetPassCardType)
    (:NewEnumerator0
      (Components|StaticMesh|SetStaticMesh (Variables|Default|GetPickups) "/Game/Fab_Temporary/CC0_-_Magnet_Card/cc0_magnet_card.cc0_magnet_card")
      (Rendering|Components|TextRender|SetText (Variables|Default|GetObjectType) (Utilities|Text|ToText(String) "KeyCard1")))
    (:NewEnumerator1
      (Components|StaticMesh|SetStaticMesh (Variables|Default|GetPickups) "/Game/Fab_Temporary/CC0_-_Magnet_Card/cc0_magnet_card.cc0_magnet_card")
      (Rendering|Components|TextRender|SetText (Variables|Default|GetObjectType) (Utilities|Text|ToText(String) "KeyCard2")))
    (:NewEnumerator2
      (Components|StaticMesh|SetStaticMesh (Variables|Default|GetPickups) "/Game/Fab_Temporary/CC0_-_Magnet_Card/cc0_magnet_card.cc0_magnet_card")
      (Rendering|Components|TextRender|SetText (Variables|Default|GetObjectType) (Utilities|Text|ToText(String) "KeyCard3")))))

(fn E2Interactive
  (bind _returnvalue (Game|GetPlayerCharacter 0))
  (bind _asbp_3dcharacter_p (Utilities|Casting|CastToBP_3DCharacter_P _returnvalue))
  (switch Utilities|FlowControl|Switch|SwitchonE_PassCardType (Variables|Default|GetPassCardType)
    (:NewEnumerator0
      (Rendering|SetActorHiddenInGame true)
      (Collision|SetCollisionEnabled (Variables|Default|GetPickups) "NoCollision")
      (Collision|SetCollisionEnabled (Variables|Default|GetPickTriggerBox) "NoCollision")
      (Development|PrintString "拾取门禁1")
      (Default|GetPassCard _asbp_3dcharacter_p "NewEnumerator0")
      (Default|AddHint _asbp_3dcharacter_p "Keycard" (Utilities|String|ToString(Text) (Variables|Default|GetNameOrBelong)) false false)
      (Default|SetHint _asbp_3dcharacter_p)
      (return true "NewEnumerator9" 0 0 "" ""))
    (:NewEnumerator1
      (Rendering|SetActorHiddenInGame true)
      (Collision|SetCollisionEnabled (Variables|Default|GetPickups) "NoCollision")
      (Collision|SetCollisionEnabled (Variables|Default|GetPickTriggerBox) "NoCollision")
      (Development|PrintString "拾取门禁2")
      (Default|GetPassCard _asbp_3dcharacter_p "NewEnumerator1")
      (Default|AddHint _asbp_3dcharacter_p "Keycard" (Utilities|String|ToString(Text) (Variables|Default|GetNameOrBelong)) false false)
      (Default|SetHint _asbp_3dcharacter_p)
      (return true "NewEnumerator9" 0 0 "" ""))
    (:NewEnumerator2
      (Rendering|SetActorHiddenInGame true)
      (Collision|SetCollisionEnabled (Variables|Default|GetPickups) "NoCollision")
      (Collision|SetCollisionEnabled (Variables|Default|GetPickTriggerBox) "NoCollision")
      (Development|PrintString "拾取门禁3")
      (Default|GetPassCard _asbp_3dcharacter_p "NewEnumerator2")
      (Default|AddHint _asbp_3dcharacter_p "Keycard" (Utilities|String|ToString(Text) (Variables|Default|GetNameOrBelong)) false false)
      (Default|SetHint _asbp_3dcharacter_p)
      (return true "NewEnumerator9" 0 0 "" ""))))