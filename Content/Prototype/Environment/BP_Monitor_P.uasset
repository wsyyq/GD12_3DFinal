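; BP_Monitor_P is a prototype surveillance monitor that raises an alarm when the player enters its sensing capsule.
; A construction-sized alert box tracks overlapping guard AIs in a list.
; On detection it changes the light color, plays a looping alarm and sends listed guards its location, then reverts after a warning duration.
; A DoOnce that resets one second after the warning ends blocks overlapping alarms.
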(event OnComponentBeginOverlap(AlertBox)
  (params (OverlappedComponent :type Primitive%20Component%20Object%20Reference) (OtherActor :type Actor%20Object%20Reference) (OtherComp :type Primitive%20Component%20Object%20Reference) (OtherBodyIndex :type Integer) (bFromSweep :type Boolean) (SweepResult :type Hit%20Result%20Structure%20%28by%20ref%29))
  ;[0.15 0.15 0.15 0.5] 通知范围内的敌人
  (bind _asbp_aiguard_p (Utilities|Casting|CastToBP_AIGuard_P OtherActor))
  (Utilities|Array|Add (Variables|Default|GetNoticeAIs) _asbp_aiguard_p))

(event OnComponentEndOverlap(AlertBox)
  (params (OverlappedComponent :type Primitive%20Component%20Object%20Reference) (OtherActor :type Actor%20Object%20Reference) (OtherComp :type Primitive%20Component%20Object%20Reference) (OtherBodyIndex :type Integer))
  ;[0.15 0.15 0.15 0.5] 通知范围内的敌人
  (bind _asbp_aiguard_p (Utilities|Casting|CastToBP_AIGuard_P OtherActor))
  (Utilities|Array|RemoveItem (Variables|Default|GetNoticeAIs) _asbp_aiguard_p))

(event OnComponentBeginOverlap(SensingPlayerCapsule)
  (params (OverlappedComponent :type Primitive%20Component%20Object%20Reference) (OtherActor :type Actor%20Object%20Reference) (OtherComp :type Primitive%20Component%20Object%20Reference) (OtherBodyIndex :type Integer) (bFromSweep :type Boolean) (SweepResult :type Hit%20Result%20Structure%20%28by%20ref%29))
  ;[0.15 0.15 0.15 0.5] 检测范围内的玩家
  (Utilities|Casting|CastToBP_3DCharacter_P OtherActor)
  (Utilities|FlowControl|DoOnce false :!label _label
    (:Completed
      (CallFunction|AlartandCallAI)
      (Utilities|FlowControl|Delay (+ (Variables|Default|GetWarningDuration) 1.0))
      (goto _label Reset))))

(event Custom|AlartAndCallAI
  ;[0.15 0.15 0.15 0.5] 灯光闪烁
  (Rendering|Components|Light|SetLightColor (Variables|Default|GetSensingAreaLight) (Variables|Default|GetSensingLightAlart) true)
  ;[0.15 0.15 0.15 0.5] 发出警报
  (bind _returnvalue (Audio|SpawnSoundatLocation "/Game/GD12_3D/Audio/SoundWaves/Prompt/A_Loop_Alarm_02.A_Loop_Alarm_02" (Transformation|GetActorLocation) "0, 0, 0" 1.0 1.0 0.0 "/Game/GD12_3D/Audio/Attenuation/ATT_Character.ATT_Character" 0))
  ;[0.15 0.15 0.15 0.5] 通知AI
  (for _array_element (Variables|Default|GetNoticeAIs)
    (Class|BIAIAlartandMoveP|AIMovetoAlartPlace(Message) _array_element (Transformation|GetActorLocation)))
  ;[0.15 0.15 0.15 0.5] 结束警报
  (Utilities|FlowControl|Delay (Variables|Default|GetWarningDuration))
  (Class|AudioComponent|SetPaused _returnvalue true)
  (Components|DestroyComponent _returnvalue)
  (Rendering|Components|Light|SetLightColor (Variables|Default|GetSensingAreaLight) (Variables|Default|GetSensingLightNormal) true))

(event EventBeginPlay
  (Rendering|Components|Light|SetLightColor (Variables|Default|GetSensingAreaLight) (Variables|Default|GetSensingLightNormal) true))

(fn ConstructionScript
  (Components|Box|SetBoxExtent (Variables|Default|GetAlertBox) (Variables|Default|GetInBoxExtent) true))