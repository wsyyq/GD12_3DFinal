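; Prototype double sliding door that opens automatically for AI guards and toggles on player interaction.
; TriggerBox overlaps open or close it for BP_AIGuard_P and set CanUseDoor for BP_3DCharacter_P, which gates ToggleDoor in the E2Interactive function.
; Separate open and close timelines lerp both panels between their captured start positions and end-place components.
; IsDoorOpening blocks new requests during movement, so a guard leaving mid-opening leaves the door open.
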(event OnComponentBeginOverlap(TriggerBox)
  (params (OverlappedComponent :type Primitive%20Component%20Object%20Reference) (OtherActor :type Actor%20Object%20Reference) (OtherComp :type Primitive%20Component%20Object%20Reference) (OtherBodyIndex :type Integer) (bFromSweep :type Boolean) (SweepResult :type Hit%20Result%20Structure%20%28by%20ref%29))
  ;[0.15 0.15 0.15 0.5] 敌人经过时，门自动打开，离开自动关闭
  (Utilities|Casting|CastToBP_AIGuard_P OtherActor
    (:then
      (if (and (not (Variables|Default|GetIsDoorOpen)) (not (Variables|Default|GetIsDoorOpening)))
        (CallFunction|DoorOpen)))
    (:CastFailed
      ;[0.15 0.15 0.15 0.5] 玩家接近时，允许开门
      (Utilities|Casting|CastToBP_3DCharacter_P OtherActor)
      (Variables|Default|SetCanUseDoor true))))

(event OnComponentEndOverlap(TriggerBox)
  (params (OverlappedComponent :type Primitive%20Component%20Object%20Reference) (OtherActor :type Actor%20Object%20Reference) (OtherComp :type Primitive%20Component%20Object%20Reference) (OtherBodyIndex :type Integer))
  ;[0.15 0.15 0.15 0.5] 敌人经过时，门自动打开，离开自动关闭
  (Utilities|Casting|CastToBP_AIGuard_P OtherActor
    (:then
      (if (and (Variables|Default|GetIsDoorOpen) (not (Variables|Default|GetIsDoorOpening)))
        (CallFunction|DoorClose)))
    (:CastFailed
      ;[0.15 0.15 0.15 0.5] 玩家接近时，允许开门
      (Utilities|Casting|CastToBP_3DCharacter_P OtherActor)
      (Variables|Default|SetCanUseDoor false))))

(event Custom|DoorClose
  ;[0.15 0.15 0.15 0.5] 开关门以及门状态切换
  (Variables|Default|SetIsDoorOpening true)
  (bind _newtrack_0 (Timeline|Timeline_CloseDoor PlayFromStart)
    (:Update
      (Transformation|SetRelativeLocation (Variables|Default|GetRight_Door) (Math|Vector|Lerp(Vector) (Variables|/Script/Engine.SceneComponent|GetRelativeLocation (Variables|Default|GetRightDoorEndPlace)) (Variables|Default|GetRightDoorRelativeLocation) _newtrack_0) false false)
      (Transformation|SetRelativeLocation (Variables|Default|GetLeft_Door) (Math|Vector|Lerp(Vector) (Variables|/Script/Engine.SceneComponent|GetRelativeLocation (Variables|Default|GetLeftDoorEndPlace)) (Variables|Default|GetLeftDoorRelativeLocation) _newtrack_0) false false))
    (:Finished
      (Variables|Default|SetIsDoorOpening false)
      (Variables|Default|SetIsDoorOpen false))))

(event Custom|DoorOpen
  ;[0.15 0.15 0.15 0.5] 开关门以及门状态切换
  (Variables|Default|SetIsDoorOpening true)
  (Variables|Default|SetRightDoorRelativeLocation (Variables|/Script/Engine.SceneComponent|GetRelativeLocation (Variables|Default|GetRight_Door)))
  (Variables|Default|SetLeftDoorRelativeLocation (Variables|/Script/Engine.SceneComponent|GetRelativeLocation (Variables|Default|GetLeft_Door)))
  (bind _newtrack_0 (Timeline|Timeline_OpenDoor PlayFromStart)
    (:Update
      (Transformation|SetRelativeLocation (Variables|Default|GetRight_Door) (Math|Vector|Lerp(Vector) (Variables|Default|GetRightDoorRelativeLocation) (Variables|/Script/Engine.SceneComponent|GetRelativeLocation (Variables|Default|GetRightDoorEndPlace)) _newtrack_0) false false)
      (Transformation|SetRelativeLocation (Variables|Default|GetLeft_Door) (Math|Vector|Lerp(Vector) (Variables|Default|GetLeftDoorRelativeLocation) (Variables|/Script/Engine.SceneComponent|GetRelativeLocation (Variables|Default|GetLeftDoorEndPlace)) _newtrack_0) false false))
    (:Finished
      (Variables|Default|SetIsDoorOpening false)
      (Variables|Default|SetIsDoorOpen true))))

(event Custom|ToggleDoor
  ;[0.15 0.15 0.15 0.5] 开关门以及门状态切换
  (if (not (Variables|Default|GetIsDoorOpening))
    (if (Variables|Default|GetIsDoorOpen)
      (CallFunction|DoorClose)
      (else
        (CallFunction|DoorOpen)))))

(event EventBeginPlay
  ;[0.15 0.15 0.15 0.5] 开始游戏门默认关闭
  (Transformation|SetRelativeLocation (Variables|Default|GetLeft_Door) "-50.000000,0.000000,100.000000" false false)
  (Transformation|SetRelativeLocation (Variables|Default|GetRight_Door) "50.000000,0.000000,100.000000" false false))

(fn ConstructionScript)

(fn E2Interactive
  (if (Variables|Default|GetCanUseDoor)
    (CallFunction|ToggleDoor)
    (return false "NewEnumerator1")))