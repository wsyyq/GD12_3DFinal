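; BP_FallingItems_Kill is a falling carton box that damages characters it hits while falling.
; The construction script sets the carton box mesh on FallingItem.
; When Box begins an overlap and IsFalling is true, it applies 100 damage to a BP_3DCharacter_P, or to a BP_AI_Guard only if IsAIWorking returns true.
; IsFalling is only read here; the fall itself is not handled in these graphs.
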(event OnComponentBeginOverlap(Box)
  (params (OverlappedComponent :type Primitive%20Component%20Object%20Reference) (OtherActor :type Actor%20Object%20Reference) (OtherComp :type Primitive%20Component%20Object%20Reference) (OtherBodyIndex :type Integer) (bFromSweep :type Boolean) (SweepResult :type Hit%20Result%20Structure%20%28by%20ref%29))
  (if (Variables|Default|GetIsFalling)
    (bind _asbp_3dcharacter_p (Utilities|Casting|CastToBP_3DCharacter_P OtherActor)
      (:then
        (Game|Damage|ApplyDamage _asbp_3dcharacter_p 1e+02 (Game|GetInstigatorController) self))
      (:CastFailed
        (bind _asbp_ai_guard (Utilities|Casting|CastToBP_AI_Guard OtherActor))
        (if (Default|IsAIWorking _asbp_ai_guard)
          (Game|Damage|ApplyDamage _asbp_ai_guard 1e+02 (Game|GetInstigatorController) self))))))

(fn ConstructionScript
  (Components|StaticMesh|SetStaticMesh (Variables|Default|GetFallingItem) "/Game/Fab_Temporary/PS1_Office/Static_Mesh/CartonBox01/SM_Carton_Box.SM_Carton_Box"))