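; Falling item hazard that deals lethal-style damage to characters it hits.
; On Hit, it applies a large fixed damage to the 3D player character, or to an AI guard only while that guard reports its AI is working.
; Other actors are ignored, and the construction script only calls the parent's.
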(event Collision|EventHit
  (params (MyComp :type Primitive%20Component%20Object%20Reference) (Other :type Actor%20Object%20Reference) (OtherComp :type Primitive%20Component%20Object%20Reference) (bSelfMoved :type Boolean) (HitLocation :type Vector :default "0, 0, 0") (HitNormal :type Vector :default "0, 0, 0") (NormalImpulse :type Vector :default "0, 0, 0") (Hit :type Hit%20Result%20Structure%20%28by%20ref%29))
  (bind _asbp_3dcharacter_p (Utilities|Casting|CastToBP_3DCharacter_P Other)
    (:then
      (Game|Damage|ApplyDamage _asbp_3dcharacter_p 1e+02 (Game|GetInstigatorController) self))
    (:CastFailed
      (bind _asbp_aiguard_p (Utilities|Casting|CastToBP_AIGuard_P Other))
      (if (Default|IsAIWorking _asbp_aiguard_p)
        (Game|Damage|ApplyDamage _asbp_aiguard_p 1e+02 (Game|GetInstigatorController) self)))))

(fn ConstructionScript
  (|CallParentFunction))