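; BP_FallingItems is a falling prop that lures AI guards to investigate where it lands.
; AINoiseSensingBox maintains a NoticeAIs list of overlapping BP_AI_Guard actors.
; When FallingItem first overlaps NoiseEmitterBox, a DoOnce sends every valid listed guard to the actor's location via AIMoveToAlartPlace.
; IsFalling is then held true for FallingDuration before clearing.
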(event OnComponentBeginOverlap(NoiseEmitterBox)
  (params (OverlappedComponent :type Primitive%20Component%20Object%20Reference) (OtherActor :type Actor%20Object%20Reference) (OtherComp :type Primitive%20Component%20Object%20Reference) (OtherBodyIndex :type Integer) (bFromSweep :type Boolean) (SweepResult :type Hit%20Result%20Structure%20%28by%20ref%29))
  ;[0.15 0.15 0.15 0.5] 物体坠落后，AI向目标位置移动
  (if (== OtherComp (Variables|Default|GetFallingItem))
    (Utilities|FlowControl|DoOnce false
      (:Completed
        (Variables|Default|SetIsFalling true)
        (for _array_element (Variables|Default|GetNoticeAIs)
          (Utilities|IsValid _array_element
            (:Is%20Valid
              (Default|AIMovetoAlartPlace _array_element (Transformation|GetActorLocation)))))
        (Utilities|FlowControl|Delay (Variables|Default|GetFallingDuration))
        (Variables|Default|SetIsFalling false)))))

(event OnComponentBeginOverlap(AINoiseSensingBox)
  (params (OverlappedComponent :type Primitive%20Component%20Object%20Reference) (OtherActor :type Actor%20Object%20Reference) (OtherComp :type Primitive%20Component%20Object%20Reference) (OtherBodyIndex :type Integer) (bFromSweep :type Boolean) (SweepResult :type Hit%20Result%20Structure%20%28by%20ref%29))
  (bind _asbp_aiguard_p (Utilities|Casting|CastToBP_AI_Guard OtherActor))
  (Utilities|Array|Add (Variables|Default|GetNoticeAIs) _asbp_aiguard_p))

(event OnComponentEndOverlap(AINoiseSensingBox)
  (params (OverlappedComponent :type Primitive%20Component%20Object%20Reference) (OtherActor :type Actor%20Object%20Reference) (OtherComp :type Primitive%20Component%20Object%20Reference) (OtherBodyIndex :type Integer))
  (bind _asbp_aiguard_p (Utilities|Casting|CastToBP_AI_Guard OtherActor))
  (Utilities|Array|RemoveItem (Variables|Default|GetNoticeAIs) _asbp_aiguard_p))

(fn ConstructionScript)