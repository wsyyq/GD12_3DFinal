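; Configurable world pickup for health, ammo, currency, silencer, documents, keycards and other items, selected by InteractType.
; The construction script sets mesh, scale and label; overlapping the trigger box shows an interact widget to the player character.
; E2Interactive updates player stats or flags, using a shared capped-add helper for numeric items, hides collected items and returns type and document data.
; Scan events toggle custom depth on the mesh.
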(event OnComponentBeginOverlap(PickTriggerBox)
  (params (OverlappedComponent :type Primitive%20Component%20Object%20Reference) (OtherActor :type Actor%20Object%20Reference) (OtherComp :type Primitive%20Component%20Object%20Reference) (OtherBodyIndex :type Integer) (bFromSweep :type Boolean) (SweepResult :type Hit%20Result%20Structure%20%28by%20ref%29))
  (bind _interacttype (Variables|Config|GetInteractType))
  (bind _nameorbelong (Variables|Config|GetNameOrBelong))
  (bind _interactwidget (Variables|Default|GetInteractWidget))
  (bind _returnvalue (UserInterface|GetWidget _interactwidget))
  (bind _aswbp_interact_panel (Utilities|Casting|CastToWBP_InteractPanel _returnvalue))
  ;[0.15 0.15 0.15 0.5] WBP
  (Utilities|Casting|CastToBP_3DCharacter_P OtherActor)
  (Development|SetHiddeninGame (Variables|Default|GetInteractWidget) false false)
  (switch Utilities|FlowControl|Switch|SwitchonE_InteractType _interacttype
    (:NewEnumerator7
      (Default|ShowObjectType _aswbp_interact_panel _interacttype (Variables|Default|GetMedicine) _nameorbelong false))
    (:NewEnumerator15
      (Default|ShowObjectType _aswbp_interact_panel _interacttype (Variables|Default|GetEpi-pen) _nameorbelong false))
    (:NewEnumerator0
      (Default|ShowObjectType _aswbp_interact_panel _interacttype (Variables|Default|GetAmmo%20Kit) _nameorbelong false))
    (:NewEnumerator4
      (Default|ShowObjectType _aswbp_interact_panel _interacttype (Variables|Default|GetCredits) _nameorbelong false))
    (:NewEnumerator12
      (Default|ShowObjectType _aswbp_interact_panel _interacttype (Variables|Default|GetSilencer) _nameorbelong false))
    (:NewEnumerator5
      (Default|ShowObjectType _aswbp_interact_panel _interacttype (Variables|Default|GetDoc) _nameorbelong false))
    (:NewEnumerator9
      (Default|ShowObjectType _aswbp_interact_panel _interacttype (Variables|Default|GetKeycard) _nameorbelong false))
    (:NewEnumerator16
      (Default|ShowObjectType _aswbp_interact_panel _interacttype (Variables|Default|GetLandmine) _nameorbelong false))))

(event OnComponentEndOverlap(PickTriggerBox)
  (params (OverlappedComponent :type Primitive%20Component%20Object%20Reference) (OtherActor :type Actor%20Object%20Reference) (OtherComp :type Primitive%20Component%20Object%20Reference) (OtherBodyIndex :type Integer))
  ;[0.15 0.15 0.15 0.5] WBP
  (Utilities|Casting|CastToBP_3DCharacter_P OtherActor)
  (Development|SetHiddeninGame (Variables|Default|GetInteractWidget) true false))

(event Custom|CanNotBeScanned
  ;[0.15 0.15 0.15 0.5] 被扫描开关
  (Rendering|SetRenderCustomDepth (Variables|Default|GetPickups) false))

(event Custom|CanBeScanned
  ;[0.15 0.15 0.15 0.5] 被扫描开关
  (Rendering|SetRenderCustomDepth (Variables|Default|GetPickups) true))

(event EventBeginPlay
  (bind _interactwidget (Variables|Default|GetInteractWidget))
  (Utilities|FlowControl|Sequence
    (:then_0
      (Development|SetHiddeninGame (Variables|Default|GetInteractWidget) true false)
      (Development|SetHiddeninGame (Variables|Default|GetObjectType) true false))
    (:then_1
      (Utilities|IsValid _interactwidget
        (:Is%20Not%20Valid
          (bind _aswbp_interact_panel (Utilities|Casting|CastToWBP_InteractPanel (UserInterface|GetWidget _interactwidget)))
          (Variables|Config|SetInteractPanelWBP _aswbp_interact_panel))))))

(fn ConstructionScript
  (bind _pickups (Variables|Default|GetPickups))
  (bind _pickups_2 (Variables|Default|GetPickups))
  (bind _pickups_3 (Variables|Default|GetPickups))
  (bind _pickups_4 (Variables|Default|GetPickups))
  (bind _pickups_5 (Variables|Default|GetPickups))
  (bind _pickups_6 (Variables|Default|GetPickups))
  (bind _pickups_7 (Variables|Default|GetPickups))
  (bind _pickups_8 (Variables|Default|GetPickups))
  (bind _pickups_9 (Variables|Default|GetPickups))
  (bind _pickups_10 (Variables|Default|GetPickups))
  (bind _pickups_11 (Variables|Default|GetPickups))
  ;[0.15 0.15 0.15 0.5] 为每种可拾取物设置不同外观
  (switch Utilities|FlowControl|Switch|SwitchonE_InteractType (Variables|Config|GetInteractType)
    (:NewEnumerator7
      (Components|StaticMesh|SetStaticMesh _pickups_8 "/Game/GD12_3D/Environment/Meshes/SM_Meds.SM_Meds")
      (Transformation|SetWorldScale3D _pickups_8 "2.500000,2.500000,2.500000")
      (Rendering|Components|TextRender|SetText (Variables|Default|GetObjectType) (Variables|Default|GetMedicine)))
    (:NewEnumerator15
      (Components|StaticMesh|SetStaticMesh _pickups_10 "/Game/GD12_3D/Environment/Meshes/SM_Injector.SM_Injector")
      (Transformation|SetWorldScale3D _pickups_10 "1.750000,1.750000,1.750000")
      (Rendering|Components|TextRender|SetText (Variables|Default|GetObjectType) (Variables|Default|GetEpi-pen)))
    (:NewEnumerator0
      (Components|StaticMesh|SetStaticMesh _pickups "/Game/Fab_Temporary/7_62mm_ammo_box/bullets-box-7-62.bullets-box-7-62")
      (Transformation|SetWorldScale3D _pickups "1.250000,1.250000,1.250000")
      (Rendering|Components|TextRender|SetText (Variables|Default|GetObjectType) (Variables|Default|GetAmmo%20Kit)))
    (:NewEnumerator4
      (Components|StaticMesh|SetStaticMesh _pickups_11 "/Game/Fab_Temporary/SciFi_Props/Models/SM_Box_6.SM_Box_6")
      (Transformation|SetWorldScale3D _pickups_11 "0.250000,0.250000,0.250000")
      (Rendering|Components|TextRender|SetText (Variables|Default|GetObjectType) (Variables|Default|GetCredits)))
    (:NewEnumerator12
      (Components|StaticMesh|SetStaticMesh _pickups_7 "/Game/GD12_3D/Characters/Weapon/Pistol/SM_Silencer.SM_Silencer")
      (Transformation|SetWorldScale3D _pickups_7 "1.000000,1.000000,1.000000")
      (Rendering|Components|TextRender|SetText (Variables|Default|GetObjectType) (Variables|Default|GetSilencer))
      (Variables|Config|SetNameOrBelong "Verpp"))
    (:NewEnumerator5
      (switch Utilities|FlowControl|Switch|SwitchonE_MeshType (Variables|Config|GetDocType)
        (:NewEnumerator0
          (Components|StaticMesh|SetStaticMesh _pickups_4 "/Game/Fab_Temporary/Document_File_Folder/A4_Page3Shape_2_0.A4_Page3Shape_2_0")
          (Transformation|SetWorldScale3D _pickups_4 "0.150000,0.150000,0.150000")
          (Rendering|Components|TextRender|SetText (Variables|Default|GetObjectType) (Variables|Default|GetDoc)))
        (:NewEnumerator1
          (Components|StaticMesh|SetStaticMesh _pickups_5 "/Game/Fab_Temporary/Laptop__low-poly_/laptop_dell_xps.laptop_dell_xps")
          (Transformation|SetWorldScale3D _pickups_5 "0.100000,0.100000,0.100000")
          (Rendering|Components|TextRender|SetText (Variables|Default|GetObjectType) (Variables|Default|GetDoc)))
        (:NewEnumerator2
          (Components|StaticMesh|SetStaticMesh _pickups_9 "/Engine/BasicShapes/Plane.Plane")
          (Transformation|SetWorldScale3D _pickups_9 "0.200000,0.200000,0.200000")
          (Rendering|Components|TextRender|SetText (Variables|Default|GetObjectType) (Variables|Default|GetDoc))
          (Development|SetHiddeninGame _pickups_9 true false))))
    (:NewEnumerator9
      (Components|StaticMesh|SetStaticMesh _pickups_3 "/Game/Fab_Temporary/Computer_Card_Sci-Fi/computer_card_sci_fi.computer_card_sci_fi")
      (Transformation|SetWorldScale3D _pickups_3 "0.500000,0.500000,0.500000")
      (Rendering|Components|TextRender|SetText (Variables|Default|GetObjectType) (Variables|Default|GetKeycard)))
    (:NewEnumerator3
      (Components|StaticMesh|SetStaticMesh _pickups_2 "/Game/Fab_Temporary/Scifi_Box/scifi_box.scifi_box")
      (Transformation|SetWorldScale3D _pickups_2 "1.000000,1.000000,1.000000")
      (Rendering|Components|TextRender|SetText (Variables|Default|GetObjectType) (Variables|Default|GetSafe))
      (Variables|Config|SetNameOrBelong "Mr. Judas"))
    (:NewEnumerator16
      (Components|StaticMesh|SetStaticMesh _pickups_6 "/Game/Fab_Temporary/SciFi_Props/Models/SM_Box_7.SM_Box_7")
      (Transformation|SetWorldScale3D _pickups_6 "0.350000,0.350000,0.350000")
      (Rendering|Components|TextRender|SetText (Variables|Default|GetObjectType) (Variables|Default|GetLandmine))
      (Variables|Config|SetNameOrBelong "Abel Eden"))))

(fn PickUpHPKit
  (params (OriginHP :type Integer) (PlayerMaxHP :type Integer) (IsL :type Boolean))
  (if IsL
    (bind (_newnum _canpick) (Global|PickUpNum OriginHP PlayerMaxHP (Variables|Config|GetAddInjectorNum) "血量"))
    (return _newnum _canpick)
    (else
      (bind (_newnum_2 _canpick_2) (Global|PickUpNum OriginHP PlayerMaxHP (Variables|Config|GetAddMedNum) "血量"))
      (return _newnum_2 _canpick_2))))

(fn PickUpSPKit
  (params (OriginSP :type Integer) (PlayerMaxSP :type Integer))
  (bind (_newnum _canpick) (Global|PickUpNum OriginSP PlayerMaxSP (Variables|Config|GetAddSPNum) "蓝量"))
  (return _newnum _canpick))

(fn PickUpNum
  (params (OriginNum :type Integer) (MaxNum :type Integer) (AddNum :type Integer) (RelevantItemName :type String))
  (bind _returnvalue (+ OriginNum AddNum))
  (Development|PrintString (Utilities|String|Append "获得拾取物，现在 " RelevantItemName " 为：" (Utilities|String|ToString(Integer) OriginNum)))
  (Math|Integer|CompareInt OriginNum MaxNum
    (:>
      _)
    (:==
      _)
    (:<
      (Math|Integer|CompareInt _returnvalue MaxNum
        (:>
          _)
        (:==
          _)
        (:<
          ;[0.15 0.15 0.15 0.5] 回血后未超出满血
          (Development|PrintString (Utilities|String|Append "回" RelevantItemName "：" (Utilities|String|ToString(Integer) AddNum)))
          (Rendering|SetActorHiddenInGame true)
          (Collision|SetCollisionEnabled (Variables|Default|GetPickups) "NoCollision")
          (Collision|SetCollisionEnabled (Variables|Default|GetPickTriggerBox) "NoCollision")
          (Development|PrintString (Utilities|String|Append "现在" RelevantItemName "为：" (Utilities|String|ToString(Integer) _returnvalue)))
          (return _returnvalue true)))
      ;[0.15 0.15 0.15 0.5] 回血后超出满血
      (Development|PrintString (Utilities|String|Append "回" RelevantItemName "：" (Utilities|String|ToString(Integer) (- MaxNum OriginNum))))
      (Rendering|SetActorHiddenInGame true)
      (Collision|SetCollisionEnabled (Variables|Default|GetPickups) "NoCollision")
      (Collision|SetCollisionEnabled (Variables|Default|GetPickTriggerBox) "NoCollision")
      (Development|PrintString (Utilities|String|Append "现在" "" "为：" (Utilities|String|ToString(Integer) MaxNum)))
      (return MaxNum true)))
  ;[0.15 0.15 0.15 0.5] 满物品时候无法回物品
  (Development|PrintString (Utilities|String|Append RelevantItemName "已满，无法获得。"))
  (return OriginNum false))

(fn PickUpAmmoKit
  (params (OriginAmmo :type Integer) (PlayerMaxAmmo :type Integer))
  (bind (_newnum _canpick) (Global|PickUpNum OriginAmmo PlayerMaxAmmo (Variables|Config|GetAddAmmoBoxNum) "弹夹量"))
  (return _newnum _canpick))

(fn PickUpCurrencyKit
  (params (OriginCurrency :type Integer) (PlayerMaxCurrency :type Integer))
  (bind (_newnum _canpick) (Global|PickUpNum OriginCurrency PlayerMaxCurrency (Variables|Config|GetAddCurrencyNum) "货币量"))
  (return _newnum _canpick))

(fn E2Interactive
  (bind _returnvalue (Game|Player|GetPlayerPawn 0))
  (bind _returnvalue_2 (Game|GetPlayerCharacter 0))
  (bind _interactwidget (Variables|Default|GetInteractWidget))
  (bind _returnvalue_3 (UserInterface|GetWidget _interactwidget))
  (bind _asbp_3dcharacter_p (Utilities|Casting|CastToBP_3DCharacter_P _returnvalue_2))
  (bind _asbp_3dcharacter_p_2 (Utilities|Casting|CastToBP_3DCharacter_P _returnvalue))
  (bind _aswbp_interact_panel (Utilities|Casting|CastToWBP_InteractPanel _returnvalue_3))
  (switch Utilities|FlowControl|Switch|SwitchonE_InteractType (Variables|Config|GetInteractType)
    (:NewEnumerator7
      (bind (_newhpnum _canpick) (Local|PickUpHPKit (Variables|/Game/Prototype/GameMode/BP_3DCharacter_P.BP_3DCharacter_P_C|GetCurrentHP _asbp_3dcharacter_p) (Variables|/Game/Prototype/GameMode/BP_3DCharacter_P.BP_3DCharacter_P_C|GetMaxHP _asbp_3dcharacter_p) false))
      (Variables|/Game/Prototype/GameMode/BP_3DCharacter_P.BP_3DCharacter_P_C|SetCurrentHP _asbp_3dcharacter_p _newhpnum)
      (Default|CallEventFinishInteract)
      (Default|HideObjectType _aswbp_interact_panel)
      (Default|AddHint _asbp_3dcharacter_p_2 (Variables|Default|GetMedicine) (Utilities|String|ToString(Integer) (Variables|Config|GetAddMedNum)) false false)
      (Default|SetHint _asbp_3dcharacter_p_2)
      (return _canpick "NewEnumerator7" self 0 "" ""))
    (:NewEnumerator15
      (bind (_newhpnum_2 _canpick_2) (Local|PickUpHPKit (Variables|/Game/Prototype/GameMode/BP_3DCharacter_P.BP_3DCharacter_P_C|GetCurrentHP _asbp_3dcharacter_p) (Variables|/Game/Prototype/GameMode/BP_3DCharacter_P.BP_3DCharacter_P_C|GetMaxHP _asbp_3dcharacter_p) true))
      (Variables|/Game/Prototype/GameMode/BP_3DCharacter_P.BP_3DCharacter_P_C|SetCurrentHP _asbp_3dcharacter_p _newhpnum_2)
      (Default|CallEventFinishInteract)
      (Default|HideObjectType _aswbp_interact_panel)
      (Default|AddHint _asbp_3dcharacter_p_2 (Variables|Default|GetEpi-pen) (Utilities|String|ToString(Integer) (Variables|Config|GetAddInjectorNum)) false false)
      (Default|SetHint _asbp_3dcharacter_p_2)
      (return _canpick_2 "NewEnumerator15" self 0 "" ""))
    (:NewEnumerator0
      (bind (_newammonum _canpick_3) (Local|PickUpAmmoKit (Variables|/Game/Prototype/GameMode/BP_3DCharacter_P.BP_3DCharacter_P_C|GetCurrentAmmoBox _asbp_3dcharacter_p) (Variables|/Game/Prototype/GameMode/BP_3DCharacter_P.BP_3DCharacter_P_C|GetMaxAmmoBox _asbp_3dcharacter_p)))
      (Variables|/Game/Prototype/GameMode/BP_3DCharacter_P.BP_3DCharacter_P_C|SetCurrentAmmoBox _asbp_3dcharacter_p _newammonum)
      (Default|CallEventFinishInteract)
      (Default|HideObjectType _aswbp_interact_panel)
      (Default|AddHint _asbp_3dcharacter_p_2 (Variables|Default|GetAmmo%20Kit) (Utilities|String|ToString(Integer) (Variables|Config|GetAddAmmoBoxNum)) false false)
      (Default|SetHint _asbp_3dcharacter_p_2)
      (Default|CallChangeGunState _asbp_3dcharacter_p_2)
      (return _canpick_3 "NewEnumerator0" self 0 "" ""))
    (:NewEnumerator4
      (bind (_newcurrencynum _canpick_4) (Local|PickUpCurrencyKit (Variables|/Game/Prototype/GameMode/BP_3DCharacter_P.BP_3DCharacter_P_C|GetCurrentCurrency _asbp_3dcharacter_p) (Variables|/Game/Prototype/GameMode/BP_3DCharacter_P.BP_3DCharacter_P_C|GetMaxCurrency _asbp_3dcharacter_p)))
      (Variables|/Game/Prototype/GameMode/BP_3DCharacter_P.BP_3DCharacter_P_C|SetCurrentCurrency _asbp_3dcharacter_p _newcurrencynum)
      (Default|CallEventFinishInteract)
      (Default|HideObjectType _aswbp_interact_panel)
      (Default|AddHint _asbp_3dcharacter_p_2 (Variables|Default|GetCredits) (Utilities|String|ToString(Integer) (Variables|Config|GetAddCurrencyNum)) false false)
      (Default|SetHint _asbp_3dcharacter_p_2)
      (return _canpick_4 "NewEnumerator4" self 0 "" ""))
    (:NewEnumerator12
      (Rendering|SetActorHiddenInGame true)
      (Collision|SetCollisionEnabled (Variables|Default|GetPickups) "NoCollision")
      (Collision|SetCollisionEnabled (Variables|Default|GetPickTriggerBox) "NoCollision")
      (Default|CallEventFinishInteract)
      (Default|HideObjectType _aswbp_interact_panel)
      (Default|AddHint _asbp_3dcharacter_p_2 (Variables|Default|GetSilencer) (Utilities|String|ToString(Text) (Variables|Config|GetNameOrBelong)) false false)
      (Default|SetHint _asbp_3dcharacter_p_2)
      (return true "NewEnumerator12" self 0 "" ""))
    (:NewEnumerator5
      (Default|CallEventFinishInteract)
      (Default|HideObjectType _aswbp_interact_panel)
      (Default|AddHint _asbp_3dcharacter_p_2 (Variables|Default|GetDoc) (Utilities|String|ToString(Text) (Variables|Config|GetNameOrBelong)) false false)
      (Default|SetHint _asbp_3dcharacter_p_2)
      (return false "NewEnumerator5" self 0 (Variables|Config|GetDocArthur) (Variables|Config|GetDocContent)))
    (:NewEnumerator9
      (if (not (Variables|/Game/Prototype/GameMode/BP_3DCharacter_P.BP_3DCharacter_P_C|GetHasKeyCardL1 _asbp_3dcharacter_p))
        (Variables|/Game/Prototype/GameMode/BP_3DCharacter_P.BP_3DCharacter_P_C|SetHasKeyCardL1 _asbp_3dcharacter_p true)
        (Rendering|SetActorHiddenInGame true)
        (Collision|SetCollisionEnabled (Variables|Default|GetPickups) "NoCollision")
        (Collision|SetCollisionEnabled (Variables|Default|GetPickTriggerBox) "NoCollision")
        (Default|CallEventFinishInteract)
        (Default|HideObjectType _aswbp_interact_panel)
        (return true "NewEnumerator9" self 0 "" "")))
    (:NewEnumerator8
      (if (not (Variables|/Game/Prototype/GameMode/BP_3DCharacter_P.BP_3DCharacter_P_C|GetHasHackerChip _asbp_3dcharacter_p))
        (Variables|/Game/Prototype/GameMode/BP_3DCharacter_P.BP_3DCharacter_P_C|SetHasHackerChip _asbp_3dcharacter_p true)
        (Rendering|SetActorHiddenInGame true)
        (Collision|SetCollisionEnabled (Variables|Default|GetPickups) "NoCollision")
        (Collision|SetCollisionEnabled (Variables|Default|GetPickTriggerBox) "NoCollision")
        (Default|CallEventFinishInteract)
        (Default|HideObjectType _aswbp_interact_panel)
        (return true "NewEnumerator8" self 0 "" "")))
    (:NewEnumerator16
      (Rendering|SetActorHiddenInGame true)
      (Collision|SetCollisionEnabled (Variables|Default|GetPickups) "NoCollision")
      (Collision|SetCollisionEnabled (Variables|Default|GetPickTriggerBox) "NoCollision")
      (Default|CallEventFinishInteract)
      (CallFunction|HideObjectType)
      (Default|AddHint _asbp_3dcharacter_p_2 (Variables|Default|GetLandmine) (Utilities|String|ToString(Text) (Variables|Config|GetNameOrBelong)) false false)
      (Default|SetHint _asbp_3dcharacter_p_2)
      (return true "NewEnumerator16" self 0 "" ""))))