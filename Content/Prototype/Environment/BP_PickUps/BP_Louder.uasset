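; Interactable noise-maker prop that lures guards to its location, with a speaker, laptop or plane mesh chosen by LouderType.
; Player overlap shows an interact widget, and interacting through E2Interactive plays a looping sound, or fades an existing one back in, while enlarging the AISensor box.
; The sensor tracks overlapping BP_AI_Guard actors, which are sent to the prop shortly afterwards.
; A timed delay shrinks the sensor again if the sound is still playing.
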(event OnComponentBeginOverlap(PickTriggerBox)
  (params (OverlappedComponent :type Primitive%20Component%20Object%20Reference) (OtherActor :type Actor%20Object%20Reference) (OtherComp :type Primitive%20Component%20Object%20Reference) (OtherBodyIndex :type Integer) (bFromSweep :type Boolean) (SweepResult :type Hit%20Result%20Structure%20%28by%20ref%29))
  ;[0.15 0.15 0.15 0.5] WBP
  (Utilities|Casting|CastToBP_3DCharacter_P OtherActor)
  (Development|SetHiddeninGame (Variables|Default|GetInteractWidget) false false)
  (Default|ShowObjectType (.AsWBP%20Interact%20Panel (Utilities|Casting|CastToWBP_InteractPanel (UserInterface|GetWidget (Variables|Default|GetInteractWidget)))) "NewEnumerator17" "" "Verrp"))

(event OnComponentEndOverlap(PickTriggerBox)
  (params (OverlappedComponent :type Primitive%20Component%20Object%20Reference) (OtherActor :type Actor%20Object%20Reference) (OtherComp :type Primitive%20Component%20Object%20Reference) (OtherBodyIndex :type Integer))
  ;[0.15 0.15 0.15 0.5] WBP
  (Utilities|Casting|CastToBP_3DCharacter_P OtherActor)
  (Development|SetHiddeninGame (Variables|Default|GetInteractWidget) true false))

(event OnComponentBeginOverlap(AISensor)
  (params (OverlappedComponent :type Primitive%20Component%20Object%20Reference) (OtherActor :type Actor%20Object%20Reference) (OtherComp :type Primitive%20Component%20Object%20Reference) (OtherBodyIndex :type Integer) (bFromSweep :type Boolean) (SweepResult :type Hit%20Result%20Structure%20%28by%20ref%29))
  ;[0.15 0.15 0.15 0.5] AI Sensor
  (bind _asbp_ai_guard (Utilities|Casting|CastToBP_AI_Guard OtherActor))
  (Utilities|Array|Add (Variables|Default|GetSensingAIs) _asbp_ai_guard))

(event OnComponentEndOverlap(AISensor)
  (params (OverlappedComponent :type Primitive%20Component%20Object%20Reference) (OtherActor :type Actor%20Object%20Reference) (OtherComp :type Primitive%20Component%20Object%20Reference) (OtherBodyIndex :type Integer))
  ;[0.15 0.15 0.15 0.5] AI Sensor
  (bind _asbp_ai_guard (Utilities|Casting|CastToBP_AI_Guard OtherActor))
  (Utilities|Array|RemoveItem (Variables|Default|GetSensingAIs) _asbp_ai_guard))

(event Custom|PlayerInteract
  (Utilities|FlowControl|Sequence
    (:then_0
      (Utilities|FlowControl|DoOnce false
        (:Completed
          (Components|Box|SetBoxExtent (Variables|Default|GetAISensor) "500.000000,500.000000,250.000000" true)
          (bind _returnvalue (Audio|SpawnSoundatLocation "/Game/GD12_3D/Audio/Cue/A_Illusion_Loop_Cue.A_Illusion_Loop_Cue" (Transformation|GetActorLocation) "0, 0, 0" 1.0 1.0 0.0 0 0 :!label _label))
          (Variables|Default|SetLouder _returnvalue)
          (Utilities|FlowControl|Delay 21.0 :!label _label_2)
          (if (Audio|Components|Audio|IsPlaying (Variables|Default|GetLouder))
            (Components|Box|SetBoxExtent (Variables|Default|GetAISensor) "10.000000,10.000000,10.000000" true)))))
    (:then_1
      (Utilities|IsValid (Variables|Default|GetLouder)
        (:Is%20Valid
          (if (Audio|Components|Audio|IsPlaying (Variables|Default|GetLouder))
            (Audio|Components|Audio|FadeOut (Variables|Default|GetLouder) 0.5 0.0 "Linear" :!class /Script/Engine.AudioComponent)
            (Components|Box|SetBoxExtent (Variables|Default|GetAISensor) "10.000000,10.000000,10.000000" true)
            (Utilities|FlowControl|Delay 0.5))
          (Audio|Components|Audio|FadeIn (Variables|Default|GetLouder) 0.5 1.0 0.0 "Linear" :!class /Script/Engine.AudioComponent)
          (Components|Box|SetBoxExtent (Variables|Default|GetAISensor) "500.000000,500.000000,250.000000" true)
          (goto _label_2))
        (:Is%20Not%20Valid
          (goto _label))))
    (:then_2
      (Utilities|FlowControl|Delay 1.2)
      (for _array_element (Variables|Default|GetSensingAIs)
        (Utilities|IsValid _array_element
          (:Is%20Valid
            (Default|AIMovetoAlartPlace _array_element (Transformation|GetActorLocation))
            (Development|PrintString "Louder Make Noise."))
          (:Is%20Not%20Valid
            (Utilities|Array|RemoveItem (Variables|Default|GetSensingAIs) _array_element)))))))

(event EventBeginPlay
  (Development|SetHiddeninGame (Variables|Default|GetInteractWidget) true false))

(fn ConstructionScript
  (bind _staticmesh (Variables|Default|GetStaticMesh))
  (bind _staticmesh_2 (Variables|Default|GetStaticMesh))
  (bind _staticmesh_3 (Variables|Default|GetStaticMesh))
  (switch Utilities|FlowControl|Switch|SwitchonE_MeshType (Variables|Default|GetLouderType)
    (:NewEnumerator0
      (Components|StaticMesh|SetStaticMesh _staticmesh "/Game/Fab_Temporary/Hi-Fi_Speaker/hi_fi_speaker.hi_fi_speaker")
      (Transformation|SetWorldScale3D _staticmesh "0.250000,0.250000,0.250000"))
    (:NewEnumerator1
      (Components|StaticMesh|SetStaticMesh _staticmesh_3 "/Game/Fab_Temporary/Laptop__low-poly_/laptop_dell_xps.laptop_dell_xps")
      (Transformation|SetWorldScale3D _staticmesh_3 "0.100000,0.100000,0.100000"))
    (:NewEnumerator2
      (Components|StaticMesh|SetStaticMesh _staticmesh_2 "/Engine/BasicShapes/Plane.Plane")
      (Transformation|SetWorldScale3D _staticmesh_2 "0.200000,0.200000,0.200000"))))

(fn E2Interactive
  (Default|HideObjectType (.AsWBP%20Interact%20Panel (Utilities|Casting|CastToWBP_InteractPanel (UserInterface|GetWidget (Variables|Default|GetInteractWidget)))))
  (CallFunction|PlayerInteract)
  (Default|CallEventFinishInteract)
  (return false "NewEnumerator17" self 0 "" ""))