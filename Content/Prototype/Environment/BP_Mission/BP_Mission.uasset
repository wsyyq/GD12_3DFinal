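; BP_Mission is a placeable mission objective of type Kill, Interact or Reach, hidden until started.
; BeginPlay binds completion to the kill target's death or the interact target's finish event, using a cast chain over interactable classes.
; Starting shows the logo, which turns toward the player's camera boom, and enables the overlap box for Reach.
; Completion hides the logo, disables the box and broadcasts mission success.
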(event OnComponentBeginOverlap(Box)
  (params (OverlappedComponent :type Primitive%20Component%20Object%20Reference) (OtherActor :type Actor%20Object%20Reference) (OtherComp :type Primitive%20Component%20Object%20Reference) (OtherBodyIndex :type Integer) (bFromSweep :type Boolean) (SweepResult :type Hit%20Result%20Structure%20%28by%20ref%29))
  ;[0.15 0.15 0.15 0.5] 到达目标任务完成
  (switch Utilities|FlowControl|Switch|SwitchonE_Mission (Variables|Default|GetMissionType)
    (:NewEnumerator0
      (Utilities|Casting|CastToBP_3DCharacter_P OtherActor)
      (Utilities|FlowControl|DoOnce false
        (:Completed
          (CallFunction|MissionSuccessandHideThisorGameStart))))))

(event Custom|MissionSuccess_Kill
  ;[0.15 0.15 0.15 0.5] 击杀目标任务完成
  (CallFunction|MissionSuccessandHideThisorGameStart))

(event Custom|MissionSuccess_Interact
  ;[0.15 0.15 0.15 0.5] 交互目标任务完成
  (CallFunction|MissionSuccessandHideThisorGameStart))

(event EventBeginPlay
  (bind _interacttarget (Variables|Default|GetInteractTarget))
  ;[0.15 0.15 0.15 0.5] 开始游戏时任务隐藏
  (Rendering|SetVisibility (Variables|Default|GetMissionLogo) false false)
  (Collision|SetCollisionEnabled (Variables|Default|GetBox) "NoCollision")
  (switch Utilities|FlowControl|Switch|SwitchonE_Mission (Variables|Default|GetMissionType)
    (:NewEnumerator1
      (EventDispatchers|BindEventtoEventAIDie (Variables|Default|GetKillTarget) (delegate Custom|MissionSuccess_Kill)))
    (:NewEnumerator2
      (if (Utilities|DoesObjectImplementInterface _interacttarget "/Game/Prototype/Environment/BI_Interactive.BI_Interactive_C")
        (bind _asbp_auto_door (Utilities|Casting|CastToBP_AutoDoor _interacttarget)
          (:then
            (EventDispatchers|BindEventtoEventFinishInteract _asbp_auto_door (delegate Custom|MissionSuccess_Interact)))
          (:CastFailed
            (bind _asbp_pickups (Utilities|Casting|CastToBP_Pickups _interacttarget)
              (:then
                (EventDispatchers|BindEventtoEventFinishInteract _asbp_pickups (delegate Custom|MissionSuccess_Interact)))
              (:CastFailed
                (bind _asbp_elevator_parent (Utilities|Casting|CastToBP_Elevator_Parent _interacttarget)
                  (:then
                    (EventDispatchers|BindEventtoEventFinishInteract _asbp_elevator_parent (delegate Custom|MissionSuccess_Interact)))
                  (:CastFailed
                    (bind _asbp_abel_chip_p (Utilities|Casting|CastToBP_AbelChip _interacttarget)
                      (:then
                        (EventDispatchers|BindEventtoEventFinishInteract _asbp_abel_chip_p (delegate Custom|MissionSuccess_Interact)))
                      (:CastFailed
                        (bind _asbp_abel_reborn (Utilities|Casting|CastToBP_AbelReborn _interacttarget)
                          (:then
                            (EventDispatchers|BindEventtoEventFinishInteract _asbp_abel_reborn (delegate Custom|MissionSuccess_Interact)))
                          (:CastFailed
                            (bind _asbp_vending_machine (Utilities|Casting|CastToBP_VendingMachine _interacttarget)
                              (:then
                                (EventDispatchers|BindEventtoEventFinishInteract _asbp_vending_machine (delegate Custom|MissionSuccess_Interact)))
                              (:CastFailed
                                (bind _asbp_pistol_pickup (Utilities|Casting|CastToBP_Pistol_Pickup _interacttarget))
                                (EventDispatchers|BindEventtoEventFinishInteract _asbp_pistol_pickup (delegate Custom|MissionSuccess_Interact))))))))))))))
        (else
          (Development|PrintString "任务目标非可交互物"))))))

(event EventTick
  (params (DeltaSeconds :type Float%20%28single-precision%29))
  ;[0.15 0.15 0.15 0.5] WBP面向玩家
  (if (Variables|Default|GetIsMissionStart)
    (Transformation|SetWorldRotation (Variables|Default|GetMissionLogo) (Math|Rotator|FindLookatRotation (Transformation|GetActorLocation) (Transformation|GetWorldLocation (Variables|/Game/Prototype/GameMode/BP_3DCharacter_P.BP_3DCharacter_P_C|GetCameraBoom (.AsBP%203DCharacter%20P (Utilities|Casting|CastToBP_3DCharacter_P (Game|Player|GetPlayerPawn 0)))))) false false)))

(fn ConstructionScript)

(fn MissionSuccessandHideThisorGameStart
  ;[0.15 0.15 0.15 0.5] 任务成功，标志消失
  (Rendering|SetVisibility (Variables|Default|GetMissionLogo) false false)
  (Collision|SetCollisionEnabled (Variables|Default|GetBox) "NoCollision")
  (Development|PrintString (Utilities|String|Append "任务（" (Variables|Default|GetMissionSub) "）结束"))
  (Variables|Default|SetIsMissionStart false)
  (Variables|Default|SetIsMissionSuccess false)
  (Default|CallMissionSuccess))

(fn MissionStartandShowThis
  ;[0.15 0.15 0.15 0.5] 任务出现
  (Rendering|SetVisibility (Variables|Default|GetMissionLogo) true false)
  (Development|PrintString (Utilities|String|Append "当前任务： " (Variables|Default|GetMissionSub)))
  (Variables|Default|SetIsMissionStart true)
  (switch Utilities|FlowControl|Switch|SwitchonE_Mission (Variables|Default|GetMissionType)
    (:NewEnumerator0
      (Collision|SetCollisionEnabled (Variables|Default|GetBox) "QueryOnly"))
    (:NewEnumerator1
      (Collision|SetCollisionEnabled (Variables|Default|GetBox) "NoCollision"))))

(fn GetMissionInfomation
  (return (Variables|Default|GetMission%20Main) (Variables|Default|GetMissionSub) (Variables|Default|GetMissionInfo) (Variables|Default|GetMissionType) (Variables|Default|GetKillTarget)))