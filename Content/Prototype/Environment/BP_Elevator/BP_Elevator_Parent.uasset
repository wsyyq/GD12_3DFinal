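; Parent elevator Blueprint: a platform that toggles between a start point and an editor-placed preview mesh's transform on player interaction.
; An overlap box gates E2Interactive to the 3D character, and calls are ignored mid-move.
; Timelines, rate-scaled by ElevatorMovementSpeed in the construction script, lerp location and rotation.
; Movement start and stop fire CallElevatorMove/CallElevatorStopMove and toggle four safety blocking boxes; arrival plays a bell.
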(event OnComponentEndOverlap(ElevatorInteractiveBox)
  (params (OverlappedComponent :type Primitive%20Component%20Object%20Reference) (OtherActor :type Actor%20Object%20Reference) (OtherComp :type Primitive%20Component%20Object%20Reference) (OtherBodyIndex :type Integer))
  (Utilities|Casting|CastToBP_3DCharacter_P OtherActor)
  (Variables|Default|SetCanUseElevator false))

(event OnComponentBeginOverlap(ElevatorInteractiveBox)
  (params (OverlappedComponent :type Primitive%20Component%20Object%20Reference) (OtherActor :type Actor%20Object%20Reference) (OtherComp :type Primitive%20Component%20Object%20Reference) (OtherBodyIndex :type Integer) (bFromSweep :type Boolean) (SweepResult :type Hit%20Result%20Structure%20%28by%20ref%29))
  (Utilities|Casting|CastToBP_3DCharacter_P OtherActor)
  (Variables|Default|SetCanUseElevator true))

(event Custom|ElevatorToggle
  ;[0.15 0.15 0.15 0.5] Elevator Move
  (if (not (Variables|Default|GetIsElevatorUsing))
    (if (Variables|Default|GetIsElevatorUp)
      (CallFunction|ElevatorBack)
      (else
        (CallFunction|ElevatorGo)))))

(event Custom|ElevatorGo
  (bind _movingplatform (Variables|Default|GetMovingPlatform))
  (bind _starttransform (Variables|Default|GetStartTransform))
  (bind _endtransform (Variables|Default|GetEndTransform))
  ;[0.15 0.15 0.15 0.5] Elevator Move
  (Default|CallElevatorMove)
  (CallFunction|ElevatorMoveandBlockingAppear)
  (Variables|Default|SetIsElevatorUsing true)
  (bind _newtrack_0 (Timeline|ElevatorMoveBack PlayFromStart)
    (:Update
      (Transformation|SetRelativeLocationAndRotation _movingplatform (Math|Vector|Lerp(Vector) (.location _starttransform) (.location _endtransform) _newtrack_0) (Math|Rotator|Lerp(Rotator) (.rotation _starttransform) (.rotation _endtransform) _newtrack_0) false false))
    (:Finished
      (Variables|Default|SetIsElevatorUsing false)
      (Variables|Default|SetIsElevatorUp true)
      (Default|CallElevatorStopMove)
      (CallFunction|ElevatorStopandBlockingDisappear)
      (Audio|PlaySoundatLocation "/Game/GD12_3D/Audio/Cue/A_Tone_Bell_Elevator_Cue.A_Tone_Bell_Elevator_Cue" (Transformation|GetWorldLocation _movingplatform) "0, 0, 0" 1.0 1.0 0.0 0 0 self 0))))

(event Custom|ElevatorBack
  (bind _movingplatform (Variables|Default|GetMovingPlatform))
  (bind _starttransform (Variables|Default|GetStartTransform))
  (bind _endtransform (Variables|Default|GetEndTransform))
  ;[0.15 0.15 0.15 0.5] Elevator Move
  (Default|CallElevatorMove)
  (CallFunction|ElevatorMoveandBlockingAppear)
  (Variables|Default|SetIsElevatorUsing true)
  (bind _newtrack_0 (Timeline|ElevatorMoveGo PlayFromStart)
    (:Update
      (Transformation|SetRelativeLocationAndRotation _movingplatform (Math|Vector|Lerp(Vector) (.location _endtransform) (.location _starttransform) _newtrack_0) (Math|Rotator|Lerp(Rotator) (.rotation _endtransform) (.rotation _starttransform) _newtrack_0) false false))
    (:Finished
      (Variables|Default|SetIsElevatorUsing false)
      (Variables|Default|SetIsElevatorUp false)
      (Default|CallElevatorStopMove)
      (CallFunction|ElevatorStopandBlockingDisappear)
      (Audio|PlaySoundatLocation "/Game/GD12_3D/Audio/Cue/A_Tone_Bell_Elevator_Cue.A_Tone_Bell_Elevator_Cue" (Transformation|GetWorldLocation _movingplatform) "0, 0, 0" 1.0 1.0 0.0 0 0 self 0))))

(event Custom|ElevatorStopAndBlockingDisappear
  ;[0.15 0.15 0.15 0.5] Safety Ensure
  (Collision|SetCollisionEnabled (Variables|Default|GetBoxBlocking1) "NoCollision"))

(event Custom|ElevatorMoveAndBlockingAppear
  ;[0.15 0.15 0.15 0.5] Safety Ensure
  (Collision|SetCollisionEnabled (Variables|Default|GetBoxBlocking1) "QueryAndProbe"))

(event EventBeginPlay
  (Variables|Default|SetEndTransform (Transformation|GetRelativeTransform (Variables|Default|GetPreviewMesh))))

(fn ConstructionScript
  (bind _previewmesh (Variables|Default|GetPreviewMesh))
  (Utilities|FlowControl|Sequence
    (:then_0
      (Components|Timeline|SetPlayRate (Variables|Default|GetElevatorMoveBack) (/ 1.0 (Variables|Default|GetElevatorMovementSpeed)))
      (Components|Timeline|SetPlayRate (Variables|Default|GetElevatorMoveGo) (/ 1.0 (Variables|Default|GetElevatorMovementSpeed))))
    (:then_1
      (Collision|SetCollisionEnabled _previewmesh "NoCollision")
      (Development|SetHiddeninGame _previewmesh true false)
      (Collision|SetCollisionEnabled (Variables|Default|GetBoxBlocking1) "NoCollision")
      (Variables|Default|SetStartTransform (Transformation|GetRelativeTransform (Variables|Default|GetStartPosition))))))

(fn E2Interactive
  (if (Variables|Default|GetCanUseElevator)
    (CallFunction|ElevatorToggle)
    (Default|CallEventFinishInteract)
    (return false "NewEnumerator2" self 0 "" "")))