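; Two-floor elevator, derived from a parent Blueprint, that carries the player or AI guards between floors behind optional keycard locks.
; Inside and landing triggers show interact prompts and record the interactor, while guards wanting the elevator call it automatically.
; E2Interactive checks keycards for players only, then lights the button or shows a hint, and defers to the parent.
; Parent move and stop events drive timeline-lerped inner and outer doors.
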(event OnComponentBeginOverlap(TriggerToUp)
  (params (OverlappedComponent :type Primitive%20Component%20Object%20Reference) (OtherActor :type Actor%20Object%20Reference) (OtherComp :type Primitive%20Component%20Object%20Reference) (OtherBodyIndex :type Integer) (bFromSweep :type Boolean) (SweepResult :type Hit%20Result%20Structure%20%28by%20ref%29))
  (bind _interactwidget (Variables|Default|GetInteractWidget))
  ;[0.15 0.15 0.15 0.5] Floor Selection
  (if (not (Variables|Default|GetIsElevatorUsing))
    (Utilities|Casting|CastToBP_3DCharacter_P OtherActor)
    (Transformation|SetRelativeLocation _interactwidget (+ (Variables|/Script/Engine.SceneComponent|GetRelativeLocation (Variables|Default|GetCurrenctMesh)) "130.000000,-175.000000,125.000000") false false)
    (Development|SetHiddeninGame _interactwidget false false)
    (Default|ShowObjectType (.AsWBP%20Interact%20Panel (Utilities|Casting|CastToWBP_InteractPanel (UserInterface|GetWidget (Variables|Default|GetInteractWidget)))) "NewEnumerator2" "" (Utilities|Text|ToText(String) (Utilities|String|Append "To F" (Utilities|String|ToString(Integer) (+ (Variables|Default|GetFloorNumDown) (Variables|Default|GetFloorNumBetween))))))
    (Variables|Default|SetIsInsDown true)
    (Variables|Default|SetInteractor OtherActor)))

(event OnComponentEndOverlap(TriggerToUp)
  (params (OverlappedComponent :type Primitive%20Component%20Object%20Reference) (OtherActor :type Actor%20Object%20Reference) (OtherComp :type Primitive%20Component%20Object%20Reference) (OtherBodyIndex :type Integer))
  ;[0.15 0.15 0.15 0.5] Floor Selection
  (Utilities|Casting|CastToBP_3DCharacter_P OtherActor)
  (Development|SetHiddeninGame (Variables|Default|GetInteractWidget) true false)
  (Variables|Default|SetCanUseElevator false))

(event OnComponentBeginOverlap(TriggerToUp_Out)
  (params (OverlappedComponent :type Primitive%20Component%20Object%20Reference) (OtherActor :type Actor%20Object%20Reference) (OtherComp :type Primitive%20Component%20Object%20Reference) (OtherBodyIndex :type Integer) (bFromSweep :type Boolean) (SweepResult :type Hit%20Result%20Structure%20%28by%20ref%29))
  (bind _interactwidget (Variables|Default|GetInteractWidget))
  ;[0.15 0.15 0.15 0.5] Floor Selection
  (if (not (Variables|Default|GetIsElevatorUsing))
    (Utilities|FlowControl|Sequence
      (:then_0
        (Utilities|Casting|CastToBP_3DCharacter_P OtherActor)
        (Transformation|SetRelativeLocation _interactwidget (+ (Variables|/Script/Engine.SceneComponent|GetRelativeLocation (Variables|Default|GetPreviewMesh)) "130.000000,-225.000000,125.000000") false false)
        (Development|SetHiddeninGame _interactwidget false false)
        (Default|ShowObjectType (.AsWBP%20Interact%20Panel (Utilities|Casting|CastToWBP_InteractPanel (UserInterface|GetWidget (Variables|Default|GetInteractWidget)))) "NewEnumerator2" "" (Utilities|Text|ToText(String) (Utilities|String|Append "To F" (Utilities|String|ToString(Integer) (+ (Variables|Default|GetFloorNumDown) (Variables|Default|GetFloorNumBetween))))))
        (if (Variables|Default|GetIsElevatorUp)
          (CallFunction|OpenOutside)
          (else
            (Variables|Default|SetIsOutDown true)
            (Variables|Default|SetInteractor OtherActor))))
      (:then_1
        (bind _asbp_ai_guard (Utilities|Casting|CastToBP_AI_Guard OtherActor))
        (if (Variables|/Game/Prototype/AI/BP_AI_Guard.BP_AI_Guard_C|GetWantElevator _asbp_ai_guard)
          (Utilities|FlowControl|DoOnce false
            (:Completed
              (Variables|Default|SetIsOutDown true)
              (Variables|Default|SetInteractor _asbp_ai_guard)
              (CallFunction|E2Interactive))))))))

(event OnComponentEndOverlap(TriggerToUp_Out)
  (params (OverlappedComponent :type Primitive%20Component%20Object%20Reference) (OtherActor :type Actor%20Object%20Reference) (OtherComp :type Primitive%20Component%20Object%20Reference) (OtherBodyIndex :type Integer))
  ;[0.15 0.15 0.15 0.5] Floor Selection
  (Utilities|Casting|CastToBP_3DCharacter_P OtherActor)
  (Development|SetHiddeninGame (Variables|Default|GetInteractWidget) true false)
  (Variables|Default|SetCanUseElevator false))

(event OnComponentBeginOverlap(TriggerToDown_Out)
  (params (OverlappedComponent :type Primitive%20Component%20Object%20Reference) (OtherActor :type Actor%20Object%20Reference) (OtherComp :type Primitive%20Component%20Object%20Reference) (OtherBodyIndex :type Integer) (bFromSweep :type Boolean) (SweepResult :type Hit%20Result%20Structure%20%28by%20ref%29))
  (bind _interactwidget (Variables|Default|GetInteractWidget))
  ;[0.15 0.15 0.15 0.5] Floor Selection
  (if (not (Variables|Default|GetIsElevatorUsing))
    (Utilities|Casting|CastToBP_3DCharacter_P OtherActor)
    (Transformation|SetRelativeLocation _interactwidget (+ (Variables|/Script/Engine.SceneComponent|GetRelativeLocation (Variables|Default|GetCurrenctMesh)) "130.000000,-225.000000,125.000000") false false)
    (Development|SetHiddeninGame _interactwidget false false)
    (Default|ShowObjectType (.AsWBP%20Interact%20Panel (Utilities|Casting|CastToWBP_InteractPanel (UserInterface|GetWidget (Variables|Default|GetInteractWidget)))) "NewEnumerator2" "" (Utilities|Text|ToText(String) (Utilities|String|Append "To F" (Utilities|String|ToString(Integer) (Variables|Default|GetFloorNumDown)))))
    (if (Variables|Default|GetIsElevatorUp)
      (Variables|Default|SetIsOutUp true)
      (Variables|Default|SetInteractor OtherActor)
      (else
        (CallFunction|OpenOutside)))))

(event OnComponentEndOverlap(TriggerToDown_Out)
  (params (OverlappedComponent :type Primitive%20Component%20Object%20Reference) (OtherActor :type Actor%20Object%20Reference) (OtherComp :type Primitive%20Component%20Object%20Reference) (OtherBodyIndex :type Integer))
  ;[0.15 0.15 0.15 0.5] Floor Selection
  (Utilities|Casting|CastToBP_3DCharacter_P OtherActor)
  (Development|SetHiddeninGame (Variables|Default|GetInteractWidget) true false)
  (Variables|Default|SetCanUseElevator false))

(event OnComponentBeginOverlap(TriggerToDown)
  (params (OverlappedComponent :type Primitive%20Component%20Object%20Reference) (OtherActor :type Actor%20Object%20Reference) (OtherComp :type Primitive%20Component%20Object%20Reference) (OtherBodyIndex :type Integer) (bFromSweep :type Boolean) (SweepResult :type Hit%20Result%20Structure%20%28by%20ref%29))
  (bind _interactwidget (Variables|Default|GetInteractWidget))
  ;[0.15 0.15 0.15 0.5] Floor Selection
  (if (not (Variables|Default|GetIsElevatorUsing))
    (Utilities|FlowControl|Sequence
      (:then_0
        (Utilities|Casting|CastToBP_3DCharacter_P OtherActor)
        (Transformation|SetRelativeLocation _interactwidget (+ (Variables|/Script/Engine.SceneComponent|GetRelativeLocation (Variables|Default|GetPreviewMesh)) "130.000000,-175.000000,125.000000") false false)
        (Development|SetHiddeninGame _interactwidget false false)
        (Default|ShowObjectType (.AsWBP%20Interact%20Panel (Utilities|Casting|CastToWBP_InteractPanel (UserInterface|GetWidget (Variables|Default|GetInteractWidget)))) "NewEnumerator2" "" (Utilities|Text|ToText(String) (Utilities|String|Append "To F" (Utilities|String|ToString(Integer) (Variables|Default|GetFloorNumDown)))))
        (Variables|Default|SetIsInsUp true)
        (Variables|Default|SetInteractor OtherActor))
      (:then_1
        (bind _asbp_ai_guard (Utilities|Casting|CastToBP_AI_Guard OtherActor))
        (if (Variables|/Game/Prototype/AI/BP_AI_Guard.BP_AI_Guard_C|GetWantElevator _asbp_ai_guard)
          (Utilities|FlowControl|DoOnce false
            (:Completed
              (Variables|Default|SetIsInsUp true)
              (Variables|Default|SetInteractor _asbp_ai_guard)
              (Utilities|FlowControl|Delay 1.0)
              (CallFunction|E2Interactive))))))))

(event OnComponentEndOverlap(TriggerToDown)
  (params (OverlappedComponent :type Primitive%20Component%20Object%20Reference) (OtherActor :type Actor%20Object%20Reference) (OtherComp :type Primitive%20Component%20Object%20Reference) (OtherBodyIndex :type Integer))
  ;[0.15 0.15 0.15 0.5] Floor Selection
  (Utilities|Casting|CastToBP_3DCharacter_P OtherActor)
  (Development|SetHiddeninGame (Variables|Default|GetInteractWidget) true false)
  (Variables|Default|SetCanUseElevator false))

(event Custom|CloseInside
  (bind _doorl (Variables|Default|GetDoorL))
  (bind _doorr (Variables|Default|GetDoorR))
  ;[0.15 0.15 0.15 0.5] Fuction Add-on
  (bind _time (Timeline|InsideDoorClose PlayFromStart)
    (:Update
      (Transformation|SetRelativeLocation _doorl (Math|Vector|Lerp(Vector) (Variables|/Script/Engine.SceneComponent|GetRelativeLocation _doorl) (Variables|/Script/Engine.SceneComponent|GetRelativeLocation (Variables|Default|GetDoorLClosePos)) _time) false false)
      (Transformation|SetRelativeLocation _doorr (Math|Vector|Lerp(Vector) (Variables|/Script/Engine.SceneComponent|GetRelativeLocation _doorr) (Variables|/Script/Engine.SceneComponent|GetRelativeLocation (Variables|Default|GetDoorRClosePos)) _time) false false))))

(event Custom|OpenInside
  (bind _doorl (Variables|Default|GetDoorL))
  (bind _doorr (Variables|Default|GetDoorR))
  ;[0.15 0.15 0.15 0.5] Fuction Add-on
  (bind _time (Timeline|ElevatorDoorOpen PlayFromStart)
    (:Update
      (Transformation|SetRelativeLocation _doorl (Math|Vector|Lerp(Vector) (Variables|/Script/Engine.SceneComponent|GetRelativeLocation _doorl) (Variables|/Script/Engine.SceneComponent|GetRelativeLocation (Variables|Default|GetDoorLOpenPos)) _time) false false)
      (Transformation|SetRelativeLocation _doorr (Math|Vector|Lerp(Vector) (Variables|/Script/Engine.SceneComponent|GetRelativeLocation _doorr) (Variables|/Script/Engine.SceneComponent|GetRelativeLocation (Variables|Default|GetDoorROpenPos)) _time) false false))))

(event Custom|DoorClose
  ;[0.15 0.15 0.15 0.5] Fuction Add-on
  (CallFunction|CloseInside)
  (CallFunction|CloseOutside))

(event Custom|DoorOpen
  ;[0.15 0.15 0.15 0.5] Fuction Add-on
  (CallFunction|OpenInside)
  (CallFunction|OpenOutside)
  (Rendering|Material|SetMaterial (Variables|Default|GetButtonUp_Out) 0 (Variables|Default|GetDefaultMat))
  (Variables|Default|SetIsInsDown false)
  (Variables|Default|SetIsOutDown false)
  (Variables|Default|SetIsInsUp false)
  (Variables|Default|SetIsOutUp false))

(event Custom|CloseOutside
  (bind _doorr_outup (Variables|Default|GetDoorR_OutUp))
  (bind _doorl_outup (Variables|Default|GetDoorL_OutUp))
  (bind _doorr_outdown (Variables|Default|GetDoorR_OutDown))
  (bind _doorl_outdown (Variables|Default|GetDoorL_OutDown))
  ;[0.15 0.15 0.15 0.5] Fuction Add-on
  (bind _time (Timeline|OutsideDoorClose PlayFromStart)
    (:Update
      (Utilities|FlowControl|Sequence
        (:then_0
          (if (Variables|Default|GetIsElevatorUp)
            (Transformation|SetRelativeLocation _doorl_outup (Math|Vector|Lerp(Vector) (Variables|/Script/Engine.SceneComponent|GetRelativeLocation _doorl_outup) (Variables|/Script/Engine.SceneComponent|GetRelativeLocation (Variables|Default|GetDoorL_OutUpClose)) _time) false false)
            (Transformation|SetRelativeLocation _doorr_outup (Math|Vector|Lerp(Vector) (Variables|/Script/Engine.SceneComponent|GetRelativeLocation _doorr_outup) (Variables|/Script/Engine.SceneComponent|GetRelativeLocation (Variables|Default|GetDoorR_OutUpClose)) _time) false false)))
        (:then_1
          (if (not (Variables|Default|GetIsElevatorUp))
            (Transformation|SetRelativeLocation _doorl_outdown (Math|Vector|Lerp(Vector) (Variables|/Script/Engine.SceneComponent|GetRelativeLocation _doorl_outdown) (Variables|/Script/Engine.SceneComponent|GetRelativeLocation (Variables|Default|GetDoorL_OutDownClose)) _time) false false)
            (Transformation|SetRelativeLocation _doorr_outdown (Math|Vector|Lerp(Vector) (Variables|/Script/Engine.SceneComponent|GetRelativeLocation _doorr_outdown) (Variables|/Script/Engine.SceneComponent|GetRelativeLocation (Variables|Default|GetDoorR_OutDownClose)) _time) false false)))))))

(event Custom|OpenOutside
  (bind _doorl_outup (Variables|Default|GetDoorL_OutUp))
  (bind _doorr_outup (Variables|Default|GetDoorR_OutUp))
  (bind _doorl_outdown (Variables|Default|GetDoorL_OutDown))
  (bind _doorr_outdown (Variables|Default|GetDoorR_OutDown))
  ;[0.15 0.15 0.15 0.5] Fuction Add-on
  (bind _time (Timeline|OutsideDoorOpen PlayFromStart)
    (:Update
      (Utilities|FlowControl|Sequence
        (:then_0
          (if (Variables|Default|GetIsElevatorUp)
            (Transformation|SetRelativeLocation _doorl_outup (Math|Vector|Lerp(Vector) (Variables|/Script/Engine.SceneComponent|GetRelativeLocation _doorl_outup) (Variables|/Script/Engine.SceneComponent|GetRelativeLocation (Variables|Default|GetDoorL_OutUpOpen)) _time) false false)
            (Transformation|SetRelativeLocation _doorr_outup (Math|Vector|Lerp(Vector) (Variables|/Script/Engine.SceneComponent|GetRelativeLocation _doorr_outup) (Variables|/Script/Engine.SceneComponent|GetRelativeLocation (Variables|Default|GetDoorR_OutUpOpen)) _time) false false)))
        (:then_1
          (if (not (Variables|Default|GetIsElevatorUp))
            (Transformation|SetRelativeLocation _doorl_outdown (Math|Vector|Lerp(Vector) (Variables|/Script/Engine.SceneComponent|GetRelativeLocation _doorl_outdown) (Variables|/Script/Engine.SceneComponent|GetRelativeLocation (Variables|Default|GetDoorL_OutDownOpen)) _time) false false)
            (Transformation|SetRelativeLocation _doorr_outdown (Math|Vector|Lerp(Vector) (Variables|/Script/Engine.SceneComponent|GetRelativeLocation _doorr_outdown) (Variables|/Script/Engine.SceneComponent|GetRelativeLocation (Variables|Default|GetDoorR_OutDownOpen)) _time) false false)))))))

(event EventBeginPlay
  (bind _floornumdown (Variables|Default|GetFloorNumDown))
  ;[0.15 0.15 0.15 0.5] Parent Functions
  (|CallParentFunction)
  ;[0.15 0.15 0.15 0.5] Fuction Add-on
  (Utilities|FlowControl|Sequence
    (:then_0
      (Development|SetHiddeninGame (Variables|Default|GetInteractWidget) true false)
      (Rendering|Components|TextRender|SetText (Variables|Default|GetTextRenderDown) (Utilities|Text|ToText(String) (Utilities|String|Append "F" (Utilities|String|ToString(Integer) _floornumdown))))
      (Rendering|Components|TextRender|SetText (Variables|Default|GetTextRenderUp) (Utilities|Text|ToText(String) (Utilities|String|Append "F" (Utilities|String|ToString(Integer) (+ _floornumdown (Variables|Default|GetFloorNumBetween))))))
      (EventDispatchers|BindEventtoElevatorMove (delegate Custom|DoorClose))
      (EventDispatchers|BindEventtoElevatorStopMove (delegate Custom|DoorOpen)))))

(event EventElevatorBack
  ;[0.15 0.15 0.15 0.5] Parent Functions
  (|CallParentFunction))

(event EventElevatorGo
  ;[0.15 0.15 0.15 0.5] Parent Functions
  (|CallParentFunction))

(event EventElevatorToggle
  ;[0.15 0.15 0.15 0.5] Parent Functions
  (|CallParentFunction))

(event EventElevatorMoveandBlockingAppear
  ;[0.15 0.15 0.15 0.5] Parent Functions
  (|CallParentFunction))

(event EventElevatorStopandBlockingDisappear
  ;[0.15 0.15 0.15 0.5] Parent Functions
  (|CallParentFunction))

(fn ConstructionScript
  (bind _keypad (Variables|Default|GetKeypad))
  (|CallParentFunction)
  (switch Utilities|FlowControl|Switch|SwitchonE_DoorType (Variables|Default|GetDoorType)
    (:NewEnumerator0
      (Development|SetHiddeninGame _keypad true false))
    (:NewEnumerator1
      (Development|SetHiddeninGame _keypad false false :!label _label))
    (:NewEnumerator2
      (goto _label))
    (:NewEnumerator3
      (goto _label))))

(fn E2Interactive
  (bind _returnvalue (Game|Player|GetPlayerPawn 0))
  (bind _asbp_3dcharacter_p (Utilities|Casting|CastToBP_3DCharacter_P _returnvalue))
  (bind _caninteract (CallFunction|CheckKeycard))
  (if _caninteract
    (Variables|Default|SetCanUseElevator true)
    (Default|HideObjectType (.AsWBP%20Interact%20Panel (Utilities|Casting|CastToWBP_InteractPanel (UserInterface|GetWidget (Variables|Default|GetInteractWidget)))))
    (Utilities|FlowControl|Sequence
      (:then_0
        (if (Variables|Default|GetIsInsDown)
          (Rendering|Material|SetMaterial (Variables|Default|GetButtonUp) 0 (Variables|Default|GetConfirmMat))
          (bind (_canpick _interacttype _interacttarget _passward _docarthur _doccontent) (|CallParentFunction :!label _label))
          (return _canpick _interacttype _interacttarget _passward _docarthur _doccontent)))
      (:then_1
        (if (Variables|Default|GetIsOutDown)
          (Rendering|Material|SetMaterial (Variables|Default|GetButtonUp_Out) 0 (Variables|Default|GetConfirmMat))
          (goto _label)))
      (:then_2
        (if (Variables|Default|GetIsInsUp)
          (Rendering|Material|SetMaterial (Variables|Default|GetButtonDown) 0 (Variables|Default|GetConfirmMat))
          (goto _label)))
      (:then_3
        (if (Variables|Default|GetIsOutUp)
          (Rendering|Material|SetMaterial (Variables|Default|GetButtonDown_Out) 0 (Variables|Default|GetConfirmMat))
          (goto _label))))
    (else
      (Variables|Default|SetCanUseElevator false)
      (Default|AddHint _asbp_3dcharacter_p "Elevator" (Utilities|String|ToString(Text) (Variables|Default|GetNameOrBelong)) true false)
      (Default|SetHint _asbp_3dcharacter_p)
      (goto _label))))

(fn CheckKeycard
  (bind _asbp_3dcharacter_p (Utilities|Casting|CastToBP_3DCharacter_P (Variables|Default|GetInteractor))
    (:then
      (switch Utilities|FlowControl|Switch|SwitchonE_DoorType (Variables|Default|GetDoorType)
        (:NewEnumerator0
          _)
        (:NewEnumerator1
          (if (Variables|/Game/Prototype/GameMode/BP_3DCharacter_P.BP_3DCharacter_P_C|GetHasKeycard1 _asbp_3dcharacter_p)
            _
            (else
              (bind _output_get (Variables|Default|SetCanInteract false :!label _label))
              (return _output_get))))
        (:NewEnumerator2
          (if (Variables|/Game/Prototype/GameMode/BP_3DCharacter_P.BP_3DCharacter_P_C|GetHasKeycard2 _asbp_3dcharacter_p)
            _
            (else
              (goto _label))))
        (:NewEnumerator3
          (if (Variables|/Game/Prototype/GameMode/BP_3DCharacter_P.BP_3DCharacter_P_C|GetHasKeycard3 _asbp_3dcharacter_p)
            _
            (else
              (goto _label)))))
      (bind _output_get_2 (Variables|Default|SetCanInteract true))
      (return _output_get_2))
    (:CastFailed
      (return true))))