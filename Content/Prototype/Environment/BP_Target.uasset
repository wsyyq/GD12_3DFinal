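; BP_Target is a prototype target actor that displays a value when one of its zones is hit.
; HitTarget compares the hit component against L1, L2 and L3 and sets a TextRender to that zone's value.
; The text appears with a confirmation tone at the actor's location, then hides after a delay.
; A DoOnce gates repeat hits and resets after a delay.
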(event Custom|HitTarget
  (params (HitComponent :type Actor%20Component%20Object%20Reference))
  (Utilities|FlowControl|DoOnce false :!label _label
    (:Completed
      (if (== HitComponent (Variables|Default|GetL3))
        (Rendering|Components|TextRender|SetText (Variables|Default|GetTextRender) (Variables|Default|GetValue1))
        (Development|SetHiddeninGame (Variables|Default|GetTextRender) false false :!label _label_2)
        (Audio|PlaySoundatLocation "/Game/GD12_3D/Audio/SoundWaves/Prompt/A_Tone_Confirm_03.A_Tone_Confirm_03" (Transformation|GetActorLocation) "0, 0, 0" 1.0 1.0 0.0 "/Game/GD12_3D/Audio/Attenuation/ATT_Chandelier.ATT_Chandelier" 0 self 0)
        (Utilities|FlowControl|Delay 3.0)
        (Development|SetHiddeninGame (Variables|Default|GetTextRender) true false)
        (elif (== HitComponent (Variables|Default|GetL2))
          (Rendering|Components|TextRender|SetText (Variables|Default|GetTextRender) (Variables|Default|GetValue2))
          (goto _label_2)
          (elif (== HitComponent (Variables|Default|GetL1))
            (Rendering|Components|TextRender|SetText (Variables|Default|GetTextRender) (Variables|Default|GetValue3))
            (goto _label_2)
            (else
              _))))
      (Utilities|FlowControl|Delay 0.2)
      (goto _label Reset))))

(fn ConstructionScript)