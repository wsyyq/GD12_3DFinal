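; Pass card pickup for the prototype's unique doors, with a type for the elevator door, meeting room password door or storage room.
; The construction script sets a placeholder cube mesh and a text label matching the card type.
; E2Interactive hides the actor, disables mesh and trigger collision, prints a debug message and passes the card type to BP_3DCharacter_P through PickUpPassCard.
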(event EventBeginPlay
  (|CallParentFunction))

(fn ConstructionScript
  (switch Utilities|FlowControl|Switch|SwitchonE_PassCardType (Variables|Default|GetPassCardType)
    (:NewEnumerator0
      (Components|StaticMesh|SetStaticMesh (Variables|Default|GetPickups) "/Engine/EngineMeshes/Cube.Cube")
      (Rendering|Components|TextRender|SetText (Variables|Default|GetTextRender) (Utilities|Text|ToText(String) "PassCard1")))
    (:NewEnumerator1
      (Components|StaticMesh|SetStaticMesh (Variables|Default|GetPickups) "/Engine/EngineMeshes/Cube.Cube")
      (Rendering|Components|TextRender|SetText (Variables|Default|GetTextRender) (Utilities|Text|ToText(String) "PassCard2")))
    (:NewEnumerator2
      (Components|StaticMesh|SetStaticMesh (Variables|Default|GetPickups) "/Engine/EngineMeshes/Cube.Cube")
      (Rendering|Components|TextRender|SetText (Variables|Default|GetTextRender) (Utilities|Text|ToText(String) "PassCard3")))))

(fn E2Interactive
  (bind _returnvalue (Game|GetPlayerCharacter 0))
  (bind _asbp_3dcharacter_p (Utilities|Casting|CastToBP_3DCharacter_P _returnvalue))
  (switch Utilities|FlowControl|Switch|SwitchonE_PassCardType (Variables|Default|GetPassCardType)
    (:NewEnumerator0
      (Rendering|SetActorHiddenInGame true)
      (Collision|SetCollisionEnabled (Variables|Default|GetPickups) "NoCollision")
      (Collision|SetCollisionEnabled (Variables|Default|GetPickTriggerBox) "NoCollision")
      (Development|PrintString "拾取门禁1")
      (Default|PickUpPassCard _asbp_3dcharacter_p "NewEnumerator0")
      (return true "NewEnumerator0"))
    (:NewEnumerator1
      (Rendering|SetActorHiddenInGame true)
      (Collision|SetCollisionEnabled (Variables|Default|GetPickups) "NoCollision")
      (Collision|SetCollisionEnabled (Variables|Default|GetPickTriggerBox) "NoCollision")
      (Development|PrintString "拾取门禁2")
      (Default|PickUpPassCard _asbp_3dcharacter_p "NewEnumerator1")
      (return true "NewEnumerator0"))
    (:NewEnumerator2
      (Rendering|SetActorHiddenInGame true)
      (Collision|SetCollisionEnabled (Variables|Default|GetPickups) "NoCollision")
      (Collision|SetCollisionEnabled (Variables|Default|GetPickTriggerBox) "NoCollision")
      (Development|PrintString "拾取门禁3")
      (Default|PickUpPassCard _asbp_3dcharacter_p "NewEnumerator2")
      (return true "NewEnumerator0"))))