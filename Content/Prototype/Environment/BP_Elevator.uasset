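; Child elevator Blueprint that links two adjacent floors, adding floor signage and interaction prompts on top of its parent's elevator behavior.
; On BeginPlay it hides the prompt and labels both floors from FloorDownNum.
; When the elevator is idle, the lower and upper triggers show the player a prompt naming the opposite floor and set CanUseElevator, clearing both on exit.
; Interacting hides the panel's prompt and passes through the parent's result.
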(event OnComponentBeginOverlap(TriggerDown)
  (params (OverlappedComponent :type Primitive%20Component%20Object%20Reference) (OtherActor :type Actor%20Object%20Reference) (OtherComp :type Primitive%20Component%20Object%20Reference) (OtherBodyIndex :type Integer) (bFromSweep :type Boolean) (SweepResult :type Hit%20Result%20Structure%20%28by%20ref%29))
  (bind _interactwidget (Variables|Default|GetInteractWidget))
  ;[0.15 0.15 0.15 0.5] Floor Selection
  (if (not (Variables|Default|GetIsElevatorUsing))
    (Utilities|Casting|CastToBP_3DCharacter_P OtherActor)
    (Transformation|SetRelativeLocation _interactwidget (+ (Variables|/Script/Engine.SceneComponent|GetRelativeLocation (Variables|Default|GetInsideChooseDown)) "0.000000,0.000000,10.000000") false false)
    (Development|SetHiddeninGame _interactwidget false false)
    (Default|ShowObjectType (.AsWBP%20Interact%20Panel (Utilities|Casting|CastToWBP_InteractPanel (UserInterface|GetWidget (Variables|Default|GetInteractWidget)))) (Utilities|Text|ToText(String) (Utilities|String|Append "To Floor " (Utilities|String|ToString(Integer) (+ (Variables|Default|GetFloorDownNum) 1)))) "NewEnumerator2")
    (Variables|Default|SetCanUseElevator true)))

(event OnComponentEndOverlap(TriggerDown)
  (params (OverlappedComponent :type Primitive%20Component%20Object%20Reference) (OtherActor :type Actor%20Object%20Reference) (OtherComp :type Primitive%20Component%20Object%20Reference) (OtherBodyIndex :type Integer))
  ;[0.15 0.15 0.15 0.5] Floor Selection
  (Utilities|Casting|CastToBP_3DCharacter_P OtherActor)
  (Development|SetHiddeninGame (Variables|Default|GetInteractWidget) true false)
  (Variables|Default|SetCanUseElevator false))

(event OnComponentBeginOverlap(TriggerUp)
  (params (OverlappedComponent :type Primitive%20Component%20Object%20Reference) (OtherActor :type Actor%20Object%20Reference) (OtherComp :type Primitive%20Component%20Object%20Reference) (OtherBodyIndex :type Integer) (bFromSweep :type Boolean) (SweepResult :type Hit%20Result%20Structure%20%28by%20ref%29))
  (bind _interactwidget (Variables|Default|GetInteractWidget))
  ;[0.15 0.15 0.15 0.5] Floor Selection
  (if (not (Variables|Default|GetIsElevatorUsing))
    (Utilities|Casting|CastToBP_3DCharacter_P OtherActor)
    (Transformation|SetRelativeLocation _interactwidget (+ (Variables|/Script/Engine.SceneComponent|GetRelativeLocation (Variables|Default|GetInsideChooseUp)) "0.000000,0.000000,10.000000") false false)
    (Development|SetHiddeninGame _interactwidget false false)
    (Default|ShowObjectType (.AsWBP%20Interact%20Panel (Utilities|Casting|CastToWBP_InteractPanel (UserInterface|GetWidget (Variables|Default|GetInteractWidget)))) (Utilities|Text|ToText(String) (Utilities|String|Append "To Floor " (Utilities|String|ToString(Integer) (Variables|Default|GetFloorDownNum)))) "NewEnumerator2")
    (Variables|Default|SetCanUseElevator true)))

(event OnComponentEndOverlap(TriggerUp)
  (params (OverlappedComponent :type Primitive%20Component%20Object%20Reference) (OtherActor :type Actor%20Object%20Reference) (OtherComp :type Primitive%20Component%20Object%20Reference) (OtherBodyIndex :type Integer))
  ;[0.15 0.15 0.15 0.5] Floor Selection
  (Utilities|Casting|CastToBP_3DCharacter_P OtherActor)
  (Development|SetHiddeninGame (Variables|Default|GetInteractWidget) true false)
  (Variables|Default|SetCanUseElevator false))

(event EventBeginPlay
  (bind _floordownnum (Variables|Default|GetFloorDownNum))
  ;[0.15 0.15 0.15 0.5] Parent Functions
  (|CallParentFunction)
  (Development|SetHiddeninGame (Variables|Default|GetInteractWidget) true false)
  (Rendering|Components|TextRender|SetText (Variables|Default|GetTextRenderDown) (Utilities|Text|ToText(String) (Utilities|String|Append "F" (Utilities|String|ToString(Integer) _floordownnum))))
  (Rendering|Components|TextRender|SetText (Variables|Default|GetTextRenderUp) (Utilities|Text|ToText(String) (Utilities|String|Append "F" (Utilities|String|ToString(Integer) (+ _floordownnum 1))))))

(event EventElevatorBack
  ;[0.15 0.15 0.15 0.5] Parent Functions
  (|CallParentFunction))

(event EventElevatorGo
  ;[0.15 0.15 0.15 0.5] Parent Functions
  (|CallParentFunction))

(event EventElevatorToggle
  ;[0.15 0.15 0.15 0.5] Parent Functions
  (|CallParentFunction))

(event EventElevatorMoveandBlockingAppear
  ;[0.15 0.15 0.15 0.5] Parent Functions
  (|CallParentFunction))

(event EventElevatorStopandBlockingDisappear
  ;[0.15 0.15 0.15 0.5] Parent Functions
  (|CallParentFunction))

(fn ConstructionScript
  (|CallParentFunction))

(fn E2Interactive
  (bind (_canpick _interacttype _interacttarget _passward _docarthur _doccontent) (|CallParentFunction))
  (Default|HideObjectType (.AsWBP%20Interact%20Panel (Utilities|Casting|CastToWBP_InteractPanel (UserInterface|GetWidget (Variables|Default|GetInteractWidget)))))
  (return _canpick _interacttype _interacttarget _passward _docarthur _doccontent))