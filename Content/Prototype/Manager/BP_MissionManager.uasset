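; Mission manager that runs a level's missions as a hard-coded chain of up to sixteen sequential stages, starting shortly after BeginPlay.
; Each stage starts and shows every mission in its array, stores it as RelativeMission and calls MissionChange.
; Success events decrement the stage's counter, launching the next stage at zero.
; IsLevelMain levels call AllMissionOver after stage eight; others continue through stage sixteen.
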(event Custom|CallMission9%20Or%20GameEnd
  (bind _mission9 (Variables|Default|GetMission9))
  ;[0.15 0.15 0.15 0.5] 分界位，检查是哪个关卡
  (bind _result (Math|Integer|DecrementInt (Variables|Default|GetMission8Num))
    (:%20%20
      (if (<= _result 0)
        (if (Variables|Default|GetIsLevelMain)
          (Default|CallAllMissionOver)
          (else
            (for _array_element _mission9
              (Default|MissionStartandShowThis _array_element)
              (Variables|Default|SetRelativeMission _mission9)
              (EventDispatchers|BindEventtoMissionSuccess _mission9 (delegate Custom|CallMission10))
              (Default|CallMissionChange))
            (Variables|Default|SetMission9Num (Utilities|Array|Length _mission9))))))))

(event Custom|CallMission1
  (bind _mission1 (Variables|Default|GetMission1))
  (for _array_element _mission1
    (Default|MissionStartandShowThis _array_element)
    (Variables|Default|SetRelativeMission _mission1)
    (EventDispatchers|BindEventtoMissionSuccess _mission1 (delegate Custom|CallMission2))
    (Default|CallMissionChange))
  (Variables|Default|SetMission1Num (Utilities|Array|Length _mission1)))

(event Custom|CallMission12
  (bind _mission12 (Variables|Default|GetMission12))
  (bind _result (Math|Integer|DecrementInt (Variables|Default|GetMission11Num))
    (:%20%20
      (if (<= _result 0)
        (for _array_element _mission12
          (Default|MissionStartandShowThis _array_element)
          (Variables|Default|SetRelativeMission _mission12)
          (EventDispatchers|BindEventtoMissionSuccess _mission12 (delegate Custom|CallMission13))
          (Default|CallMissionChange))
        (Variables|Default|SetMission12Num (Utilities|Array|Length _mission12))))))

(event Custom|CallMission8
  (bind _mission8 (Variables|Default|GetMission8))
  (bind _result (Math|Integer|DecrementInt (Variables|Default|GetMission7Num))
    (:%20%20
      (if (<= _result 0)
        (for _array_element _mission8
          (Default|MissionStartandShowThis _array_element)
          (Variables|Default|SetRelativeMission _mission8)
          (EventDispatchers|BindEventtoMissionSuccess _mission8 (delegate Custom|CallMission9%20Or%20GameEnd))
          (Default|CallMissionChange))
        (Variables|Default|SetMission8Num (Utilities|Array|Length _mission8))))))

(event Custom|CallMission15
  (bind _mission15 (Variables|Default|GetMission15))
  (bind _result (Math|Integer|DecrementInt (Variables|Default|GetMission14Num))
    (:%20%20
      (if (<= _result 0)
        (for _array_element _mission15
          (Default|MissionStartandShowThis _array_element)
          (Variables|Default|SetRelativeMission _mission15)
          (EventDispatchers|BindEventtoMissionSuccess _mission15 (delegate Custom|CallMission16))
          (Default|CallMissionChange))
        (Variables|Default|SetMission15Num (Utilities|Array|Length _mission15))))))

(event Custom|CallMission16
  (bind _mission16 (Variables|Default|GetMission16))
  (bind _result (Math|Integer|DecrementInt (Variables|Default|GetMission15Num))
    (:%20%20
      (if (<= _result 0)
        (for _array_element _mission16
          (Default|MissionStartandShowThis _array_element)
          (Variables|Default|SetRelativeMission _mission16)
          (EventDispatchers|BindEventtoMissionSuccess _mission16 (delegate Custom|GameEnd))
          (Default|CallMissionChange))
        (Variables|Default|SetMission16Num (Utilities|Array|Length _mission16))))))

(event Custom|CallMission13
  (bind _mission13 (Variables|Default|GetMission13))
  (bind _result (Math|Integer|DecrementInt (Variables|Default|GetMission12Num))
    (:%20%20
      (if (<= _result 0)
        (for _array_element _mission13
          (Default|MissionStartandShowThis _array_element)
          (Variables|Default|SetRelativeMission _mission13)
          (EventDispatchers|BindEventtoMissionSuccess _mission13 (delegate Custom|CallMission14))
          (Default|CallMissionChange))
        (Variables|Default|SetMission13Num (Utilities|Array|Length _mission13))))))

(event Custom|CallMission2
  (bind _mission2 (Variables|Default|GetMission2))
  (bind _result (Math|Integer|DecrementInt (Variables|Default|GetMission1Num))
    (:%20%20
      (if (<= _result 0)
        (for _array_element _mission2
          (Default|MissionStartandShowThis _array_element)
          (Variables|Default|SetRelativeMission _mission2)
          (EventDispatchers|BindEventtoMissionSuccess _mission2 (delegate Custom|CallMission3))
          (Default|CallMissionChange))
        (Variables|Default|SetMission2Num (Utilities|Array|Length _mission2))))))

(event Custom|CallMission14
  (bind _mission14 (Variables|Default|GetMission14))
  (bind _result (Math|Integer|DecrementInt (Variables|Default|GetMission13Num))
    (:%20%20
      (if (<= _result 0)
        (for _array_element _mission14
          (Default|MissionStartandShowThis _array_element)
          (Variables|Default|SetRelativeMission _mission14)
          (EventDispatchers|BindEventtoMissionSuccess _mission14 (delegate Custom|CallMission15))
          (Default|CallMissionChange))
        (Variables|Default|SetMission14Num (Utilities|Array|Length _mission14))))))

(event Custom|GameEnd
  (bind _result (Math|Integer|DecrementInt (Variables|Default|GetMission16Num))
    (:%20%20
      (if (<= _result 0)
        (if (not (Variables|Default|GetIsLevelMain))
          (Default|CallAllMissionOver))))))

(event Custom|CallMission4
  (bind _mission4 (Variables|Default|GetMission4))
  (bind _result (Math|Integer|DecrementInt (Variables|Default|GetMission3Num))
    (:%20%20
      (if (<= _result 0)
        (for _array_element _mission4
          (Default|MissionStartandShowThis _array_element)
          (Variables|Default|SetRelativeMission _mission4)
          (EventDispatchers|BindEventtoMissionSuccess _mission4 (delegate Custom|CallMission5))
          (Default|CallMissionChange))
        (Variables|Default|SetMission4Num (Utilities|Array|Length _mission4))))))

(event Custom|CallMission3
  (bind _mission3 (Variables|Default|GetMission3))
  (bind _result (Math|Integer|DecrementInt (Variables|Default|GetMission2Num))
    (:%20%20
      (if (<= _result 0)
        (for _array_element _mission3
          (Default|MissionStartandShowThis _array_element)
          (Variables|Default|SetRelativeMission _mission3)
          (EventDispatchers|BindEventtoMissionSuccess _mission3 (delegate Custom|CallMission4))
          (Default|CallMissionChange))
        (Variables|Default|SetMission3Num (Utilities|Array|Length _mission3))))))

(event Custom|CallMission5
  (bind _mission5 (Variables|Default|GetMission5))
  (bind _result (Math|Integer|DecrementInt (Variables|Default|GetMission4Num))
    (:%20%20
      (if (<= _result 0)
        (for _array_element _mission5
          (Default|MissionStartandShowThis _array_element)
          (Variables|Default|SetRelativeMission _mission5)
          (EventDispatchers|BindEventtoMissionSuccess _mission5 (delegate Custom|CallMission6))
          (Default|CallMissionChange))
        (Variables|Default|SetMission5Num (Utilities|Array|Length _mission5))))))

(event Custom|CallMission10
  (bind _mission10 (Variables|Default|GetMission10))
  (bind _result (Math|Integer|DecrementInt (Variables|Default|GetMission9Num))
    (:%20%20
      (if (<= _result 0)
        (for _array_element _mission10
          (Default|MissionStartandShowThis _array_element)
          (Variables|Default|SetRelativeMission _mission10)
          (EventDispatchers|BindEventtoMissionSuccess _mission10 (delegate Custom|CallMission11))
          (Default|CallMissionChange))
        (Variables|Default|SetMission10Num (Utilities|Array|Length _mission10))))))

(event Custom|CallMission6
  (bind _mission6 (Variables|Default|GetMission6))
  (bind _result (Math|Integer|DecrementInt (Variables|Default|GetMission5Num))
    (:%20%20
      (if (<= _result 0)
        (for _array_element _mission6
          (Default|MissionStartandShowThis _array_element)
          (Variables|Default|SetRelativeMission _mission6)
          (EventDispatchers|BindEventtoMissionSuccess _mission6 (delegate Custom|CallMission7))
          (Default|CallMissionChange))
        (Variables|Default|SetMission6Num (Utilities|Array|Length _mission6))))))

(event Custom|CallMission11
  (bind _mission11 (Variables|Default|GetMission11))
  (bind _result (Math|Integer|DecrementInt (Variables|Default|GetMission10Num))
    (:%20%20
      (if (<= _result 0)
        (for _array_element _mission11
          (Default|MissionStartandShowThis _array_element)
          (Variables|Default|SetRelativeMission _mission11)
          (EventDispatchers|BindEventtoMissionSuccess _mission11 (delegate Custom|CallMission12))
          (Default|CallMissionChange))
        (Variables|Default|SetMission11Num (Utilities|Array|Length _mission11))))))

(event Custom|CallMission7
  (bind _mission7 (Variables|Default|GetMission7))
  (bind _result (Math|Integer|DecrementInt (Variables|Default|GetMission6Num))
    (:%20%20
      (if (<= _result 0)
        (for _array_element _mission7
          (Default|MissionStartandShowThis _array_element)
          (Variables|Default|SetRelativeMission _mission7)
          (EventDispatchers|BindEventtoMissionSuccess _mission7 (delegate Custom|CallMission8))
          (Default|CallMissionChange))
        (Variables|Default|SetMission7Num (Utilities|Array|Length _mission7))))))

(event EventBeginPlay
  (Utilities|FlowControl|Delay 0.1)
  (CallFunction|CallMission1)
  (Default|CallMissionChange))

(fn ConstructionScript)