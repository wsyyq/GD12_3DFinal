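; BP_DialogueManager is a dialogue manager that plays spoken lines for three characters: Mrs. Lailah, Abel Eden and Mr. Judas.
; PlayDialogue switches on the speaker to pick that character's voice, builds a dialogue context targeting the given listener, and plays the line at a world location.
; All three branches share the character attenuation settings.
; BeginPlay caches the player character, although PlayDialogue does not use it.
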(event EventBeginPlay
  (bind _asbp_3dcharacter_p (Utilities|Casting|CastToBP_3DCharacter_P (Game|Player|GetPlayerPawn 0)))
  (Variables|Default|SetPlayer _asbp_3dcharacter_p))

(fn ConstructionScript)

(fn PlayDialogue
  (params (Speaker :type E_TargetType%20Enum :default "NewEnumerator0") (Listener :type Dialogue%20Voice%20Object%20Reference) (Dialogue :type Dialogue%20Wave%20Object%20Reference) (Location :type Vector))
  (switch Utilities|FlowControl|Switch|SwitchonE_TargetType Speaker
    (:NewEnumerator0
      (Class|GameplayStatics|PlayDialogueatLocation Dialogue (Utilities|Struct|MakeDialogueContext (Variables|Default|GetLailahVoice) (Utilities|Array|MakeArray Listener)) Location "0, 0, 0" 1.0 1.0 0.0 "/Game/GD12_3D/Audio/Attenuation/ATT_Character.ATT_Character"))
    (:NewEnumerator1
      (Class|GameplayStatics|PlayDialogueatLocation Dialogue (Utilities|Struct|MakeDialogueContext (Variables|Default|GetAbelVoice) (Utilities|Array|MakeArray Listener)) Location "0, 0, 0" 1.0 1.0 0.0 "/Game/GD12_3D/Audio/Attenuation/ATT_Character.ATT_Character"))
    (:NewEnumerator2
      (Class|GameplayStatics|PlayDialogueatLocation Dialogue (Utilities|Struct|MakeDialogueContext (Variables|Default|GetJudasVoice) (Utilities|Array|MakeArray Listener)) Location "0, 0, 0" 1.0 1.0 0.0 "/Game/GD12_3D/Audio/Attenuation/ATT_Character.ATT_Character"))))