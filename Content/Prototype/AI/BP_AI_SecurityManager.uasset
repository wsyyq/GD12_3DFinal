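; Security Manager NPC "Mr. Judas", whom the player can talk to, shoot or assassinate.
; Trigger overlaps toggle an interact widget, and PawnSensing walks him to the player on first sight, then fires the finish-interact call.
; Damage kills him unless protection, shown by NSProtection, is active.
; Assassination snaps the player to a spot, sets melee state flags on both, logs a hint, and reports his death to the player.
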(event OnSeePawn(PawnSensing)
  (params (Pawn :type Pawn%20Object%20Reference))
  (bind _player (Variables|Default|GetPlayer))
  (Utilities|Casting|CastToBP_3DCharacter_P Pawn)
  (if (Components|Activation|IsActive (Variables|Default|GetPawnSensing))
    (Utilities|FlowControl|DoOnce false
      (:Completed
        (Utilities|FlowControl|Delay 0.2)
        (Utilities|FlowControl|Sequence
          (:then_0
            (AI|AIMoveTo (AI|GetAIController self) (Transformation|GetActorLocation _player) _player 1.5e+02 "Enable" "Default" true true))
          (:then_1
            (Default|CallEventFinishInteract)))))))

(event OnComponentBeginOverlap(DialogueTrigger)
  (params (OverlappedComponent :type Primitive%20Component%20Object%20Reference) (OtherActor :type Actor%20Object%20Reference) (OtherComp :type Primitive%20Component%20Object%20Reference) (OtherBodyIndex :type Integer) (bFromSweep :type Boolean) (SweepResult :type Hit%20Result%20Structure%20%28by%20ref%29))
  (bind _interactwidget (Variables|Default|GetInteractWidget))
  (bind _returnvalue (UserInterface|GetWidget _interactwidget))
  (bind _aswbp_interact_panel (Utilities|Casting|CastToWBP_InteractPanel _returnvalue))
  (Utilities|Casting|CastToBP_3DCharacter_P OtherActor)
  (Development|SetHiddeninGame _interactwidget false false)
  (if (Variables|Default|GetIsKnown)
    (Default|ShowObjectType _aswbp_interact_panel "NewEnumerator14" "Security Manager" "Mr. Judas" true)
    (else
      (Default|ShowObjectType _aswbp_interact_panel "NewEnumerator14" "? ? ?" "" true))))

(event OnComponentEndOverlap(DialogueTrigger)
  (params (OverlappedComponent :type Primitive%20Component%20Object%20Reference) (OtherActor :type Actor%20Object%20Reference) (OtherComp :type Primitive%20Component%20Object%20Reference) (OtherBodyIndex :type Integer))
  (Utilities|Casting|CastToBP_3DCharacter_P OtherActor)
  (Development|SetHiddeninGame (Variables|Default|GetInteractWidget) true false))

(event OnComponentBeginOverlap(AsassinateTrigger)
  (params (OverlappedComponent :type Primitive%20Component%20Object%20Reference) (OtherActor :type Actor%20Object%20Reference) (OtherComp :type Primitive%20Component%20Object%20Reference) (OtherBodyIndex :type Integer) (bFromSweep :type Boolean) (SweepResult :type Hit%20Result%20Structure%20%28by%20ref%29))
  (bind _interactwidget (Variables|Default|GetInteractWidget))
  ;[0.15 0.15 0.15 0.5] WBP
  (Utilities|Casting|CastToBP_3DCharacter_P OtherActor)
  (Development|SetHiddeninGame _interactwidget false false)
  (Default|ShowObjectType (.AsWBP%20Interact%20Panel (Utilities|Casting|CastToWBP_InteractPanel (UserInterface|GetWidget _interactwidget))) "NewEnumerator14" "" "" false))

(event OnComponentEndOverlap(AsassinateTrigger)
  (params (OverlappedComponent :type Primitive%20Component%20Object%20Reference) (OtherActor :type Actor%20Object%20Reference) (OtherComp :type Primitive%20Component%20Object%20Reference) (OtherBodyIndex :type Integer))
  ;[0.15 0.15 0.15 0.5] WBP
  (Utilities|Casting|CastToBP_3DCharacter_P OtherActor)
  (Development|SetHiddeninGame (Variables|Default|GetInteractWidget) true false))

(event Custom|EnterSecurityRoom
  (Components|Activation|Activate (Variables|Default|GetPawnSensing) false))

(event Custom|Death
  (params (IsShooted :type Boolean))
  ;[0.15 0.15 0.15 0.5] Death
  (if IsShooted
    (Variables|Default|SetIsShootKilled true)
    (else
      (Variables|Default|SetIsMeleeKilled true)))
  (Variables|Default|SetIsDied true)
  (Default|CallManagerDeath (Variables|Default|GetPlayer)))

(event Custom|TalkAnimation
  (Variables|Default|SetIsMaleTalking true))

(event Custom|CheckInvincibility
  (params (IsInvincible :type Boolean))
  ;[0.15 0.15 0.15 0.5] If Invincible
  (if (!= IsInvincible (Variables|Default|GetIsInvincible))
    (bind _output_get (Variables|Default|SetIsInvincible IsInvincible))
    (if _output_get
      (Development|SetHiddeninGame (Variables|Default|GetNS_Protection) false false)
      (else
        (Development|SetHiddeninGame (Variables|Default|GetNS_Protection) true false)))))

(event Game|Damage|EventAnyDamage
  (params (Damage :type Float%20%28single-precision%29) (DamageType :type Damage%20Type%20Object%20Reference) (InstigatedBy :type Controller%20Object%20Reference) (DamageCauser :type Actor%20Object%20Reference))
  ;[0.15 0.15 0.15 0.5] Hit
  (if (not (Variables|Default|GetIsInvincible))
    (Variables|Default|SetIsHit true)
    (Utilities|FlowControl|Sequence
      (:then_0
        (Utilities|FlowControl|Delay 2.0)
        (Variables|Default|SetIsHit false))
      (:then_1
        (CallFunction|Death true)))))

(event EventBeginPlay
  (Utilities|FlowControl|Sequence
    (:then_0
      (bind _asbp_3dcharacter_p (Utilities|Casting|CastToBP_3DCharacter_P (Game|Player|GetPlayerPawn 0)))
      (Variables|Default|SetPlayer _asbp_3dcharacter_p))
    (:then_1
      (EventDispatchers|BindEventtoEventFinishInteract (delegate Custom|TalkAnimation)))))

(event EventAssassinate
  (bind _player (Variables|Default|GetPlayer))
  (bind _player_2 (Variables|Default|GetPlayer))
  ;[0.15 0.15 0.15 0.5] Assassinate
  (Utilities|FlowControl|Sequence
    (:then_0
      _)
    (:then_1
      (if (Variables|/Game/Prototype/GameMode/BP_3DCharacter_P.BP_3DCharacter_P_C|GetCanMelee (Variables|Default|GetPlayer))
        (Utilities|FlowControl|Delay 1.0))
      (CallFunction|Death false)))
  (Variables|Default|SetIsBeingMelee true)
  (Utilities|FlowControl|Sequence
    (:then_0
      (Utilities|FlowControl|Sequence
        (:then_0
          (if (Variables|/Game/Prototype/GameMode/BP_3DCharacter_P.BP_3DCharacter_P_C|GetCanMelee (Variables|Default|GetPlayer))
            (Utilities|FlowControl|Delay 2.5)
            (else
              (Utilities|FlowControl|Delay 1.5)))
          (Variables|/Game/Prototype/GameMode/BP_3DCharacter_P.BP_3DCharacter_P_C|SetCanMelee _player false)
          (Variables|/Game/Prototype/GameMode/BP_3DCharacter_P.BP_3DCharacter_P_C|SetIsMelee _player false)
          (Variables|/Game/Prototype/GameMode/BP_3DCharacter_P.BP_3DCharacter_P_C|SetCanMove _player true)
          (Variables|Default|SetIsBeingMelee false))
        (:then_1
          (Default|HideObjectType (.AsWBP%20Interact%20Panel (Utilities|Casting|CastToWBP_InteractPanel (UserInterface|GetWidget (Variables|Default|GetInteractWidget))))))))
    (:then_1
      (Utilities|FlowControl|DoOnce false
        (:Completed
          (Default|AddHint _player_2 "Manager" "Mr. Judas" false true)
          (Default|SetHint _player_2)
          (Default|SetLog _player_2 false "" "" (Variables|/Game/Prototype/GameMode/BP_3DCharacter_P.BP_3DCharacter_P_C|GetHintLog _player_2)))))))

(fn ConstructionScript
  (Variables|/Script/Engine.CharacterMovementComponent|SetMaxWalkSpeed (Variables|Character|GetCharacterMovement) 2e+02))

(fn E2Interactive
  (Default|HideObjectType (.AsWBP%20Interact%20Panel (Utilities|Casting|CastToWBP_InteractPanel (UserInterface|GetWidget (Variables|Default|GetInteractWidget)))))
  (Default|CallEventFinishInteract)
  (return false "NewEnumerator14" self 0 "" ""))

(fn IsTargetAlive
  (return (not (Variables|Default|GetIsDied))))

(fn TryAssassinate
  (return 0))

(fn TryAssassinateHuman
  (bind _assassinate_spot (Variables|Default|GetAssassinate%20Spot))
  (bind _player (Variables|Default|GetPlayer))
  (bind _returnvalue (Transformation|GetWorldTransform _assassinate_spot))
  (bind (_location _rotation) (Math|Transform|BreakTransform _returnvalue))
  (Transformation|SetActorLocationAndRotation _player _location _rotation)
  (Variables|/Game/Prototype/GameMode/BP_3DCharacter_P.BP_3DCharacter_P_C|SetCanMove _player false)
  (if (Variables|/Script/Engine.Character|GetbIsCrouched _player)
    (Variables|/Game/Prototype/GameMode/BP_3DCharacter_P.BP_3DCharacter_P_C|SetCanMelee _player true)
    (else
      (Variables|/Game/Prototype/GameMode/BP_3DCharacter_P.BP_3DCharacter_P_C|SetIsMelee _player true)))
  (Variables|Default|SetIsBeingMelee true)
  (return self))