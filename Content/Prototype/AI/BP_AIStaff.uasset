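; BP_AIStaff is a prototype civilian staff NPC that screams, alerts nearby guards and flees on seeing the player.
; The AlertBox overlap volume maintains a list of BP_AIGuard_P guards, which are sent the player's location when PawnSensing spots a BP_3DCharacter_P.
; It then moves to RunningEndPostion and destroys itself on arrival, with a ShouldFlee flag blocking further reactions.
; The construction script picks the skeletal mesh and scream sound from StuffType.
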(event OnSeePawn(PawnSensing)
  (params (Pawn :type Pawn%20Object%20Reference))
  (bind _myscreamsound (Variables|Default|GetMyScreamSound))
  ;[0.15 0.15 0.15 0.5] 看到玩家
  (if (not (Variables|Default|GetShouldFlee))
    (bind _asbp_3dcharacter_p (Utilities|Casting|CastToBP_3DCharacter_P Pawn))
    (Utilities|IsValid _myscreamsound
      (:Is%20Valid
        (CallFunction|Scream _myscreamsound)
        (CallFunction|SeePlayerAlert (Transformation|GetActorLocation _asbp_3dcharacter_p))
        (CallFunction|RunAway)
        (Variables|Default|SetShouldFlee true)))))

(event OnComponentBeginOverlap(AlertBox)
  (params (OverlappedComponent :type Primitive%20Component%20Object%20Reference) (OtherActor :type Actor%20Object%20Reference) (OtherComp :type Primitive%20Component%20Object%20Reference) (OtherBodyIndex :type Integer) (bFromSweep :type Boolean) (SweepResult :type Hit%20Result%20Structure%20%28by%20ref%29))
  ;[0.15 0.15 0.15 0.5] 更改会被通知的AI
  (if (not (Variables|Default|GetShouldFlee))
    (bind _asbp_aiguard_p (Utilities|Casting|CastToBP_AIGuard_P OtherActor))
    (Utilities|Array|Add (Variables|Default|GetSensingAI) _asbp_aiguard_p)))

(event OnComponentEndOverlap(AlertBox)
  (params (OverlappedComponent :type Primitive%20Component%20Object%20Reference) (OtherActor :type Actor%20Object%20Reference) (OtherComp :type Primitive%20Component%20Object%20Reference) (OtherBodyIndex :type Integer))
  ;[0.15 0.15 0.15 0.5] 更改会被通知的AI
  (if (not (Variables|Default|GetShouldFlee))
    (bind _asbp_aiguard_p (Utilities|Casting|CastToBP_AIGuard_P OtherActor))
    (Utilities|Array|RemoveItem (Variables|Default|GetSensingAI) _asbp_aiguard_p)))

(event Custom|SeePlayerAlert
  (params (PlayerCharacterLocation :type Vector))
  (bind _sensingai (Variables|Default|GetSensingAI))
  ;[0.15 0.15 0.15 0.5] 通知其他AI
  (for _array_element _sensingai
    (Utilities|IsValid _array_element
      (:Is%20Valid
        (Class|BIAIAlartandMoveP|AIMovetoAlartPlace(Message) _array_element PlayerCharacterLocation))
      (:Is%20Not%20Valid
        (Utilities|Array|RemoveItem _sensingai _array_element)))))

(event Custom|RunAway
  ;[0.15 0.15 0.15 0.5] 到达目标点后消失
  (AI|AIMoveTo self (Transformation|GetWorldLocation (Variables|Default|GetRunningEndPostion)) 0 5.0 false
    (:OnSuccess
      (Actor|DestroyActor))))

(event Custom|Scream
  (params (ScreamSound :type Sound%20Base%20Object%20Reference))
  ;[0.15 0.15 0.15 0.5] 叫
  (Audio|PlaySoundatLocation ScreamSound (Transformation|GetActorLocation) "0, 0, 0" 1.0 1.0 0.0 0 0 0 0))

(fn ConstructionScript
  (switch Utilities|FlowControl|Switch|SwitchonE_StuffTypes (Variables|Default|GetStuffType)
    (:NewEnumerator0
      ;[0.15 0.15 0.15 0.5] 根据所选种类更换Mesh
      (Components|SkeletalMesh|SetSkeletalMeshAsset (Variables|Character|GetMesh) (Utilities|Array|Get(acopy) (Variables|Default|GetSkeletalMeshes)))
      ;[0.15 0.15 0.15 0.5] 设置尖叫声
      (Variables|Default|SetMyScreamSound (Utilities|Array|Get(acopy) (Variables|Default|GetScreamSounds))))
    (:NewEnumerator1
      (Components|SkeletalMesh|SetSkeletalMeshAsset (Variables|Character|GetMesh) (Utilities|Array|Get(acopy) (Variables|Default|GetSkeletalMeshes) 2))
      (Variables|Default|SetMyScreamSound (Utilities|Array|Get(acopy) (Variables|Default|GetScreamSounds) 1)))
    (:NewEnumerator2
      (Components|SkeletalMesh|SetSkeletalMeshAsset (Variables|Character|GetMesh) (Utilities|Array|Get(acopy) (Variables|Default|GetSkeletalMeshes) 1))
      (Variables|Default|SetMyScreamSound (Utilities|Array|Get(acopy) (Variables|Default|GetScreamSounds) 2)))))