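; Second boss AI, shielded by an invincibility effect while any of its four assigned guard AIs is working.
; Each guard's death triggers a boss-fight ammo spawn and a respawn timer; the shield drops only when all four are down and returns on a respawn.
; Any damage to the unshielded boss kills it immediately, notifies the player and cleans up only guards 1 and 2; the two-hit logic is disconnected.
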(event Custom|BossStartWorking
  (Utilities|FlowControl|Sequence
    (:then_0
      ;[0.15 0.15 0.15 0.5] Boss获取玩家
      (bind _asbp_3dcharacter_p (Utilities|Casting|CastToBP_3DCharacter_P (Game|Player|GetPlayerPawn 0)))
      (Variables|Default|SetPlayer _asbp_3dcharacter_p))
    (:then_1
      ;[0.15 0.15 0.15 0.5] 开始时，为无敌状态IsInvincible
      (Variables|Default|SetIsInvincible true))
    (:then_2
      (bind _sonai1 (Variables|Default|GetSonAI1)
        (:then
          (EventDispatchers|BindEventtoEventAIDie _sonai1 (delegate Custom|CheckTwoAIAfter15s_AI1))
          (EventDispatchers|BindEventtoEventAIReborn _sonai1 (delegate Custom|OpenBossProtection)))
        (:else
          (Development|PrintString "BossAISonA1未设置"))))
    (:then_3
      (bind _sonai2 (Variables|Default|GetSonAI2)
        (:then
          (EventDispatchers|BindEventtoEventAIDie _sonai2 (delegate Custom|CheckTwoAIAfter15s_AI2))
          (EventDispatchers|BindEventtoEventAIReborn _sonai2 (delegate Custom|OpenBossProtection)))
        (:else
          (Development|PrintString "BossAISonA2未设置"))))
    (:then_6
      (bind _sonai3 (Variables|Default|GetSonAI3)
        (:then
          (EventDispatchers|BindEventtoEventAIDie _sonai3 (delegate Custom|CheckTwoAIAfter15s_AI3))
          (EventDispatchers|BindEventtoEventAIReborn _sonai3 (delegate Custom|OpenBossProtection)))
        (:else
          (Development|PrintString "BossAISonA3未设置"))))
    (:then_7
      (bind _sonai4 (Variables|Default|GetSonAI4)
        (:then
          (EventDispatchers|BindEventtoEventAIDie _sonai4 (delegate Custom|CheckTwoAIAfter15s_AI4))
          (EventDispatchers|BindEventtoEventAIReborn _sonai4 (delegate Custom|OpenBossProtection)))
        (:else
          (Development|PrintString "BossAISonA4未设置"))))))

(event Custom|SecondBossDeath
  ;[0.15 0.15 0.15 0.5] Boss死亡
  (Variables|Anim|SetIsShootKilled true)
  (Default|CallBossSecondDeath (Variables|Default|GetPlayer)))

(event Custom|CanNotBeScanned
  ;[0.15 0.15 0.15 0.5] 能否被扫描到
  (Rendering|SetRenderCustomDepth (Variables|Character|GetMesh) false))

(event Custom|CanBeScanned
  ;[0.15 0.15 0.15 0.5] 能否被扫描到
  (Rendering|SetRenderCustomDepth (Variables|Character|GetMesh) true))

(event Custom|CheckShouldRebornAI2
  ;[0.15 0.15 0.15 0.5] AI死亡15秒后复活
  (CallFunction|CheckShouldReborn (Variables|Default|GetSonAI2Timer) (Variables|Default|GetSonAI2)))

(event Custom|CheckTwoAIAfter15s_AI2
  ;[0.15 0.15 0.15 0.5] AI死亡15秒后复活
  (Default|AISpawnAmmoBossFightOnly (stale Custom|BossStartWorking _sonai2))
  (bind _returnvalue (Utilities|Time|SetTimerbyEvent (delegate Custom|CheckShouldRebornAI2) (Variables|Default|GetAIRebornDuration)))
  (Variables|Default|SetSonAI2Timer _returnvalue)
  (Variables|Default|SetIsAI2Die true)
  (CallFunction|CloseBossProtection))

(event Custom|CheckTwoAIAfter15s_AI3
  ;[0.15 0.15 0.15 0.5] AI死亡15秒后复活
  (Default|AISpawnAmmoBossFightOnly (stale Custom|BossStartWorking _sonai3))
  (bind _returnvalue (Utilities|Time|SetTimerbyEvent (delegate Custom|CheckShouldRebornAI3) (Variables|Default|GetAIRebornDuration)))
  (Variables|Default|SetSonAI3Timer _returnvalue)
  (Variables|Default|SetIsAI3Die true)
  (CallFunction|CloseBossProtection))

(event Custom|CheckShouldRebornAI3
  ;[0.15 0.15 0.15 0.5] AI死亡15秒后复活
  (CallFunction|CheckShouldReborn (Variables|Default|GetSonAI3Timer) (Variables|Default|GetSonAI3)))

(event Custom|SetMySon
  (params (SonAI1 :type BP%20AI%20Guard%20Object%20Reference%20%28by%20ref%29) (SonAI2 :type BP%20AI%20Guard%20Object%20Reference%20%28by%20ref%29) (SonAI3 :type BP%20AI%20Guard%20Object%20Reference%20%28by%20ref%29) (SonAI4 :type BP%20AI%20Guard%20Object%20Reference%20%28by%20ref%29))
  (Variables|Default|SetSonAI1 SonAI1)
  (Variables|Default|SetSonAI2 SonAI2)
  (Variables|Default|SetSonAI3 SonAI3)
  (Variables|Default|SetSonAI4 SonAI4))

(event Custom|CheckTwoAIAfter15s_AI1
  ;[0.15 0.15 0.15 0.5] AI死亡15秒后复活
  (Default|AISpawnAmmoBossFightOnly (stale Custom|BossStartWorking _sonai1))
  (bind _returnvalue (Utilities|Time|SetTimerbyEvent (delegate Custom|CheckShouldRebornAI1) (Variables|Default|GetAIRebornDuration)))
  (Variables|Default|SetSonAI1Timer _returnvalue)
  (Variables|Default|SetIsAI1Die true)
  (CallFunction|CloseBossProtection))

(event Custom|CheckShouldRebornAI1
  ;[0.15 0.15 0.15 0.5] AI死亡15秒后复活
  (CallFunction|CheckShouldReborn (Variables|Default|GetSonAI1Timer) (Variables|Default|GetSonAI1)))

(event Custom|CheckTwoAIAfter15s_AI4
  ;[0.15 0.15 0.15 0.5] AI死亡15秒后复活
  (Default|AISpawnAmmoBossFightOnly (stale Custom|BossStartWorking _sonai4))
  (bind _returnvalue (Utilities|Time|SetTimerbyEvent (delegate Custom|CheckShouldRebornAI4) (Variables|Default|GetAIRebornDuration)))
  (Variables|Default|SetSonAI4Timer _returnvalue)
  (Variables|Default|SetIsAI4Die true)
  (CallFunction|CloseBossProtection))

(event Custom|CheckShouldRebornAI4
  ;[0.15 0.15 0.15 0.5] AI死亡15秒后复活
  (CallFunction|CheckShouldReborn (Variables|Default|GetSonAI4Timer) (Variables|Default|GetSonAI4)))

(event Custom|ChangeInvincibleState
  (params (IsInvincible :type Boolean))
  ;[0.15 0.15 0.15 0.5] 改变BOSS是否当前为无敌
  (if (!= IsInvincible (Variables|Default|GetIsInvincible))
    (bind _output_get (Variables|Default|SetIsInvincible IsInvincible))
    (if _output_get
      (Development|SetHiddeninGame (Variables|Default|GetNS_Protection) false false)
      (Variables|Anim|SetHasSheild true)
      (else
        (Development|SetHiddeninGame (Variables|Default|GetNS_Protection) true false)
        (Variables|Anim|SetHasSheild false)))))

(event Custom|CloseBossProtection
  ;[0.15 0.15 0.15 0.5] 如果四个AI都死亡，则关闭BOSS防护罩
  (if (Math|Boolean|ANDBoolean (not (Default|IsAIWorking (Variables|Default|GetSonAI1))) (not (Default|IsAIWorking (Variables|Default|GetSonAI2))) (not (Default|IsAIWorking (Variables|Default|GetSonAI3))) (not (Default|IsAIWorking (Variables|Default|GetSonAI4))))
    (CallFunction|ChangeInvincibleState false)))

(event Custom|OpenBossProtection
  ;[0.15 0.15 0.15 0.5] 如果四AI有其一还存活，则打开BOSS防护罩
  (if (Math|Boolean|ORBoolean (Default|IsAIWorking (Variables|Default|GetSonAI1)) (Default|IsAIWorking (Variables|Default|GetSonAI2)) (Default|IsAIWorking (Variables|Default|GetSonAI3)) (Default|IsAIWorking (Variables|Default|GetSonAI4)))
    (CallFunction|ChangeInvincibleState true)))

(event Custom|CheckShouldReborn
  (params (TimeHandle :type Timer%20Handle%20Structure%20%28by%20ref%29) (BPAIGuard :type BP%20AI%20Guard%20Object%20Reference%20%28by%20ref%29))
  ;[0.15 0.15 0.15 0.5] AI死亡15秒后复活
  (if (Utilities|Time|IsValidTimerHandle TimeHandle)
    (Utilities|Time|ClearandInvalidateTimerbyHandle TimeHandle)
    (if (not (Default|IsAIWorking BPAIGuard))
      (Default|DisappearorRebornSelf BPAIGuard false)
      (Variables|Default|SetIsAI1Die false)
      (Default|CallEventAIReborn BPAIGuard))))

(event Game|Damage|EventAnyDamage
  (params (Damage :type Float%20%28single-precision%29) (DamageType :type Damage%20Type%20Object%20Reference) (InstigatedBy :type Controller%20Object%20Reference) (DamageCauser :type Actor%20Object%20Reference))
  (bind _sonai1timer (Variables|Default|GetSonAI1Timer))
  (bind _sonai2timer (Variables|Default|GetSonAI2Timer))
  ;[0.15 0.15 0.15 0.5] Boss被攻击一次，防护罩恢复，被攻击两次，死亡
  (if (Variables|Default|GetIsInvincible)
    (Development|PrintString "Boss处于防护罩内攻击无效")
    (else
      (Utilities|FlowControl|Sequence
        (:then_0
          (Variables|Anim|SetIsHit true)
          (Utilities|FlowControl|Delay 2.0)
          (Variables|Anim|SetIsHit false))
        (:then_1
          (Utilities|FlowControl|Sequence
            (:then_0
              (if (Utilities|Time|IsValidTimerHandle _sonai1timer)
                (Utilities|Time|ClearandInvalidateTimerbyHandle _sonai1timer)))
            (:then_1
              (if (Utilities|Time|IsValidTimerHandle _sonai2timer)
                (Utilities|Time|ClearandInvalidateTimerbyHandle _sonai2timer)))
            (:then_2
              (CallFunction|SecondBossDeath))
            (:then_3
              (Default|DisappearorRebornSelf (Variables|Default|GetSonAI1) true)
              (Default|DisappearorRebornSelf (Variables|Default|GetSonAI2) true))))))))

(event EventBeginPlay)

(fn ConstructionScript)