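; Civilian staff NPC that, on seeing the player, alerts nearby guards, screams and flees.
; An AlertBox overlap tracks guards in range, and PawnSensing sends them the player's location after a short retriggerable delay.
; If ScreamSound is valid, it plays type-specific audio, runs to RunningEndPostion and destroys itself.
; The construction script sets mesh and pose flags from StuffType and PoseType, assigning ScreamSound only for female types.
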(event OnSeePawn(PawnSensing)
  (params (Pawn :type Pawn%20Object%20Reference))
  ;[0.15 0.15 0.15 0.5] 看到玩家
  (if (not (Variables|Default|GetShouldFlee))
    (bind _asbp_3dcharacter_p (Utilities|Casting|CastToBP_3DCharacter_P Pawn))
    (Utilities|FlowControl|RetriggerableDelay 0.5)
    (CallFunction|SeePlayerAlert (Transformation|GetActorLocation _asbp_3dcharacter_p))
    (Variables|Default|SetShouldFlee true)
    (Utilities|IsValid (Variables|Default|GetScreamSound)
      (:Is%20Valid
        (CallFunction|Scream)
        (Utilities|FlowControl|Delay 1.0)
        (CallFunction|RunAway)))))

(event OnComponentBeginOverlap(AlertBox)
  (params (OverlappedComponent :type Primitive%20Component%20Object%20Reference) (OtherActor :type Actor%20Object%20Reference) (OtherComp :type Primitive%20Component%20Object%20Reference) (OtherBodyIndex :type Integer) (bFromSweep :type Boolean) (SweepResult :type Hit%20Result%20Structure%20%28by%20ref%29))
  ;[0.15 0.15 0.15 0.5] 更改会被通知的AI
  (if (not (Variables|Default|GetShouldFlee))
    (bind _asbp_aiguard_p (Utilities|Casting|CastToBP_AI_Guard OtherActor))
    (Utilities|Array|Add (Variables|Default|GetSensingAI) _asbp_aiguard_p)))

(event OnComponentEndOverlap(AlertBox)
  (params (OverlappedComponent :type Primitive%20Component%20Object%20Reference) (OtherActor :type Actor%20Object%20Reference) (OtherComp :type Primitive%20Component%20Object%20Reference) (OtherBodyIndex :type Integer))
  ;[0.15 0.15 0.15 0.5] 更改会被通知的AI
  (if (not (Variables|Default|GetShouldFlee))
    (bind _asbp_aiguard_p (Utilities|Casting|CastToBP_AI_Guard OtherActor))
    (Utilities|Array|RemoveItem (Variables|Default|GetSensingAI) _asbp_aiguard_p)))

(event Custom|SeePlayerAlert
  (params (PlayerCharacterLocation :type Vector))
  (bind _sensingai (Variables|Default|GetSensingAI))
  ;[0.15 0.15 0.15 0.5] 通知其他AI
  (for _array_element _sensingai
    (Utilities|IsValid _array_element
      (:Is%20Valid
        (Class|BIAIAlartandMoveP|AIMovetoAlartPlace(Message) _array_element PlayerCharacterLocation))
      (:Is%20Not%20Valid
        (Utilities|Array|RemoveItem _sensingai _array_element)))))

(event Custom|RunAway
  (bind _charactermovement (Variables|Character|GetCharacterMovement))
  ;[0.15 0.15 0.15 0.5] 到达目标点后消失
  (Variables|/Script/Engine.CharacterMovementComponent|SetMaxWalkSpeed _charactermovement 4e+02)
  (AI|AIMoveTo self (Variables|Default|GetTargetLocation) 0 5.0 false
    (:OnSuccess
      (Variables|/Script/Engine.CharacterMovementComponent|SetMaxWalkSpeed _charactermovement 0.0)
      (Utilities|FlowControl|Delay 1.0)
      (Actor|DestroyActor))))

(event Custom|Scream
  (bind _returnvalue (Transformation|GetActorLocation))
  (bind _self self)
  ;[0.15 0.15 0.15 0.5] 叫
  (switch Utilities|FlowControl|Switch|SwitchonE_StuffTypes (Variables|Default|GetStuffType)
    (:NewEnumerator0
      (Utilities|FlowControl|Delay 0.5)
      (Audio|PlaySoundatLocation "/Game/GD12_3D/Audio/Cue/A_Breath_Scream_Female_02_Cue.A_Breath_Scream_Female_02_Cue" _returnvalue "0, 0, 0" 1.0 1.0 0.0 0 0 _self 0))
    (:NewEnumerator1
      (Utilities|FlowControl|Delay 0.5)
      (Audio|PlaySoundatLocation "/Game/GD12_3D/Audio/Cue/A_Breath_Scream_Female_Cue.A_Breath_Scream_Female_Cue" _returnvalue "0, 0, 0" 1.0 1.0 0.0 0 0 _self 0))
    (:NewEnumerator2
      (Audio|PlaySoundatLocation "/Game/GD12_3D/Audio/Cue/A_NPC_Huh_Cue.A_NPC_Huh_Cue" _returnvalue "0, 0, 0" 1.0 1.1 0.0 0 0 _self 0)
      (Utilities|FlowControl|Delay 1.0)
      (Audio|PlaySoundatLocation "/Game/GD12_3D/Audio/Cue/A_NPC_She_Is_Here_Cue.A_NPC_She_Is_Here_Cue" _returnvalue "0, 0, 0" 1.0 1.1 0.0 0 0 _self 0))))

(event EventBeginPlay
  (Variables|Default|SetTargetLocation (Transformation|GetWorldLocation (Variables|Default|GetRunningEndPostion)))
  (Variables|/Script/Engine.CharacterMovementComponent|SetMaxWalkSpeed (Variables|Character|GetCharacterMovement) 0.0))

(fn ConstructionScript
  (bind _mesh (Variables|Character|GetMesh))
  (bind _mesh_2 (Variables|Character|GetMesh))
  (bind _mesh_3 (Variables|Character|GetMesh))
  (Utilities|FlowControl|Sequence
    (:then_0
      (switch Utilities|FlowControl|Switch|SwitchonE_StuffTypes (Variables|Default|GetStuffType)
        (:NewEnumerator0
          ;[0.15 0.15 0.15 0.5] 根据所选种类更换Mesh
          (Components|SkeletalMesh|SetSkeletalMeshAsset _mesh_2 (Utilities|Array|Get(acopy) (Variables|Default|GetSkeletalMeshes)))
          (Transformation|SetRelativeLocation _mesh_2 "0.000000,0.000000,-89.000000" false true)
          ;[0.15 0.15 0.15 0.5] 设置尖叫声
          (Variables|Default|SetScreamSound (Utilities|Array|Get(acopy) (Variables|Default|GetScreamSounds))))
        (:NewEnumerator1
          (Components|SkeletalMesh|SetSkeletalMeshAsset _mesh_3 (Utilities|Array|Get(acopy) (Variables|Default|GetSkeletalMeshes) 2))
          (Transformation|SetRelativeLocation _mesh_3 "0.000000,0.000000,-96.000000" false true)
          (Variables|Default|SetScreamSound (Utilities|Array|Get(acopy) (Variables|Default|GetScreamSounds) 1)))
        (:NewEnumerator2
          (Components|SkeletalMesh|SetSkeletalMeshAsset _mesh (Utilities|Array|Get(acopy) (Variables|Default|GetSkeletalMeshes) 1))
          (Transformation|SetRelativeLocation _mesh "0.000000,0.000000,-91.000000" false true))))
    (:then_1
      (switch Utilities|FlowControl|Switch|SwitchonE_PoseType (Variables|Default|GetPoseType)
        (:NewEnumerator0
          (Variables|Default|SetIsStandIdleF true))
        (:NewEnumerator4
          (Variables|Default|SetIsStandIdleM true))
        (:NewEnumerator1
          (Variables|Default|SetIsSitIdle true))
        (:NewEnumerator2
          (Variables|Default|SetIsStandTalkF true))
        (:NewEnumerator3
          (Variables|Default|SetIsStandScratchM true))
        (:NewEnumerator5
          (Variables|Default|SetIsSitTalkF true))
        (:NewEnumerator6
          (Variables|Default|SetIsSitTalkM true))
        (:NewEnumerator7
          (Variables|Default|SetIsStandWander true))))))