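; Prototype AI guard character that patrols and can be choked out, shot or hacked by the player.
; It ping-pongs along a PatrolPath spline with per-point waits, and can investigate in-range alert locations before resuming patrol.
; An AI state enum gates the paired-montage takedown and hack info, while a timer turns the hack widget toward the camera.
; Perception handlers are empty, and state changes only record and print.
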(event OnTargetPerceptionForgotten(AIPerception)
  (params (Actor :type Actor%20Object%20Reference))
  ;[0.15 0.15 0.15 0.5] AI视线检测
)

(event OnTargetPerceptionUpdated(AIPerception)
  (params (Actor :type Actor%20Object%20Reference) (Stimulus :type AI%20Stimulus%20Structure))
  ;[0.15 0.15 0.15 0.5] AI视线检测
)

(event Custom|AIPatrolToNextPoint
  ;[0.15 0.15 0.15 0.5] 巡逻逻辑
  (Utilities|IsValid (Variables|Patrol|GetPatrolPath)
    (:Is%20Valid
      ;;[0.149 0.02745 0.01569 0.502] 设置当前路线的巡逻点数量
      (Patrol|SetMaxPatrolPathPointNum)
      ;;[0.149 0.02745 0.01569 0.502] 移动向当前目标点
      (AI|AIMoveTo (AI|GetAIController self) (Spline|GetLocationatSplinePoint (Variables|/Game/Prototype/AI/BP_PatrolPath_P.BP_PatrolPath_P_C|GetSpline (Variables|Patrol|GetPatrolPath)) (- (Variables|Patrol|GetCurrentPatrolPointNum) 1) "World") 0 5.0 "Default" "Default" true true
        (:OnRequestFailed
          (Development|PrintString "AI can not move to next point"))
        (:OnMoveFinished
          ;;[0.149 0.02745 0.01569 0.502] 等待
          (Utilities|FlowControl|Delay (Utilities|Array|Get(acopy) (Variables|/Game/Prototype/AI/BP_PatrolPath_P.BP_PatrolPath_P_C|GetPointWaitTime (Variables|Patrol|GetPatrolPath)) (- (Variables|Patrol|GetCurrentPatrolPointNum) 1)))
          ;;[0.149 0.02745 0.01569 0.502] 设置下一个巡逻点
          (Patrol|SetNextPatrolPathPoint)
          ;;[0.149 0.02745 0.01569 0.502] 前往下一个巡逻点
          (Default|CallReachthePointandWaitforNextMove))))
    (:Is%20Not%20Valid
      (Development|PrintString "AI no patrol path"))))

(event EventBeginPlay
  (Utilities|FlowControl|Sequence
    (:then_0
      (Variables|Default|SetPlayer (Game|GetPlayerCharacter 0)))
    (:then_1
      (EventDispatchers|BindEventtoReachthePointandWaitforNextMove (delegate Custom|AIPatrolToNextPoint))
      (if (Variables|Move|GetShouldAIMoveAtStart)
        (Default|CallReachthePointandWaitforNextMove)))))

(event EventAIHacked
  ;[0.15 0.15 0.15 0.5] AI被骇入
  (Hack|ResetAIHackState true))

(event EventTryAssassinate
  (bind _returnvalue (Game|GetPlayerController 0))
  (bind _assassinate_point (Variables|Default|GetAssassinate%20Point))
  (bind _player (Variables|Default|GetPlayer))
  (bind _returnvalue_2 (Transformation|GetWorldTransform _assassinate_point))
  (bind (_location _rotation) (Math|Transform|BreakTransform _returnvalue_2))
  ;[0.15 0.15 0.15 0.5] 勒晕
  (switch Utilities|FlowControl|Switch|SwitchonE_AIState_P (Variables|State|GetAIState)
    (:NewEnumerator0
      (Development|PrintString "勒晕成功" :!label _label)
      (Utilities|FlowControl|Sequence
        (:then_0
          (Animation|Montage|PlayMontage (Variables|Character|GetMesh) "/Game/GD12_3D/Characters/Animations/Melee/AM_Assassinate.AM_Assassinate"
            (:OnCompleted
              (CallFunction|ChangeAIState "NewEnumerator4"))))
        (:then_1
          (Transformation|SetActorLocationAndRotation _player _location _rotation)
          (Input|DisableInput _player _returnvalue)
          (Animation|Montage|PlayMontage (Variables|/Script/Engine.Character|GetMesh _player) "/Game/GD12_3D/Characters/Animations/Melee/AM_Assassinate.AM_Assassinate"
            (:OnCompleted
              (Input|EnableInput _player _returnvalue))))))
    (:NewEnumerator1
      (goto _label))
    (:NewEnumerator2
      (Development|PrintString "无法暗杀" :!label _label_2))
    (:NewEnumerator3
      (goto _label_2))
    (:NewEnumerator4
      (goto _label_2))
    (:NewEnumerator5
      (goto _label_2))))

(event EventAIMovetoAlartPlace
  (params (TargetLocation :type Vector :default "0, 0, 0"))
  ;[0.15 0.15 0.15 0.5] AI前往怀疑点
  ;;[0.149 0.02745 0.01569 0.502] 目标警戒点是否在 巡逻感知范围 内， 前往该点（50CM范围），等待10秒后返回原位置
  (Math|Float|CompareFloat (Math|Vector|VectorLength (- TargetLocation (Transformation|GetActorLocation))) (Variables|Alert|GetPatrolSensingLength)
    (:>
      ;;[0.149 0.02745 0.01569 0.502] 目标警戒点是否在不在任何感知范围中
      (Development|PrintString "AI与警戒目标点：当前AI不在巡逻感知范围以及警戒感知范围中"))
    (:==
      (Development|PrintString "AI与警戒目标点：当前AI不在巡逻感知范围以及警戒感知范围" :!label _label)
      (AI|AIMoveTo self (+ TargetLocation (* (Math|Random|RandomUnitVector) 5e+01)) 0 5.0 false
        (:OnSuccess
          (Utilities|FlowControl|Delay (Variables|Alert|GetWaitTimeAfterReachingAlertTarget))
          (CallFunction|AIPatroltoNextPoint))))
    (:<
      (goto _label))))

(event EventAILeaveHackSenseRadius
  ;[0.15 0.15 0.15 0.5] AI被骇入
  (Hack|ShowHackInfoorNot false))

(event EventAIEnterHackSenseRadius
  ;[0.15 0.15 0.15 0.5] AI被骇入
  (Hack|ShowHackInfoorNot true))

(event EventAIShooted
  ;[0.15 0.15 0.15 0.5] 被射死
  (Variables|Default|SetIsDead true)
  (CallFunction|ChangeAIState "NewEnumerator4"))

(fn ConstructionScript
  (bind _charactermovement (Variables|Character|GetCharacterMovement))
  (Variables|/Script/Engine.CharacterMovementComponent|SetMaxWalkSpeed _charactermovement 4e+02)
  (Variables|/Script/Engine.CharacterMovementComponent|SetMaxWalkSpeedCrouched _charactermovement 2e+02))

(fn SetMaxPatrolPathPointNum
  ;[0.15 0.15 0.15 0.5] 巡逻路上有几个巡逻点
  (Variables|Patrol|SetMaxPatrolPointNum (Spline|GetNumberOfSplinePoints (Variables|/Game/Prototype/AI/BP_PatrolPath_P.BP_PatrolPath_P_C|GetSpline (Variables|Patrol|GetPatrolPath))))
  (return))

(fn SetNextPatrolPathPoint
  (if (Variables|Move|GetIsAIMoveForward)
    ;[0.15 0.15 0.15 0.5] AI按路线方向前进
    (Math|Integer|CompareInt (Variables|Patrol|GetCurrentPatrolPointNum) (Variables|Patrol|GetMaxPatrolPointNum)
      (:>
        _)
      (:==
        _)
      (:<
        (bind _result (Math|Integer|IncrementInt (Variables|Patrol|GetCurrentPatrolPointNum))
          (:%20%20
            (return _result)))))
    (bind _result_2 (Math|Integer|DecrementInt (Variables|Patrol|GetCurrentPatrolPointNum))
      (:%20%20
        (Variables|Move|SetIsAIMoveForward false)
        (return _result_2)))
    (else
      ;[0.15 0.15 0.15 0.5] AI按路线方向后退
      (Math|Integer|CompareInt (Variables|Patrol|GetCurrentPatrolPointNum) 1
        (:>
          (bind _result_3 (Math|Integer|DecrementInt (Variables|Patrol|GetCurrentPatrolPointNum))
            (:%20%20
              (return _result_3))))
        (:==
          _)
        (:<
          _))
      (bind _result_4 (Math|Integer|IncrementInt (Variables|Patrol|GetCurrentPatrolPointNum))
        (:%20%20
          (Variables|Move|SetIsAIMoveForward true)
          (return _result_4))))))

(fn ChangeAIState
  (params (NewAIState :type E_AIState_P%20Enum :default "NewEnumerator0"))
  (bind _output_get (LocalVariables|SetNowAIState NewAIState))
  (bind _output_get_2 (LocalVariables|SetBeforeAIState (Variables|State|GetAIState)))
  (Variables|State|SetAIState _output_get)
  (Development|PrintString (Utilities|String|Append "AI State from " (Utilities|String|EnumtoString _output_get_2) "to " (Utilities|String|EnumtoString _output_get)))
  (return))

(fn GetAIInfomation
  (switch Utilities|FlowControl|Switch|SwitchonE_AIState_P (Variables|State|GetAIState)
    (:NewEnumerator0
      (return (Variables|Insight|GetHackInfoAlive)))
    (:NewEnumerator1
      (return (Variables|Insight|GetHackInfoAlive)))
    (:NewEnumerator2
      (Development|PrintString "AI正在警戒无法骇入"))
    (:NewEnumerator3
      (Development|PrintString "AI正在战斗无法骇入"))
    (:NewEnumerator4
      (return (Variables|Insight|GetHackInfoDead)))
    (:NewEnumerator5
      (return (Variables|Insight|GetHackInfoDead)))))

(fn ResetAIHackState
  (params (IsInvestigated :type Boolean))
  (if IsInvestigated
    (bind _aswbp_abel_hack_state (Utilities|Casting|CastToWBP_AbelHackState (UserInterface|GetWidget (Variables|Default|GetWBP_AIHackState))))
    (Default|ChooseAIHackState _aswbp_abel_hack_state IsInvestigated)
    (else
      (bind _aswbp_abel_hack_state_2 (Utilities|Casting|CastToWBP_AbelHackState (UserInterface|GetWidget (Variables|Default|GetWBP_AIHackState))))
      (Default|ChooseAIHackState _aswbp_abel_hack_state_2 (not IsInvestigated)))))

(fn ShowHackInfoorNot
  (params (ShouldShowHackInfo :type Boolean))
  (if ShouldShowHackInfo
    ;[0.15 0.15 0.15 0.5] 出现
    (Development|SetHiddeninGame (Variables|Default|GetWBP_AIHackState) false false)
    ;[0.15 0.15 0.15 0.5] UI跟随玩家摄像机显示
    (bind _returnvalue (Utilities|Time|SetTimerbyFunctionName 0 "UIFollowPlayerCameraDoOnce" 0.05 true))
    (else
      ;[0.15 0.15 0.15 0.5] 消失
      (Development|SetHiddeninGame (Variables|Default|GetWBP_AIHackState) true false)
      (Utilities|Time|ClearandInvalidateTimerbyHandle _returnvalue))))

(fn UIFollowPlayerCameraDoOnce
  (Transformation|SetWorldRotation (Variables|Default|GetWBP_AIHackState) (Math|Rotator|MakeRotator 0.0 0.0 (.yaw (Math|Rotator|FindLookatRotation (Transformation|GetActorLocation) (Camera|GetCameraLocation (Variables|/Script/Engine.PlayerController|GetPlayerCameraManager (Game|GetPlayerController 0)))))) false false))