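; First boss AI character: plays an intro dialogue on first seeing the player, then fights behind an invincibility shield maintained by two minion AIs.
; Minion death events spawn ammo and start respawn timers; the shield drops while both are down and returns on a respawn.
; Any damage while unshielded kills the boss, cancelling respawns, removing both minions and notifying the player; the two-hit logic is left disconnected.
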(event OnSeePawn(PawnSensing)
  (params (Pawn :type Pawn%20Object%20Reference))
  (bind _returnvalue (Game|GetGameState))
  (bind _self self)
  (bind _asbp_3dgame_state_p (Utilities|Casting|CastToBP_3DGameState_P _returnvalue))
  (Utilities|Casting|CastToBP_3DCharacter_P Pawn)
  (Utilities|FlowControl|Delay 2.0)
  (Utilities|FlowControl|DoOnce false
    (:Completed
      (Variables|Anim|SetIsFemaleTalking true)
      (Default|PlayDialogue _asbp_3dgame_state_p _self "/Game/GD12_3D/Audio/Dialogue/Lailah/A_Lailah_07.A_Lailah_07")
      (Utilities|FlowControl|Delay 9.0)
      (Default|PlayDialogue _asbp_3dgame_state_p _self "/Game/GD12_3D/Audio/Dialogue/Lailah/A_Lailah_08.A_Lailah_08")
      (Utilities|FlowControl|Delay 5.0)
      (Variables|Anim|SetIsFemaleTalking false)
      (Default|CallEndFirstBossCG)
      (Variables|Default|SetIsInvincible true)
      (Default|PlayDialogue _asbp_3dgame_state_p (Variables|Default|GetPlayer) "/Game/GD12_3D/Audio/Dialogue/Abel/A_Abel_30.A_Abel_30"))))

(event Custom|BossStartWorking
  (Utilities|FlowControl|Sequence
    (:then_0
      ;[0.15 0.15 0.15 0.5] 进入Boss关，Boss获取玩家
      (bind _asbp_3dcharacter_p (Utilities|Casting|CastToBP_3DCharacter_P (Game|Player|GetPlayerPawn 0)))
      (Variables|Default|SetPlayer _asbp_3dcharacter_p))
    (:then_1
      ;[0.15 0.15 0.15 0.5] 开始时，为无敌状态IsInvincible
      (Variables|Default|SetIsInvincible true)
      (Development|SetHiddeninGame (Variables|Default|GetNS_Protection) false false))
    (:then_2
      ;[0.15 0.15 0.15 0.5] AI死亡15秒后复活
      (bind _sonai1 (Variables|Default|GetSonAI1)
        (:then
          (EventDispatchers|BindEventtoEventAIDie _sonai1 (delegate Custom|CheckTwoAIAfter15s_AI1)))
        (:else
          (Development|PrintString "BossAISonA1未设置"))))
    (:then_3
      (bind _sonai2 (Variables|Default|GetSonAI2)
        (:then
          (EventDispatchers|BindEventtoEventAIDie _sonai2 (delegate Custom|CheckTwoAIAfter15s_AI2)))
        (:else
          (Development|PrintString "BossAISonA2未设置"))))
    (:then_4
      (bind _sonai1_2 (Variables|Default|GetSonAI1)
        (:then
          (EventDispatchers|BindEventtoEventAIReborn _sonai1_2 (delegate Custom|OpenBossProtection)))
        (:else)))
    (:then_5
      (bind _sonai2_2 (Variables|Default|GetSonAI2)
        (:then
          (EventDispatchers|BindEventtoEventAIReborn _sonai2_2 (delegate Custom|OpenBossProtection)))
        (:else)))))

(event Custom|FirstBossDeath
  (bind _player (Variables|Default|GetPlayer))
  ;[0.15 0.15 0.15 0.5] Boss死亡
  (Utilities|IsValid _player
    (:Is%20Valid
      (Variables|/Game/Prototype/GameMode/BP_3DCharacter_P.BP_3DCharacter_P_C|SetIsFirstKilledBoss _player true)
      (Variables|Anim|SetIsShootKilled true)
      (Components|Activation|Deactivate (Variables|Default|GetPawnSensing))
      (Default|CallBossFirstDeath _player)
      (Default|CallEventFirstBossDie)
      (Development|PrintString "First Boss Death"))))

(event Custom|CanNotBeScanned
  ;[0.15 0.15 0.15 0.5] 能否被扫描到
  (Rendering|SetRenderCustomDepth (Variables|Character|GetMesh) false))

(event Custom|CanBeScanned
  ;[0.15 0.15 0.15 0.5] 能否被扫描到
  (Rendering|SetRenderCustomDepth (Variables|Character|GetMesh) true))

(event Custom|EnterLabRoom
  (Components|Activation|Activate (Variables|Default|GetPawnSensing) false))

(event Custom|CheckTwoAIAfter15s_AI1
  ;[0.15 0.15 0.15 0.5] AI死亡15秒后复活
  (Default|AISpawnAmmoBossFightOnly (stale Custom|BossStartWorking _sonai1))
  (bind _returnvalue (Utilities|Time|SetTimerbyEvent (delegate Custom|CheckShouldRebornAI1) (Variables|Default|GetAIRebornDuration)))
  (Variables|Default|SetSonAI1Timer _returnvalue)
  (Variables|Default|SetIsAI1Die true)
  (CallFunction|CloseBossProtection))

(event Custom|CheckShouldRebornAI1
  (bind _sonai1 (Variables|Default|GetSonAI1))
  (bind _sonai1timer (Variables|Default|GetSonAI1Timer))
  ;[0.15 0.15 0.15 0.5] AI死亡15秒后复活
  (if (Utilities|Time|IsValidTimerHandle _sonai1timer)
    (Utilities|Time|ClearandInvalidateTimerbyHandle _sonai1timer)
    (if (not (Default|IsAIWorking _sonai1))
      (Default|DisappearorRebornSelf _sonai1 false)
      (Variables|Default|SetIsAI1Die false)
      (Default|CallEventAIReborn _sonai1))))

(event Custom|CheckTwoAIAfter15s_AI2
  ;[0.15 0.15 0.15 0.5] AI死亡15秒后复活
  (Default|AISpawnAmmoBossFightOnly (stale Custom|BossStartWorking _sonai2))
  (bind _returnvalue (Utilities|Time|SetTimerbyEvent (delegate Custom|CheckShouldRebornAI2) (Variables|Default|GetAIRebornDuration)))
  (Variables|Default|SetSonAI2Timer _returnvalue)
  (Variables|Default|SetIsAI2Die true)
  (CallFunction|CloseBossProtection))

(event Custom|CheckShouldRebornAI2
  (bind _sonai2 (Variables|Default|GetSonAI2))
  (bind _sonai2timer (Variables|Default|GetSonAI2Timer))
  ;[0.15 0.15 0.15 0.5] AI死亡15秒后复活
  (if (Utilities|Time|IsValidTimerHandle _sonai2timer)
    (Utilities|Time|ClearandInvalidateTimerbyHandle _sonai2timer)
    (if (not (Default|IsAIWorking _sonai2))
      (Default|DisappearorRebornSelf _sonai2 false)
      (Variables|Default|SetIsAI2Die false)
      (Default|CallEventAIReborn _sonai2))))

(event Custom|ChangeInvincibleState
  (params (IsInvincible :type Boolean))
  ;[0.15 0.15 0.15 0.5] 改变BOSS是否当前为无敌
  (if (!= IsInvincible (Variables|Default|GetIsInvincible))
    (bind _output_get (Variables|Default|SetIsInvincible IsInvincible))
    (if _output_get
      (Development|SetHiddeninGame (Variables|Default|GetNS_Protection) false false)
      (Variables|Anim|SetHasSheild true)
      (else
        (Development|SetHiddeninGame (Variables|Default|GetNS_Protection) true false)
        (Variables|Anim|SetHasSheild false)))))

(event Custom|CloseBossProtection
  (bind _sonai1 (Variables|Default|GetSonAI1))
  (bind _sonai2 (Variables|Default|GetSonAI2))
  ;[0.15 0.15 0.15 0.5] 如果两个AI都死亡，则关闭BOSS防护罩
  (if (and (Utilities|IsValid _sonai1) (Utilities|IsValid _sonai2))
    (if (and (not (Default|IsAIWorking _sonai1)) (not (Default|IsAIWorking _sonai2)))
      (CallFunction|ChangeInvincibleState false))))

(event Custom|OpenBossProtection
  (bind _sonai1 (Variables|Default|GetSonAI1))
  (bind _sonai2 (Variables|Default|GetSonAI2))
  ;[0.15 0.15 0.15 0.5] 如果二AI有其一还存活，则打开BOSS防护罩
  (if (and (Utilities|IsValid _sonai1) (Utilities|IsValid _sonai2))
    (if (or (Default|IsAIWorking _sonai1) (Default|IsAIWorking _sonai2))
      (CallFunction|ChangeInvincibleState true))))

(event Custom|SetMySon
  (params (Son1 :type BP%20AI%20Guard%20Object%20Reference) (Son2 :type BP%20AI%20Guard%20Object%20Reference))
  (Variables|Default|SetSonAI1 Son1)
  (Variables|Default|SetSonAI2 Son2))

(event Game|Damage|EventAnyDamage
  (params (Damage :type Float%20%28single-precision%29) (DamageType :type Damage%20Type%20Object%20Reference) (InstigatedBy :type Controller%20Object%20Reference) (DamageCauser :type Actor%20Object%20Reference))
  (bind _sonai1timer (Variables|Default|GetSonAI1Timer))
  (bind _sonai2timer (Variables|Default|GetSonAI2Timer))
  ;[0.15 0.15 0.15 0.5] Boss被攻击一次，防护罩恢复，被攻击两次，死亡
  (if (Variables|Default|GetIsInvincible)
    (Development|PrintString "Boss处于防护罩内攻击无效")
    (else
      (Utilities|FlowControl|Sequence
        (:then_0
          (Variables|Anim|SetIsHit true)
          (Utilities|FlowControl|Delay 2.0)
          (Variables|Anim|SetIsHit false))
        (:then_1
          (Utilities|FlowControl|Sequence
            (:then_0
              (if (Utilities|Time|IsValidTimerHandle _sonai1timer)
                (Utilities|Time|ClearandInvalidateTimerbyHandle _sonai1timer)))
            (:then_1
              (if (Utilities|Time|IsValidTimerHandle _sonai2timer)
                (Utilities|Time|ClearandInvalidateTimerbyHandle _sonai2timer)))
            (:then_2
              (CallFunction|FirstBossDeath))
            (:then_3
              (Default|DisappearorRebornSelf (Variables|Default|GetSonAI1) true)
              (Default|DisappearorRebornSelf (Variables|Default|GetSonAI2) true))))))))

(event EventBeginPlay
  (Components|Activation|Deactivate (Variables|Default|GetPawnSensing))
  (Development|SetHiddeninGame (Variables|Default|GetNS_Protection) true false)
  (Variables|Default|SetIsInvincible false))

(fn ConstructionScript
  (Variables|/Script/Engine.CharacterMovementComponent|SetMaxWalkSpeed (Variables|Character|GetCharacterMovement) 2e+02))