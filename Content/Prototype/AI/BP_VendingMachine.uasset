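; AI-driven vending machine that patrols back and forth along the spline points of an assigned PatrolPath.
; BeginPlay binds the patrol event to the ReachThePointAndWaitForNextMove dispatcher and fires it, issuing an AI MoveTo toward the current point.
; Each finished move steps the one-based point index, reversing direction at either end, then fires the dispatcher again to continue the loop.
; A missing path or failed move request only prints a message.
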(event Custom|AIPatrolToNextPoint
  (Utilities|IsValid (Variables|Default|GetPatrolPath)
    (:Is%20Valid
      (CallFunction|SetMaxPatrolPointNum)
      (AI|AIMoveTo (AI|GetAIController self) (Spline|GetLocationatSplinePoint (Variables|/Game/Prototype/AI/BP_PatrolPath_P.BP_PatrolPath_P_C|GetSpline (Variables|Default|GetPatrolPath)) (- (Variables|Default|GetCurrentPatrolPointNum) 1) "World") 0 5.0 "Default" "Default" true true
        (:OnRequestFailed
          (Development|PrintString "AI cannot move to Next Point."))
        (:OnMoveFinished
          (CallFunction|SetNextPatrolPoint)
          (Default|CallReachthePointandWaitforNextMove))))
    (:Is%20Not%20Valid
      (Development|PrintString "NO Vending Machine Patrol Path."))))

(event EventBeginPlay
  (EventDispatchers|BindEventtoReachthePointandWaitforNextMove (delegate Custom|AIPatrolToNextPoint))
  (Default|CallReachthePointandWaitforNextMove))

(fn ConstructionScript)

(fn SetMaxPatrolPointNum
  (Variables|Default|SetMaxPatrolPointNum (Spline|GetNumberOfSplinePoints (Variables|/Game/Prototype/AI/BP_PatrolPath_P.BP_PatrolPath_P_C|GetSpline (Variables|Default|GetPatrolPath))))
  (return))

(fn SetNextPatrolPoint
  (if (Variables|Default|GetIsAIMoveForward)
    ;[0.15 0.15 0.15 0.5] AI按路线方向前进
    (Math|Integer|CompareInt (Variables|Default|GetCurrentPatrolPointNum) (Variables|Default|GetMaxPatrolPointNum)
      (:>
        _)
      (:==
        _)
      (:<
        (bind _result (Math|Integer|IncrementInt (Variables|Default|GetCurrentPatrolPointNum))
          (:%20%20
            (return _result)))))
    (bind _result_2 (Math|Integer|DecrementInt (Variables|Default|GetCurrentPatrolPointNum))
      (:%20%20
        (Variables|Default|SetIsAIMoveForward false)
        (return _result_2)))
    (else
      ;[0.15 0.15 0.15 0.5] AI按路线方向后退
      (Math|Integer|CompareInt (Variables|Default|GetCurrentPatrolPointNum) 1
        (:>
          (bind _result_3 (Math|Integer|DecrementInt (Variables|Default|GetCurrentPatrolPointNum))
            (:%20%20
              (return _result_3))))
        (:==
          _)
        (:<
          _))
      (bind _result_4 (Math|Integer|IncrementInt (Variables|Default|GetCurrentPatrolPointNum))
        (:%20%20
          (Variables|Default|SetIsAIMoveForward true)
          (return _result_4))))))