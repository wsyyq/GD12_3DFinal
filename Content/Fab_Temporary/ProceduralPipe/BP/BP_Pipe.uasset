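; Procedural pipe actor that builds a bent pipe along an editable spline in its construction script.
; It forces the spline linear, then derives a second spline that splits each inner corner into two points offset by TurnDistance, with scaled tangents to round the bends.
; Spline mesh segments form the pipe along that spline, and optional short connector meshes cap bend boundaries, plus both ends when enabled.
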(event EventBeginPlay)

(event Collision|EventActorBeginOverlap
  (params (OtherActor :type Actor%20Object%20Reference)))

(event EventTick
  (params (DeltaSeconds :type Float%20%28single-precision%29)))

(fn ConstructionScript
  (Utilities|FlowControl|Sequence
    (:then_0
      (for _index (range 0 (Spline|GetNumberOfSplinePoints (Variables|Default|GetSpline)))
        (Spline|SetSplinePointType (Variables|Default|GetSpline) _index "Linear" true)))
    (:then_1
      (CallFunction|SpawnSpline)
      (CallFunction|SpawnPipe)
      (if (Variables|Connect|GetIs%20Connected)
        (CallFunction|SpawnConnectMesh)))))

(fn SpawnSpline
  (bind _spline (Variables|Default|GetSpline))
  (bind _spline_2 (Variables|Default|GetSpline))
  (bind _spline_3 (Variables|Default|GetSpline))
  (bind _spline_4 (Variables|Default|GetSpline))
  (bind _spline_5 (Variables|Default|GetSpline))
  (bind _returnvalue (Spline|GetNumberOfSplinePoints _spline))
  (bind _returnvalue_2 (- _returnvalue 1))
  (bind _returnvalue_3 (AddComponent|AddSplineComponent false))
  (bind _output_get (Variables|Default|SetNewSpline _returnvalue_3))
  (Spline|ClearSplinePoints _output_get true)
  (for _index (range 0 (- (Spline|GetNumberOfSplinePoints (Variables|Default|GetSpline)) 1))
    (if (== _index 0)
      (Spline|AddSplinePoint (Variables|Default|GetNewSpline) (Spline|GetLocationatSplinePoint _spline_5 0 "Local") "Local" true)
      (Utilities|Array|Add (Variables|Default|GetSplineTangent) (Spline|GetTangentatSplinePoint _spline_5 0 "Local"))
      (elif (== _index _returnvalue_2)
        (Spline|AddSplinePoint (Variables|Default|GetNewSpline) (Spline|GetLocationatSplinePoint _spline_4 _returnvalue_2 "Local") "Local" true)
        (Utilities|Array|Add (Variables|Default|GetSplineTangent) (Spline|GetTangentatSplinePoint _spline_4 _returnvalue_2 "Local"))
        (else
          (Spline|AddSplinePoint (Variables|Default|GetNewSpline) (Spline|GetLocationatDistanceAlongSpline _spline_3 (- (Spline|GetDistanceAlongSplineatSplinePoint (Variables|Default|GetSpline) _index) (Variables|Default|GetTurnDistance)) "Local") "Local" true)
          (Spline|AddSplinePoint (Variables|Default|GetNewSpline) (Spline|GetLocationatDistanceAlongSpline _spline_2 (+ (Spline|GetDistanceAlongSplineatSplinePoint (Variables|Default|GetSpline) _index) (Variables|Default|GetTurnDistance)) "Local") "Local" true)
          (Utilities|Array|Add (Variables|Default|GetSplineTangent) (Spline|GetTangentatDistanceAlongSpline _spline_3 (- (Spline|GetDistanceAlongSplineatSplinePoint (Variables|Default|GetSpline) _index) (Variables|Default|GetTurnDistance)) "Local"))
          (Utilities|Array|Add (Variables|Default|GetSplineTangent) (Spline|GetTangentatDistanceAlongSpline _spline_2 (+ (Spline|GetDistanceAlongSplineatSplinePoint (Variables|Default|GetSpline) _index) (Variables|Default|GetTurnDistance)) "Local"))))))
  ;[0 0 0] 设置样条点切线
  (for _index_2 (range 0 (- (Spline|GetNumberOfSplinePoints (Variables|Default|GetNewSpline)) 1))
    (Spline|SetTangentatSplinePoint (Variables|Default|GetNewSpline) _index_2 (* (Math|Vector|Normalize (Utilities|Array|Get(acopy) (Variables|Default|GetSplineTangent) _index_2)) (* (Variables|Default|GetTurnDistance) 2.0)) "Local" true)))

(fn SpawnConnectMesh
  (bind _newspline (Variables|Default|GetNewSpline))
  (bind _connectmeshradiu (Variables|Connect|GetConnectMeshRadiu))
  (bind _newspline_2 (Variables|Default|GetNewSpline))
  (bind _connectmeshradiu_2 (Variables|Connect|GetConnectMeshRadiu))
  (bind _newspline_3 (Variables|Default|GetNewSpline))
  (bind _returnvalue (Spline|GetNumberOfSplinePoints _newspline_3))
  (for _index (range (select (Variables|Connect|GetConnectInStartAndEnd) 0 1) (select (Variables|Connect|GetConnectInStartAndEnd) (- _returnvalue 1) (- _returnvalue 2)))
    (Variables|Default|SetIndex_0 _index)
    (if (== (.Remainder (Math|Float|Division(WholeandRemainder) (Math|Conversions|ToFloat(Integer) _index) 2.0)) 1.0)
      (bind _returnvalue_2 (AddComponent|AddSplineMeshComponent false))
      (Components|StaticMesh|SetStaticMesh _returnvalue_2 (Variables|Connect|GetConnectMesh))
      (Rendering|Material|SetMaterial _returnvalue_2 0 (Variables|Default|GetPipe_Material))
      (SplineMesh|SetStartandEnd _returnvalue_2 (Spline|GetLocationatDistanceAlongSpline _newspline_2 (- (Spline|GetDistanceAlongSplineatSplinePoint (Variables|Default|GetNewSpline) (Variables|Default|GetIndex_0)) (Variables|Connect|GetConnectLength)) "Local") (Math|Vector|Normalize (Spline|GetTangentatDistanceAlongSpline _newspline_2 (- (Spline|GetDistanceAlongSplineatSplinePoint (Variables|Default|GetNewSpline) (Variables|Default|GetIndex_0)) (Variables|Connect|GetConnectLength)) "Local")) (Spline|GetLocationatDistanceAlongSpline _newspline_2 (Spline|GetDistanceAlongSplineatSplinePoint (Variables|Default|GetNewSpline) (Variables|Default|GetIndex_0)) "Local") (Math|Vector|Normalize (Spline|GetTangentatDistanceAlongSpline _newspline_2 (Spline|GetDistanceAlongSplineatSplinePoint (Variables|Default|GetNewSpline) (Variables|Default|GetIndex_0)) "Local")) true :!class /Script/Engine.SplineMeshComponent)
      (SplineMesh|SetStartScale _returnvalue_2 (Math|Vector2D|MakeVector2D _connectmeshradiu_2 _connectmeshradiu_2) true :!class /Script/Engine.SplineMeshComponent)
      (SplineMesh|SetEndScale _returnvalue_2 (Math|Vector2D|MakeVector2D _connectmeshradiu_2 _connectmeshradiu_2) true :!class /Script/Engine.SplineMeshComponent)
      (else
        (bind _returnvalue_3 (AddComponent|AddSplineMeshComponent false))
        (Components|StaticMesh|SetStaticMesh _returnvalue_3 (Variables|Connect|GetConnectMesh))
        (Rendering|Material|SetMaterial _returnvalue_3 0 (Variables|Default|GetPipe_Material))
        (SplineMesh|SetStartandEnd _returnvalue_3 (Spline|GetLocationatDistanceAlongSpline _newspline (Spline|GetDistanceAlongSplineatSplinePoint (Variables|Default|GetNewSpline) (Variables|Default|GetIndex_0)) "Local") (Math|Vector|Normalize (Spline|GetTangentatDistanceAlongSpline _newspline (Spline|GetDistanceAlongSplineatSplinePoint (Variables|Default|GetNewSpline) (Variables|Default|GetIndex_0)) "Local")) (Spline|GetLocationatDistanceAlongSpline _newspline (+ (Spline|GetDistanceAlongSplineatSplinePoint (Variables|Default|GetNewSpline) (Variables|Default|GetIndex_0)) (Variables|Connect|GetConnectLength)) "Local") (Math|Vector|Normalize (Spline|GetTangentatDistanceAlongSpline _newspline (+ (Spline|GetDistanceAlongSplineatSplinePoint (Variables|Default|GetNewSpline) (Variables|Default|GetIndex_0)) (Variables|Connect|GetConnectLength)) "Local")) true :!class /Script/Engine.SplineMeshComponent)
        (SplineMesh|SetStartScale _returnvalue_3 (Math|Vector2D|MakeVector2D _connectmeshradiu _connectmeshradiu) true :!class /Script/Engine.SplineMeshComponent)
        (SplineMesh|SetEndScale _returnvalue_3 (Math|Vector2D|MakeVector2D _connectmeshradiu _connectmeshradiu) true :!class /Script/Engine.SplineMeshComponent)))))

(fn SpawnPipe
  (bind _newspline (Variables|Default|GetNewSpline))
  (bind _piperadiu (Variables|Default|GetPipeRadiu))
  (for _index (range 0 (- (Spline|GetNumberOfSplinePoints (Variables|Default|GetNewSpline)) 2))
    (bind _returnvalue (AddComponent|AddSplineMeshComponent false))
    (Components|StaticMesh|SetStaticMesh _returnvalue (Variables|Default|GetPipeMesh))
    (Rendering|Material|SetMaterial _returnvalue 0 (Variables|Default|GetPipe_Material))
    (SplineMesh|SetStartandEnd _returnvalue (.Location (Spline|GetLocationandTangentatSplinePoint _newspline _index "Local")) (.Tangent (Spline|GetLocationandTangentatSplinePoint _newspline _index "Local")) (.Location (Spline|GetLocationandTangentatSplinePoint _newspline (+ _index 1) "Local")) (.Tangent (Spline|GetLocationandTangentatSplinePoint _newspline (+ _index 1) "Local")) true :!class /Script/Engine.SplineMeshComponent)
    (SplineMesh|SetStartScale _returnvalue (Math|Vector2D|MakeVector2D _piperadiu _piperadiu) true :!class /Script/Engine.SplineMeshComponent)
    (SplineMesh|SetEndScale _returnvalue (Math|Vector2D|MakeVector2D _piperadiu _piperadiu) true :!class /Script/Engine.SplineMeshComponent)))